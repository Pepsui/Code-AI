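; AI spawner actor for the EasyMultiSave content that populates the level with saved AI pawns a single time.
; On BeginPlay it waits for an async operation to complete, then spawns a SavedAIPawn at every TargetPoint in the world with random yaw, ignoring collisions.
; The saved AlreadySpawned flag prevents spawning again, and its ComponentsToSave function returns no components.
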(event EventBeginPlay
  (|AsyncWaitforOperation
    (:OnCompleted
      (if (not (Variables|Default|GetbAlreadySpawned))
        (bind _outactors (Actor|GetAllActorsOfClass "/Script/Engine.TargetPoint"))
        (for _array_element _outactors
          (Game|SpawnActorfromClass "/Game/EasyMultiSaveContent/Blueprints/AI/SavedAIPawn.SavedAIPawn_C" (CallFunction|MakeSpawnTransform _array_element) "AlwaysSpawn" 0 0))
        (Variables|Default|SetbAlreadySpawned true) ; Saved
      ))))

(fn ConstructionScript)

(fn MakeSpawnTransform
  (params (SpawnPoint :type Actor%20Object%20Reference))
  (return (Math|Transform|MakeTransform (Transformation|GetActorLocation SpawnPoint) (Math|Rotator|MakeRotator 0.0 0.0 (.Yaw (Math|Rotator|BreakRotator (Math|Random|RandomRotator false)))))))

(fn ComponentstoSave
  (return 0))