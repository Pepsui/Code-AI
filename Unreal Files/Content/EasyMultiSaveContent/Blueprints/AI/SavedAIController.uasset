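; AI controller for the Easy Multi Save system that keeps its link to the possessed pawn across save and load.
; ActorPreSave stores the controlled pawn as a soft object reference.
; ActorLoaded resolves that reference and possesses the pawn only if none is controlled, which covers spawned pawns since placed ones already have it.
; It then prints the pawn and controller names on screen for debugging.
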(event EventActorLoaded
  (bind _possessedpawn (Variables|Default|GetPossessedPawn))
  (bind _output (Utilities|ResolveSoftReference _possessedpawn))
  (Utilities|IsValid _output
    (:Is%20Valid
      (Utilities|FlowControl|Sequence
        (:then_0
          (Utilities|IsValid (Pawn|GetControlledPawn) ; For placed AI pawns it will be valid.\nFor spawned not
            (:Is%20Not%20Valid
              (Pawn|Possess _output) ; Possess from the saved soft object ref
            )))
        (:then_1
          (CallFunction|DebugPrint))))))

(event EventActorPreSave
  (Variables|Default|SetPossessedPawn (Utilities|ResolveSoftReference (Pawn|GetControlledPawn))))

(fn ConstructionScript)

(fn DebugPrint
  (bind _returnvalue (Pawn|GetControlledPawn))
  (Utilities|IsValid _returnvalue
    (:Is%20Valid
      (Development|PrintString (Utilities|String|Append (Utilities|GetDisplayName _returnvalue) "     -     " (Utilities|GetDisplayName self)) true true "(R=0.000000,G=1.000000,B=0.262510,A=1.000000)" 3.0))))

(fn ComponentstoSave
  (return 0))