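; AI pawn for the Easy Multi Save system that possesses itself with an AI controller when it was not restored from a save.
; On BeginPlay it waits for the pending operation to complete, then spawns its AIControllerClass and possesses itself if it is neither flagged as loaded nor already controlled.
; ActorLoaded sets that flag, ComponentsToSave returns no components, and a helper builds an origin transform with random yaw.
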(event EventBeginPlay
  (|AsyncWaitforOperation
    (:OnCompleted
      (if (not (Variables|Default|GetbEMSLoaded))
        (Utilities|IsValid (Pawn|GetController)
          (:Is%20Not%20Valid
            (CallFunction|PerformPossession)))))))

(event EventActorLoaded
  (Variables|Default|SetbEMSLoaded true))

(fn ConstructionScript)

(fn MakeSpawnTransform
  (return (Math|Transform|MakeTransform "0, 0, 0" (Math|Rotator|MakeRotator 0.0 0.0 (.Yaw (Math|Rotator|BreakRotator (Math|Random|RandomRotator false)))))))

(fn PerformPossession
  (bind _returnvalue (Game|SpawnActorfromClass (Variables|Default|GetAIControllerClass) (Math|Transform|MakeTransform "0, 0, 0") "AlwaysSpawn" 0 0))
  (Pawn|Possess _returnvalue self))

(fn ComponentstoSave
  (return 0))