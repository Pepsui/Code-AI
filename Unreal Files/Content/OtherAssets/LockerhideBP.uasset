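; Locker hiding spot Blueprint that lets the player toggle hiding inside it.
; Box overlap with the ThirdPersonCharacter stores it, enables input and opens a gate for the Hide action; leaving disables both.
; Hide toggles the character's visibility and collision, blends the camera between character and locker, and plays a timeline rotating the door.
; A separate AISearch event, apparently for searching AI, swings the same door with its own timeline.
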(event OnComponentBeginOverlap(Box)
  (params (OverlappedComponent :type Primitive%20Component%20Object%20Reference) (OtherActor :type Actor%20Object%20Reference) (OtherComp :type Primitive%20Component%20Object%20Reference) (OtherBodyIndex :type Integer) (bFromSweep :type Boolean) (SweepResult :type Hit%20Result%20Structure%20%28by%20ref%29))
  (bind _asthird_person_character (Utilities|Casting|CastToThirdPersonCharacter OtherActor))
  (Variables|Default|SetChar%20REF _asthird_person_character)
  (Input|EnableInput (Game|GetPlayerController 0))
  (Utilities|FlowControl|Gate true) ; enters at Open
)

(event OnComponentEndOverlap(Box)
  (params (OverlappedComponent :type Primitive%20Component%20Object%20Reference) (OtherActor :type Actor%20Object%20Reference) (OtherComp :type Primitive%20Component%20Object%20Reference) (OtherBodyIndex :type Integer))
  (bind _returnvalue (Game|GetPlayerController 0))
  (Utilities|Casting|CastToThirdPersonCharacter OtherActor)
  (Input|DisableInput _returnvalue)
  (Utilities|FlowControl|Gate true) ; enters at Close
)

(event Custom|AISearch
  (bind _doortrack (Timeline|Timeline_0 PlayFromStart)
    (:Update
      (Transformation|SetRelativeRotation (Variables|Default|GetLocker_Door) (Math|Rotator|MakeRotator 0.0 0.0 (Math|Float|Lerp (Variables|Default|GetClosed_Angle) (Variables|Default|GetOpen_Angle) _doortrack)) false false))))

(event Input|ActionEvents|InputActionHide
  (params (Key :type Key%20Structure :default "None"))
  (:Pressed
    (Utilities|FlowControl|Gate true :!label _label
      (:Exit
        (Utilities|FlowControl|Sequence
          (:then_0
            (CallFunction|ToggleHide)
            (Utilities|FlowControl|Delay 0.2)
            (Input|EnableInput (Game|GetPlayerController 0))
            (goto _label Open))
          (:then_1
            (|CollapseGraph_0)))))))

(fn ConstructionScript)

(fn ToggleHide
  (bind _returnvalue (Game|GetPlayerController 0))
  (bind _char_ref (Variables|Default|GetChar%20REF))
  (if (Variables|Default|GetIsHiding)
    (Variables|Default|SetIsHiding false)
    (Rendering|SetActorHiddenInGame _char_ref false)
    (Collision|SetActorEnableCollision _char_ref true)
    (Game|Player|SetViewTargetwithBlend _returnvalue _char_ref 0.8 "VTBlend_Linear" 0.0 false)
    (else
      (Variables|Default|SetIsHiding true)
      (Rendering|SetActorHiddenInGame _char_ref true)
      (Collision|SetActorEnableCollision _char_ref false)
      (Game|Player|SetViewTargetwithBlend _returnvalue self 0.8 "VTBlend_Linear" 0.0 false))))