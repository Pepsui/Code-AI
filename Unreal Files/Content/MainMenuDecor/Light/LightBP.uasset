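; LightBP is a flickering light fixture, filed under main menu decor, with a neon tube flicker sound.
; BeginPlay plays the sound at the actor's location, then enters an endless Flicker loop of randomized delays alternating TurnOff and TurnOn.
; These events toggle SpotLight visibility and swap the bulb mesh between black and lit materials.
; TurnOff also calls PlaySoundAtLocation with no sound assigned.
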(event Custom|Flicker
  (Utilities|FlowControl|Delay (Math|Random|RandomFloatinRange 0.8 1.4))
  (CallFunction|TurnOff)
  (Utilities|FlowControl|Delay (Math|Random|RandomFloatinRange 0.1 0.3))
  (CallFunction|Turnon)
  (Utilities|FlowControl|Delay (Math|Random|RandomFloatinRange 1.0 1.5))
  (CallFunction|TurnOff)
  (Utilities|FlowControl|Delay (Math|Random|RandomFloatinRange 0.3 0.7))
  (CallFunction|Turnon)
  (CallFunction|Flicker))

(event Custom|Turn%20Off
  (Rendering|Material|SetMaterial (Variables|Default|GetBulbSM) 0 "/Game/MainMenuDecor/BlackUnitMaterial.BlackUnitMaterial")
  (Rendering|SetVisibility (Variables|Default|GetSpotLight) false false)
  (Audio|PlaySoundatLocation 0 "0, 0, 0" "0, 0, 0" 1.0 1.0 0.0 0 0 0))

(event Custom|Turn%20On
  (Rendering|Material|SetMaterial (Variables|Default|GetBulbSM) 0 "/Game/MainMenuDecor/Light/LightMat.LightMat")
  (Rendering|SetVisibility (Variables|Default|GetSpotLight) true false))

(event EventBeginPlay
  (Audio|PlaySoundatLocation "/Game/MainMenuDecor/Light/500693__bolkmar__neon-tube-light-flickering_Cue.500693__bolkmar__neon-tube-light-flickering_Cue" (Transformation|GetActorLocation) "0, 0, 0" 1.0 1.0 0.0 0 0 0)
  (Utilities|FlowControl|Delay (Math|Random|RandomFloatinRange 0.8 1.4))
  (CallFunction|TurnOff)
  (Utilities|FlowControl|Delay (Math|Random|RandomFloatinRange 0.1 0.3))
  (CallFunction|Turnon)
  (Utilities|FlowControl|Delay (Math|Random|RandomFloatinRange 1.0 1.5))
  (CallFunction|TurnOff)
  (Utilities|FlowControl|Delay (Math|Random|RandomFloatinRange 0.3 0.7))
  (CallFunction|Turnon)
  (CallFunction|Flicker))

(fn ConstructionScript)