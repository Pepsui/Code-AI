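; MainMenuPawnBP is the main menu pawn that opens the menu UI when the first local player controller possesses it.
; On possession it creates the main menu container widget, adds it to the viewport, switches input to UI only and shows the mouse cursor.
; The intro plays unless the game mode's options string sets showIntro to false, an option passed through Open Level from the in-game menu.
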(event EventPossessed
  (params (NewController :type Controller%20Object%20Reference))
  (if (== NewController (Game|GetPlayerController 0))
    (bind _asplayer_controller (Utilities|Casting|CastToPlayerController NewController))
    ;[1 0.3634 0] Open Main Menu
    (bind _returnvalue (UserInterface|CreateWidget "/Game/MenuSystemPro/Blueprints/UI/Menus/Main/MainMenuContainerWidgetBP.MainMenuContainerWidgetBP_C" _asplayer_controller (CallFunction|ShouldShowIntro)))
    (UserInterface|Viewport|AddtoViewport _returnvalue 0)
    (Input|SetInputModeUIOnly _asplayer_controller _returnvalue "DoNotLock")
    (Variables|/Script/Engine.PlayerController|SetbShowMouseCursor _asplayer_controller true)))

(fn ConstructionScript)

(fn ShouldShowIntro
  ;[1 1 1] Get show intro option which is set by Open Level node in IngameMenuOverviewWidgetBP
  (return (Utilities|Enum|NotEqual(Enum) (Class|GameplayStatics|ParseOption (Variables|/Script/Engine.GameModeBase|GetOptionsString (Game|GetGameMode)) "showIntro") "false")))