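; Character component that gives each local player an in-game pause menu and applies saved control settings.
; On initialization it resolves the player index from the game mode's controller list and creates a collapsed menu widget.
; Opening switches to UI-only input with gamepad-aware cursor and notifies MenuControllerComponent; resuming restores game input after a short delay and reloads controls.
; It also provides axis speed/inversion scaling and preview rumble when enabled.
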(event Custom|LoadControls
  ;[0.8235 0.1804 0] Load Controls
  (bind (_invertlookx _invertlooky _cameraspeedx _cameraspeedy _rumble) (CallFunction|GetControlsSettings false false 0.0 0.0 false)) ; Defaults are set if nothing could be loaded
  (Variables|Default|SetbInvertLookX _invertlookx)
  (Variables|Default|SetbInvertLookY _invertlooky)
  (Variables|Default|SetCameraSpeedX _cameraspeedx)
  (Variables|Default|SetCameraSpeedY _cameraspeedy)
  (Variables|Default|SetbRumble _rumble))

(event Custom|OpenPauseMenu
  (bind _ingamemenuwidget (Variables|Default|GetIngameMenuWidget))
  (bind _playercontroller (Variables|Default|GetPlayerController))
  ;[0.8235 0.1804 0] Pause Menu
  (Widget|SetVisibility _ingamemenuwidget "SelfHitTestInvisible")
  (Default|OnNavigationEnter _ingamemenuwidget 0 (Variables|Default|GetIsGamepadBeingUsed) (Variables|Default|GetPlayerIndex))
  (Input|SetInputModeUIOnly _playercontroller _ingamemenuwidget "LockAlways")
  (Variables|/Script/Engine.PlayerController|SetbShowMouseCursor _playercontroller (not (Variables|Default|GetIsGamepadBeingUsed)))
  (Class|PauseGameBPI|Pause(Message) (Actor|GetComponentbyClass _playercontroller "/Game/MenuSystemPro/Blueprints/Player/MenuControllerComponent.MenuControllerComponent_C")))

(event Custom|OpenPauseMenuKeyboard
  ;[0.8235 0.1804 0] Pause Menu
  (Variables|Default|SetIsGamepadBeingUsed false)
  (CallFunction|OpenPauseMenu))

(event Custom|OpenPauseMenuGamepad
  ;[0.8235 0.1804 0] Pause Menu
  (Variables|Default|SetIsGamepadBeingUsed true)
  (CallFunction|OpenPauseMenu))

(event Custom|Rumble
  ;[0.8235 0.1804 0] Rumble
  (if (Variables|Default|GetbRumble)
    (Game|Feedback|ClientPlayForceFeedback (Variables|Default|GetPlayerController) "/Game/MenuSystemPro/Misc/PreviewForceFeedbackEffect.PreviewForceFeedbackEffect" "None" false false false) ; Play Preview Rumble
  ))

(event Custom|InitializeMenu
  (params (PlayerController :type Player%20Controller%20Object%20Reference))
  ;[0.8235 0.1804 0] Initialize Menu
  (CallFunction|LoadControls)
  (CallFunction|SetupLocalPlayer PlayerController)
  (bind _returnvalue (UserInterface|CreateWidget "/Game/MenuSystemPro/Blueprints/UI/Menus/Ingame/IngameMenuContainerWidgetBP.IngameMenuContainerWidgetBP_C" (Variables|Default|GetPlayerController) (Variables|Default|GetPlayerIndex)))
  (bind _output_get (Variables|Default|SetIngameMenuWidget _returnvalue))
  (UserInterface|Viewport|AddtoViewport _output_get 0)
  (Widget|SetVisibility _output_get "Collapsed")
  (Variables|/Script/Engine.PlayerController|SetbShowMouseCursor (Variables|Default|GetPlayerController) false)
  (Input|SetInputModeGameOnly (Variables|Default|GetPlayerController)))

(event EventResume
  (bind _playercontroller (Variables|Default|GetPlayerController))
  ;[1 0.2156 0] Pause Game Interface Events
  (Widget|SetVisibility (Variables|Default|GetIngameMenuWidget) "Collapsed")
  (Utilities|FlowControl|Delay 0.25)
  (Input|SetInputModeGameOnly _playercontroller)
  (Variables|/Script/Engine.PlayerController|SetbShowMouseCursor _playercontroller false)
  (CallFunction|LoadControls))

(event EventPause
  ;[1 0.2156 0] Pause Game Interface Events
)

(fn ModifyAxisValue
  (params (InVal :type Float%20%28single-precision%29) (SpeedMultiplier :type Float%20%28single-precision%29) (InvertAxis :type Boolean))
  (bind _returnvalue (* InVal SpeedMultiplier))
  (if InvertAxis
    (bind _result (Math|Float|NegateFloat _returnvalue)
      (:%20%20
        (return _result)))
    (else
      (return _returnvalue))))

(fn SetupLocalPlayer
  (params (PlayerController :type Player%20Controller%20Object%20Reference))
  ;[1 1 1] Find player controller that this component belongs to
  (Variables|Default|SetPlayerController PlayerController)
  (bind _asbase_game_mode_bp (Utilities|Casting|CastToBaseGameModeBP (Game|GetGameMode))
    (:then
      (for (_array_element _array_index) (Variables|/Game/MenuSystemPro/Blueprints/GameMode/MenuGameModeComponent.MenuGameModeComponent_C|GetPlayerControllers (Variables|/Game/MenuSystemPro/Blueprints/GameMode/BaseGameModeBP.BaseGameModeBP_C|GetMenuGameModeComponent _asbase_game_mode_bp))
        (if (== _array_element (Variables|Default|GetPlayerController))
          (Variables|Default|SetPlayerIndex _array_index)
          (return))))
    (:CastFailed
      (Variables|Default|SetPlayerIndex 0)
      (return))))