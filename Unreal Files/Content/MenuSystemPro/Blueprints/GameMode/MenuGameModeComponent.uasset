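; Game mode component from Menu System Pro that spawns players for local multiplayer.
; On BeginPlay it gathers all PlayerStarts, then matches one to each player index up to PlayerCount by its numeric PlayerStartTag.
; Each match creates a local player with its controller, using the start's array position as ControllerId, then spawns CharacterClass there and has that player index's controller possess it.
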(event EventBeginPlay
  ;[1 1 1] Spawn logic to support local multiplayer - Menu System Pro
  (CallFunction|GetPlayerStarts)
  (CallFunction|SpawnPlayers))

(fn GetPlayerStarts
  (bind _outactors (Actor|GetAllActorsOfClass "/Script/Engine.PlayerStart"))
  (Variables|MenuSystemPro|SetPlayerSpawnpoints _outactors))

(fn SpawnPlayers
  ;[1 1 1] Create a new local player for every player start in the level and assign a new PlayerController & PlayerCharacter to them.
  (for _index (range 0 (- (Variables|MenuSystemPro|GetPlayerCount) 1))
    (LocalVariables|SetPlayerIndex _index)
    (bind (_array_element _array_index) (Utilities|Array|ForEachLoopwithBreak (Variables|MenuSystemPro|GetPlayerSpawnpoints) :!label _label)
      (:LoopBody
        (if (Utilities|Name|Equal(Name) (Variables|/Script/Engine.PlayerStart|GetPlayerStartTag _array_element) (Utilities|String|StringToName (Utilities|String|ToString(Integer) _index)))
          (bind _returnvalue (Class|GameplayStatics|CreatePlayer _array_index))
          (Utilities|Array|AddUnique (Variables|MenuSystemPro|GetPlayerControllers) _returnvalue)
          (bind _returnvalue_2 (Game|SpawnActorfromClass (Variables|MenuSystemPro|GetCharacterClass) (Transformation|GetActorTransform _array_element) "AlwaysSpawn" 0 0))
          (bind _aspawn (Utilities|Casting|CastToPawn _returnvalue_2))
          (Pawn|Possess (Game|GetPlayerController (LocalVariables|GetPlayerIndex)) _aspawn)
          (goto _label Break))))))