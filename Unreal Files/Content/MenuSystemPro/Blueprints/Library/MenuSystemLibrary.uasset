(fn GetSupportedScreenResolutions
  (bind _returnvalue (Settings|GetGameUserSettings))
  (bind _resolutions (Class|KismetSystemLibrary|GetSupportedFullscreenResolutions)) ; Get all resolutions from RHI
  (for (_array_element _array_index) _resolutions
    ;[1 1 1] Build screen res display string
    (Utilities|Array|Add (LocalVariables|GetResolutions) (Utilities|String|Append (Utilities|String|ToString(Integer) (.X (Utilities|Struct|BreakIntPoint _array_element))) " x " (Utilities|String|ToString(Integer) (.Y (Utilities|Struct|BreakIntPoint _array_element)))))
    ;[1 1 1] Get Current Resolution index
    (if (Class|KismetMathLibrary|EqualIntPointIntPoint _array_element (Class|GameUserSettings|GetScreenResolution _returnvalue))
      (LocalVariables|SetCurrentResIndex _array_index)))
  (return (LocalVariables|GetResolutions) (LocalVariables|GetCurrentResIndex)))

(fn SetPersistentVariable
  (params (Name :type String) (Value :type String))
  (bind _output_get (LocalVariables|SetSaveGame (CallFunction|GetSettingsSaveGame (LocalVariables|Get__WorldContext))))
  (Default|SetPersistentVar _output_get Name Value)
  (CallFunction|SaveSettingstoSlot _output_get (LocalVariables|Get__WorldContext)))

(fn GetPersistentVariable
  (params (Name :type String))
  (bind (_value _bfound) (Default|GetPersistentVar (CallFunction|GetSettingsSaveGame (LocalVariables|Get__WorldContext)) Name))
  (return _value _bfound))

(fn GetSettingsSaveGame
  ;[1 1 1] Try to load Settings Save Slot
  (bind _returnvalue (SaveGame|DoesSaveGameExist "MenuSettingsSaveSlot"))
  (if _returnvalue
    (bind _returnvalue_2 (SaveGame|LoadGamefromSlot "MenuSettingsSaveSlot"))
    (bind _asmenu_settings_save_game_bp (Utilities|Casting|CastToMenuSettingsSaveGameBP _returnvalue_2))
    (return _asmenu_settings_save_game_bp)
    (else
      ;[1 1 1] Create Settings Save Slot if doesn't exist
      (bind _returnvalue_3 (SaveGame|CreateSaveGameObject "/Game/MenuSystemPro/Blueprints/SaveGame/MenuSettingsSaveGameBP.MenuSettingsSaveGameBP_C"))
      (SaveGame|SaveGametoSlot _returnvalue_3 "MenuSettingsSaveSlot")
      (return _returnvalue_3))))

(fn SetBenchmarkAlreadyRan
  (params (bBenchmarkRan :type Boolean))
  (bind _output_get (LocalVariables|SetSaveGame (CallFunction|GetSettingsSaveGame (LocalVariables|Get__WorldContext))))
  (Variables|/Game/MenuSystemPro/Blueprints/SaveGame/MenuSettingsSaveGameBP.MenuSettingsSaveGameBP_C|SetbBenchmarkAlreadyRan _output_get bBenchmarkRan)
  (CallFunction|SaveSettingstoSlot _output_get (LocalVariables|Get__WorldContext)))

(fn GetBenchmarkAlreadyRan
  (return (Variables|/Game/MenuSystemPro/Blueprints/SaveGame/MenuSettingsSaveGameBP.MenuSettingsSaveGameBP_C|GetbBenchmarkAlreadyRan (CallFunction|GetSettingsSaveGame (LocalVariables|Get__WorldContext)))))

(fn SaveSettingstoSlot
  (params (SaveGameObject :type Save%20Game%20Object%20Reference))
  (SaveGame|SaveGametoSlot SaveGameObject "MenuSettingsSaveSlot"))

(fn GetPostProcessingSettings
  (params (MotionBlurDefault :type Boolean) (LensFlaresDefault :type Boolean) (SSRDefault :type Boolean) (BloomDefault :type Boolean) (AntiAliasingDefault :type Integer) (AmbientOcclusionDefault :type Boolean))
  (Utilities|FlowControl|Sequence
    (:then_0
      ;[1 1 1] Get Menu Settings Save Game instance
      (LocalVariables|SetSaveGame (CallFunction|GetSettingsSaveGame (LocalVariables|Get__WorldContext))))
    (:then_1
      ;[1 1 1] First Run: Set Variables from Default Values
      (if (Variables|/Game/MenuSystemPro/Blueprints/SaveGame/MenuSettingsSaveGameBP.MenuSettingsSaveGameBP_C|GetbPostProcessingFirstRun (LocalVariables|GetSaveGame)) ; Is first run?
        (Utilities|FlowControl|Sequence
          (:then_0
            (Variables|/Game/MenuSystemPro/Blueprints/SaveGame/MenuSettingsSaveGameBP.MenuSettingsSaveGameBP_C|SetMotionBlur (LocalVariables|GetSaveGame) MotionBlurDefault))
          (:then_1
            (Variables|/Game/MenuSystemPro/Blueprints/SaveGame/MenuSettingsSaveGameBP.MenuSettingsSaveGameBP_C|SetLensFlares (LocalVariables|GetSaveGame) LensFlaresDefault))
          (:then_2
            (Variables|/Game/MenuSystemPro/Blueprints/SaveGame/MenuSettingsSaveGameBP.MenuSettingsSaveGameBP_C|SetSSR (LocalVariables|GetSaveGame) SSRDefault))
          (:then_3
            (Variables|/Game/MenuSystemPro/Blueprints/SaveGame/MenuSettingsSaveGameBP.MenuSettingsSaveGameBP_C|SetBloom (LocalVariables|GetSaveGame) BloomDefault))
          (:then_4
            (Variables|/Game/MenuSystemPro/Blueprints/SaveGame/MenuSettingsSaveGameBP.MenuSettingsSaveGameBP_C|SetAntiAliasing (LocalVariables|GetSaveGame) AntiAliasingDefault))
          (:then_5
            (Variables|/Game/MenuSystemPro/Blueprints/SaveGame/MenuSettingsSaveGameBP.MenuSettingsSaveGameBP_C|SetAmbientOcclusion (LocalVariables|GetSaveGame) AmbientOcclusionDefault))
          (:then_6
            (Variables|/Game/MenuSystemPro/Blueprints/SaveGame/MenuSettingsSaveGameBP.MenuSettingsSaveGameBP_C|SetbPostProcessingFirstRun (LocalVariables|GetSaveGame) false))
          (:then_7
            (CallFunction|SaveSettingstoSlot (LocalVariables|GetSaveGame) (LocalVariables|Get__WorldContext))))))
    (:then_2
      ;[1 1 1] Get Post Processing Settings from Settings Save Game
      (return (Variables|/Game/MenuSystemPro/Blueprints/SaveGame/MenuSettingsSaveGameBP.MenuSettingsSaveGameBP_C|GetMotionBlur (LocalVariables|GetSaveGame)) (Variables|/Game/MenuSystemPro/Blueprints/SaveGame/MenuSettingsSaveGameBP.MenuSettingsSaveGameBP_C|GetLensFlares (LocalVariables|GetSaveGame)) (Variables|/Game/MenuSystemPro/Blueprints/SaveGame/MenuSettingsSaveGameBP.MenuSettingsSaveGameBP_C|GetSSR (LocalVariables|GetSaveGame)) (Variables|/Game/MenuSystemPro/Blueprints/SaveGame/MenuSettingsSaveGameBP.MenuSettingsSaveGameBP_C|GetBloom (LocalVariables|GetSaveGame)) (Variables|/Game/MenuSystemPro/Blueprints/SaveGame/MenuSettingsSaveGameBP.MenuSettingsSaveGameBP_C|GetAntiAliasing (LocalVariables|GetSaveGame)) (Variables|/Game/MenuSystemPro/Blueprints/SaveGame/MenuSettingsSaveGameBP.MenuSettingsSaveGameBP_C|GetAmbientOcclusion (LocalVariables|GetSaveGame))))))

(fn SetPostProcessingSettings
  (params (MotionBlur :type Boolean) (LensFlares :type Boolean) (SSR :type Boolean) (Bloom :type Boolean) (AntiAliasing :type Integer) (AmbientOcclusion :type Boolean))
  (Utilities|FlowControl|Sequence
    (:then_0
      ;[1 1 1] Get Menu Settings Save Game instance
      (LocalVariables|SetSaveGame (CallFunction|GetSettingsSaveGame (LocalVariables|Get__WorldContext))))
    (:then_1
      ;[1 1 1] Set Variables
      (Utilities|FlowControl|Sequence
        (:then_0
          (Variables|/Game/MenuSystemPro/Blueprints/SaveGame/MenuSettingsSaveGameBP.MenuSettingsSaveGameBP_C|SetMotionBlur (LocalVariables|GetSaveGame) MotionBlur))
        (:then_1
          (Variables|/Game/MenuSystemPro/Blueprints/SaveGame/MenuSettingsSaveGameBP.MenuSettingsSaveGameBP_C|SetLensFlares (LocalVariables|GetSaveGame) LensFlares))
        (:then_2
          (Variables|/Game/MenuSystemPro/Blueprints/SaveGame/MenuSettingsSaveGameBP.MenuSettingsSaveGameBP_C|SetSSR (LocalVariables|GetSaveGame) SSR))
        (:then_3
          (Variables|/Game/MenuSystemPro/Blueprints/SaveGame/MenuSettingsSaveGameBP.MenuSettingsSaveGameBP_C|SetBloom (LocalVariables|GetSaveGame) Bloom))
        (:then_4
          (Variables|/Game/MenuSystemPro/Blueprints/SaveGame/MenuSettingsSaveGameBP.MenuSettingsSaveGameBP_C|SetAntiAliasing (LocalVariables|GetSaveGame) AntiAliasing))
        (:then_5
          (Variables|/Game/MenuSystemPro/Blueprints/SaveGame/MenuSettingsSaveGameBP.MenuSettingsSaveGameBP_C|SetAmbientOcclusion (LocalVariables|GetSaveGame) AmbientOcclusion))))
    (:then_2
      ;[1 1 1] Save Settings to Save Game Slot
      (CallFunction|SaveSettingstoSlot (LocalVariables|GetSaveGame) (LocalVariables|Get__WorldContext)))
    (:then_3
      ;[1 1 1] Apply Post Processing Settings
      (CallFunction|ApplyPostProcessingSettings MotionBlur LensFlares SSR Bloom AntiAliasing AmbientOcclusion (LocalVariables|Get__WorldContext)))))

(fn ApplyPostProcessingSettings
  (params (MotionBlur :type Boolean) (LensFlares :type Boolean) (SSR :type Boolean) (Bloom :type Boolean) (AntiAliasing :type Integer) (AmbientOcclusion :type Boolean))
  (Utilities|FlowControl|Sequence
    (:then_0
      ;[1 1 1] Motion Blur
      (Development|ExecuteConsoleCommand (LocalVariables|Get__WorldContext) (Utilities|String|Append "r.MotionBlur.Amount " (Utilities|String|SelectString "0.5" "0" MotionBlur)) (Game|GetPlayerController (LocalVariables|Get__WorldContext))))
    (:then_1
      ;[1 1 1] Lens Flares
      (Development|ExecuteConsoleCommand (LocalVariables|Get__WorldContext) (Utilities|String|Append "r.DefaultFeature.LensFlare " (Utilities|String|SelectString "1" "0" LensFlares)) (Game|GetPlayerController (LocalVariables|Get__WorldContext))))
    (:then_2
      ;[1 1 1] SSR
      (Development|ExecuteConsoleCommand (LocalVariables|Get__WorldContext) (Utilities|String|Append "r.SSR.Quality " (Utilities|String|SelectString "3" "0" SSR)) (Game|GetPlayerController (LocalVariables|Get__WorldContext))))
    (:then_3
      ;[1 1 1] Bloom
      (Development|ExecuteConsoleCommand (LocalVariables|Get__WorldContext) (Utilities|String|Append "r.BloomQuality " (Utilities|String|SelectString "5" "0" Bloom)) (Game|GetPlayerController (LocalVariables|Get__WorldContext))))
    (:then_4
      ;[1 1 1] Anti Aliasing
      (Development|ExecuteConsoleCommand (LocalVariables|Get__WorldContext) (Utilities|String|Append "r.DefaultFeature.AntiAliasing " (Utilities|String|ToString(Integer) AntiAliasing)) (Game|GetPlayerController (LocalVariables|Get__WorldContext))))
    (:then_5
      ;[1 1 1] Motion Blur
      (Development|ExecuteConsoleCommand (LocalVariables|Get__WorldContext) (Utilities|String|Append "r.DefaultFeature.AmbientOcclusion " (Utilities|String|SelectString "1" "0" AmbientOcclusion)) (Game|GetPlayerController (LocalVariables|Get__WorldContext))))))

(fn SetDefaultBindingsFirstRun
  (params (bDefaultBindingsFirstRun :type Boolean))
  (bind _output_get (LocalVariables|SetSaveGame (CallFunction|GetSettingsSaveGame (LocalVariables|Get__WorldContext))))
  (Variables|/Game/MenuSystemPro/Blueprints/SaveGame/MenuSettingsSaveGameBP.MenuSettingsSaveGameBP_C|SetbDefaultBindingsFirstRun _output_get bDefaultBindingsFirstRun)
  (CallFunction|SaveSettingstoSlot _output_get (LocalVariables|Get__WorldContext)))

(fn GetDefaultBindingsFirstRun
  (return (Variables|/Game/MenuSystemPro/Blueprints/SaveGame/MenuSettingsSaveGameBP.MenuSettingsSaveGameBP_C|GetbDefaultBindingsFirstRun (CallFunction|GetSettingsSaveGame (LocalVariables|Get__WorldContext)))))

(fn SetDefaultActionMappings
  (params (ActionKeyMappings :type Array%20of%20Input%20Action%20Key%20Mapping%20Structures))
  (bind _output_get (LocalVariables|SetSaveGame (CallFunction|GetSettingsSaveGame (LocalVariables|Get__WorldContext))))
  (Variables|/Game/MenuSystemPro/Blueprints/SaveGame/MenuSettingsSaveGameBP.MenuSettingsSaveGameBP_C|SetDefaultActionMappings _output_get ActionKeyMappings)
  (CallFunction|SaveSettingstoSlot _output_get (LocalVariables|Get__WorldContext)))

(fn SetDefaultAxisMappings
  (params (AxisKeyMappings :type Array%20of%20Input%20Axis%20Key%20Mapping%20Structures))
  (bind _output_get (LocalVariables|SetSaveGame (CallFunction|GetSettingsSaveGame (LocalVariables|Get__WorldContext))))
  (Variables|/Game/MenuSystemPro/Blueprints/SaveGame/MenuSettingsSaveGameBP.MenuSettingsSaveGameBP_C|SetDefaultAxisMappings _output_get AxisKeyMappings)
  (CallFunction|SaveSettingstoSlot _output_get (LocalVariables|Get__WorldContext)))

(fn GetDefaultActionMappings
  (return (Variables|/Game/MenuSystemPro/Blueprints/SaveGame/MenuSettingsSaveGameBP.MenuSettingsSaveGameBP_C|GetDefaultActionMappings (CallFunction|GetSettingsSaveGame (LocalVariables|Get__WorldContext)))))

(fn GetDefaultAxisMappings
  (return (Variables|/Game/MenuSystemPro/Blueprints/SaveGame/MenuSettingsSaveGameBP.MenuSettingsSaveGameBP_C|GetDefaultAxisMappings (CallFunction|GetSettingsSaveGame (LocalVariables|Get__WorldContext)))))

(fn GetRaytracingSettings
  (params (RaytracedShadowsDefault :type Integer) (RaytracedReflectionsDefault :type Integer) (RaytracedTranslucencyDefault :type Integer) (RaytracedAmbientOcclusionDefault :type Integer) (RaytracedGlobalIlluminationDefault :type Integer) (DLSSDefault :type Integer))
  (Utilities|FlowControl|Sequence
    (:then_0
      ;[1 1 1] Get Menu Settings Save Game instance
      (LocalVariables|SetSaveGame (CallFunction|GetSettingsSaveGame (LocalVariables|Get__WorldContext))))
    (:then_1
      ;[1 1 1] First Run: Set Variables from Default Values
      (if (Variables|/Game/MenuSystemPro/Blueprints/SaveGame/MenuSettingsSaveGameBP.MenuSettingsSaveGameBP_C|GetbRaytracingFirstRun (LocalVariables|GetSaveGame)) ; Is first run?
        (Utilities|FlowControl|Sequence
          (:then_0
            (Variables|/Game/MenuSystemPro/Blueprints/SaveGame/MenuSettingsSaveGameBP.MenuSettingsSaveGameBP_C|SetRaytracedShadows (LocalVariables|GetSaveGame) RaytracedShadowsDefault))
          (:then_1
            (Variables|/Game/MenuSystemPro/Blueprints/SaveGame/MenuSettingsSaveGameBP.MenuSettingsSaveGameBP_C|SetRaytracedReflections (LocalVariables|GetSaveGame) RaytracedReflectionsDefault))
          (:then_2
            (Variables|/Game/MenuSystemPro/Blueprints/SaveGame/MenuSettingsSaveGameBP.MenuSettingsSaveGameBP_C|SetRaytracedTranslucency (LocalVariables|GetSaveGame) RaytracedTranslucencyDefault))
          (:then_3
            (Variables|/Game/MenuSystemPro/Blueprints/SaveGame/MenuSettingsSaveGameBP.MenuSettingsSaveGameBP_C|SetRaytracedAmbientOcclusion (LocalVariables|GetSaveGame) RaytracedAmbientOcclusionDefault))
          (:then_4
            (Variables|/Game/MenuSystemPro/Blueprints/SaveGame/MenuSettingsSaveGameBP.MenuSettingsSaveGameBP_C|SetRaytracedGlobalIllumination (LocalVariables|GetSaveGame) RaytracedGlobalIlluminationDefault))
          (:then_5
            (Variables|/Game/MenuSystemPro/Blueprints/SaveGame/MenuSettingsSaveGameBP.MenuSettingsSaveGameBP_C|SetDLSS (LocalVariables|GetSaveGame) DLSSDefault))
          (:then_6
            (Variables|/Game/MenuSystemPro/Blueprints/SaveGame/MenuSettingsSaveGameBP.MenuSettingsSaveGameBP_C|SetbRaytracingFirstRun (LocalVariables|GetSaveGame) false))
          (:then_7
            (CallFunction|SaveSettingstoSlot (LocalVariables|GetSaveGame) (LocalVariables|Get__WorldContext))))))
    (:then_2
      ;[1 1 1] Get Raytracing Settings from Settings Save Game
      (return (Variables|/Game/MenuSystemPro/Blueprints/SaveGame/MenuSettingsSaveGameBP.MenuSettingsSaveGameBP_C|GetRaytracedShadows (LocalVariables|GetSaveGame)) (Variables|/Game/MenuSystemPro/Blueprints/SaveGame/MenuSettingsSaveGameBP.MenuSettingsSaveGameBP_C|GetRaytracedReflections (LocalVariables|GetSaveGame)) (Variables|/Game/MenuSystemPro/Blueprints/SaveGame/MenuSettingsSaveGameBP.MenuSettingsSaveGameBP_C|GetRaytracedTranslucency (LocalVariables|GetSaveGame)) (Variables|/Game/MenuSystemPro/Blueprints/SaveGame/MenuSettingsSaveGameBP.MenuSettingsSaveGameBP_C|GetRaytracedAmbientOcclusion (LocalVariables|GetSaveGame)) (Variables|/Game/MenuSystemPro/Blueprints/SaveGame/MenuSettingsSaveGameBP.MenuSettingsSaveGameBP_C|GetRaytracedGlobalIllumination (LocalVariables|GetSaveGame)) (Variables|/Game/MenuSystemPro/Blueprints/SaveGame/MenuSettingsSaveGameBP.MenuSettingsSaveGameBP_C|GetDLSS (LocalVariables|GetSaveGame))))))

(fn SetRaytracingSettings
  (params (RaytracedShadows :type Integer) (RaytracedReflections :type Integer) (RaytracedTranslucency :type Integer) (RaytracedAmbientOcclusion :type Integer) (RaytracedGlobalIllumination :type Integer) (DLSS :type Integer))
  (Utilities|FlowControl|Sequence
    (:then_0
      ;[1 1 1] Get Menu Settings Save Game instance
      (LocalVariables|SetSaveGame (CallFunction|GetSettingsSaveGame (LocalVariables|Get__WorldContext))))
    (:then_1
      ;[1 1 1] Set Variables
      (Utilities|FlowControl|Sequence
        (:then_0
          (Variables|/Game/MenuSystemPro/Blueprints/SaveGame/MenuSettingsSaveGameBP.MenuSettingsSaveGameBP_C|SetRaytracedShadows (LocalVariables|GetSaveGame) RaytracedShadows))
        (:then_1
          (Variables|/Game/MenuSystemPro/Blueprints/SaveGame/MenuSettingsSaveGameBP.MenuSettingsSaveGameBP_C|SetRaytracedReflections (LocalVariables|GetSaveGame) RaytracedReflections))
        (:then_2
          (Variables|/Game/MenuSystemPro/Blueprints/SaveGame/MenuSettingsSaveGameBP.MenuSettingsSaveGameBP_C|SetRaytracedTranslucency (LocalVariables|GetSaveGame) RaytracedTranslucency))
        (:then_3
          (Variables|/Game/MenuSystemPro/Blueprints/SaveGame/MenuSettingsSaveGameBP.MenuSettingsSaveGameBP_C|SetRaytracedAmbientOcclusion (LocalVariables|GetSaveGame) RaytracedAmbientOcclusion))
        (:then_4
          (Variables|/Game/MenuSystemPro/Blueprints/SaveGame/MenuSettingsSaveGameBP.MenuSettingsSaveGameBP_C|SetRaytracedGlobalIllumination (LocalVariables|GetSaveGame) RaytracedGlobalIllumination))
        (:then_5
          (Variables|/Game/MenuSystemPro/Blueprints/SaveGame/MenuSettingsSaveGameBP.MenuSettingsSaveGameBP_C|SetDLSS (LocalVariables|GetSaveGame) DLSS))))
    (:then_2
      ;[1 1 1] Save Settings to Save Game Slot
      (CallFunction|SaveSettingstoSlot (LocalVariables|GetSaveGame) (LocalVariables|Get__WorldContext)))
    (:then_3
      ;[1 1 1] Apply Raytracing Settings
      (CallFunction|ApplyRaytracingSettings RaytracedShadows RaytracedReflections RaytracedTranslucency RaytracedAmbientOcclusion RaytracedGlobalIllumination DLSS (LocalVariables|Get__WorldContext)))))

(fn ApplyRaytracingSettings
  (params (RaytracedShadows :type Integer) (RaytracedReflections :type Integer) (RaytracedTranslucency :type Integer) (RaytracedAmbientOcclusion :type Integer) (RaytracedGlobalIllumination :type Integer) (DLSS :type Integer))
  (Utilities|FlowControl|Sequence
    (:then_0
      ;[1 1 1] Raytraced Shadows
      (Development|ExecuteConsoleCommand (LocalVariables|Get__WorldContext) (Utilities|String|Append "r.RayTracing.Shadows " (Utilities|String|ToString(Integer) RaytracedShadows)) (Game|GetPlayerController (LocalVariables|Get__WorldContext))))
    (:then_1
      ;[1 1 1] Raytraced Reflections
      (Development|ExecuteConsoleCommand (LocalVariables|Get__WorldContext) (Utilities|String|Append "r.RayTracing.Reflections " (Utilities|String|ToString(Integer) RaytracedReflections)) (Game|GetPlayerController (LocalVariables|Get__WorldContext))))
    (:then_2
      ;[1 1 1] Raytraced Translucency
      (Development|ExecuteConsoleCommand (LocalVariables|Get__WorldContext) (Utilities|String|Append "r.RayTracing.Translucency " (Utilities|String|ToString(Integer) RaytracedTranslucency)) (Game|GetPlayerController (LocalVariables|Get__WorldContext))))
    (:then_3
      ;[1 1 1] Raytraced Ambient Occlusion
      (Development|ExecuteConsoleCommand (LocalVariables|Get__WorldContext) (Utilities|String|Append "r.RayTracing.AmbientOcclusion " (Utilities|String|ToString(Integer) RaytracedAmbientOcclusion)) (Game|GetPlayerController (LocalVariables|Get__WorldContext))))
    (:then_4
      ;[1 1 1] Raytraced Global Illumination
      (Development|ExecuteConsoleCommand (LocalVariables|Get__WorldContext) (Utilities|String|Append "r.RayTracing.GlobalIllumination  " (Utilities|String|ToString(Integer) RaytracedGlobalIllumination)) (Game|GetPlayerController (LocalVariables|Get__WorldContext))))
    (:then_5
      ;[1 1 1] DLSS - Enable Nvidia DLSS Plugin for this to work
      (Utilities|FlowControl|Sequence
        (:then_0
          (LocalVariables|SetDLSSEnable (Math|Integer|SelectInt 1 0 (> DLSS 0))))
        (:then_1
          (LocalVariables|SetDLSSQuality (Utilities|Select :Index DLSS :Option%200 0 :Option%201 -1 :Option%202 0 :Option%203 1 :Option%204 -2 :Option%205 2)))
        (:then_2
          (Development|ExecuteConsoleCommand (LocalVariables|Get__WorldContext) (Utilities|String|Append "r.NGX.DLSS.Enable " (Utilities|String|ToString(Integer) (LocalVariables|GetDLSSEnable))) (Game|GetPlayerController (LocalVariables|Get__WorldContext))))
        (:then_3
          (Development|ExecuteConsoleCommand (LocalVariables|Get__WorldContext) (Utilities|String|Append "r.NGX.DLSS.Quality " (Utilities|String|ToString(Integer) (LocalVariables|GetDLSSQuality))) (Game|GetPlayerController (LocalVariables|Get__WorldContext))))))))

(fn GetDisplaySettings
  (params (BrightnessDefault :type Float%20%28single-precision%29) (FieldOfViewDefault :type Float%20%28single-precision%29))
  (Utilities|FlowControl|Sequence
    (:then_0
      ;[1 1 1] Get Menu Settings Save Game instance
      (LocalVariables|SetSaveGame (CallFunction|GetSettingsSaveGame (LocalVariables|Get__WorldContext))))
    (:then_1
      ;[1 1 1] First Run: Set Variables from Default Values
      (if (Variables|/Game/MenuSystemPro/Blueprints/SaveGame/MenuSettingsSaveGameBP.MenuSettingsSaveGameBP_C|GetbDisplaySettingsFirstRun (LocalVariables|GetSaveGame)) ; Is first run?
        (Utilities|FlowControl|Sequence
          (:then_0
            (Variables|/Game/MenuSystemPro/Blueprints/SaveGame/MenuSettingsSaveGameBP.MenuSettingsSaveGameBP_C|SetBrightness (LocalVariables|GetSaveGame) BrightnessDefault))
          (:then_1
            (Variables|/Game/MenuSystemPro/Blueprints/SaveGame/MenuSettingsSaveGameBP.MenuSettingsSaveGameBP_C|SetFieldOfView (LocalVariables|GetSaveGame) FieldOfViewDefault))
          (:then_2
            (Variables|/Game/MenuSystemPro/Blueprints/SaveGame/MenuSettingsSaveGameBP.MenuSettingsSaveGameBP_C|SetbDisplaySettingsFirstRun (LocalVariables|GetSaveGame) false))
          (:then_3
            (CallFunction|SaveSettingstoSlot (LocalVariables|GetSaveGame) (LocalVariables|Get__WorldContext))))))
    (:then_2
      ;[1 1 1] Get Display Settings from Settings Save Game
      (return (Variables|/Game/MenuSystemPro/Blueprints/SaveGame/MenuSettingsSaveGameBP.MenuSettingsSaveGameBP_C|GetBrightness (LocalVariables|GetSaveGame)) (Variables|/Game/MenuSystemPro/Blueprints/SaveGame/MenuSettingsSaveGameBP.MenuSettingsSaveGameBP_C|GetFieldOfView (LocalVariables|GetSaveGame))))))

(fn SetDisplaySettings
  (params (Brightness :type Float%20%28single-precision%29) (FieldOfView :type Float%20%28single-precision%29))
  (Utilities|FlowControl|Sequence
    (:then_0
      ;[1 1 1] Get Menu Settings Save Game instance
      (LocalVariables|SetSaveGame (CallFunction|GetSettingsSaveGame (LocalVariables|Get__WorldContext))))
    (:then_1
      ;[1 1 1] Set Variables
      (Utilities|FlowControl|Sequence
        (:then_0
          (Variables|/Game/MenuSystemPro/Blueprints/SaveGame/MenuSettingsSaveGameBP.MenuSettingsSaveGameBP_C|SetBrightness (LocalVariables|GetSaveGame) Brightness))
        (:then_1
          (Variables|/Game/MenuSystemPro/Blueprints/SaveGame/MenuSettingsSaveGameBP.MenuSettingsSaveGameBP_C|SetFieldOfView (LocalVariables|GetSaveGame) FieldOfView))))
    (:then_2
      ;[1 1 1] Save Settings to Save Game Slot
      (CallFunction|SaveSettingstoSlot (LocalVariables|GetSaveGame) (LocalVariables|Get__WorldContext)))))

(fn SetAudioSettings
  (params (MasterAudioVolume :type Float%20%28single-precision%29) (MusicAudioVolume :type Float%20%28single-precision%29) (SFXAudioVolume :type Float%20%28single-precision%29) (VoiceAudioVolume :type Float%20%28single-precision%29) (MasterSoundClass :type Sound%20Class%20Object%20Reference) (MusicSoundClass :type Sound%20Class%20Object%20Reference) (SFXSoundClass :type Sound%20Class%20Object%20Reference) (VoiceSoundClass :type Sound%20Class%20Object%20Reference))
  (Utilities|FlowControl|Sequence
    (:then_0
      ;[1 1 1] Get Menu Settings Save Game instance
      (LocalVariables|SetSaveGame (CallFunction|GetSettingsSaveGame (LocalVariables|Get__WorldContext))))
    (:then_1
      ;[1 1 1] Set Variables
      (Utilities|FlowControl|Sequence
        (:then_0
          (bind _output_get (Variables|/Game/MenuSystemPro/Blueprints/SaveGame/MenuSettingsSaveGameBP.MenuSettingsSaveGameBP_C|SetMasterAudioVolume (LocalVariables|GetSaveGame) MasterAudioVolume))
          (CallFunction|SetSoundClassVolumeProperty MasterSoundClass _output_get (LocalVariables|Get__WorldContext)))
        (:then_1
          (bind _output_get_2 (Variables|/Game/MenuSystemPro/Blueprints/SaveGame/MenuSettingsSaveGameBP.MenuSettingsSaveGameBP_C|SetMusicAudioVolume (LocalVariables|GetSaveGame) MusicAudioVolume))
          (CallFunction|SetSoundClassVolumeProperty MusicSoundClass _output_get_2 (LocalVariables|Get__WorldContext)))
        (:then_2
          (bind _output_get_3 (Variables|/Game/MenuSystemPro/Blueprints/SaveGame/MenuSettingsSaveGameBP.MenuSettingsSaveGameBP_C|SetSFXAudioVolume (LocalVariables|GetSaveGame) SFXAudioVolume))
          (CallFunction|SetSoundClassVolumeProperty SFXSoundClass _output_get_3 (LocalVariables|Get__WorldContext)))
        (:then_3
          (bind _output_get_4 (Variables|/Game/MenuSystemPro/Blueprints/SaveGame/MenuSettingsSaveGameBP.MenuSettingsSaveGameBP_C|SetVoiceAudioVolume (LocalVariables|GetSaveGame) VoiceAudioVolume))
          (CallFunction|SetSoundClassVolumeProperty VoiceSoundClass _output_get_4 (LocalVariables|Get__WorldContext)))))
    (:then_2
      ;[1 1 1] Save Settings to Save Game Slot
      (CallFunction|SaveSettingstoSlot (LocalVariables|GetSaveGame) (LocalVariables|Get__WorldContext)))))

(fn GetAudioSettings
  (params (MasterAudioVolumeDefault :type Float%20%28single-precision%29) (MusicAudioVolumeDefault :type Float%20%28single-precision%29) (SFXAudioVolumeDefault :type Float%20%28single-precision%29) (VoiceAudioVolumeDefault :type Float%20%28single-precision%29))
  (Utilities|FlowControl|Sequence
    (:then_0
      ;[1 1 1] Get Menu Settings Save Game instance
      (LocalVariables|SetSaveGame (CallFunction|GetSettingsSaveGame (LocalVariables|Get__WorldContext))))
    (:then_1
      ;[1 1 1] First Run: Set Variables from Default Values
      (if (Variables|/Game/MenuSystemPro/Blueprints/SaveGame/MenuSettingsSaveGameBP.MenuSettingsSaveGameBP_C|GetbAudioSettingsFirstRun (LocalVariables|GetSaveGame)) ; Is first run?
        (Utilities|FlowControl|Sequence
          (:then_0
            (Variables|/Game/MenuSystemPro/Blueprints/SaveGame/MenuSettingsSaveGameBP.MenuSettingsSaveGameBP_C|SetMasterAudioVolume (LocalVariables|GetSaveGame) MasterAudioVolumeDefault))
          (:then_1
            (Variables|/Game/MenuSystemPro/Blueprints/SaveGame/MenuSettingsSaveGameBP.MenuSettingsSaveGameBP_C|SetMusicAudioVolume (LocalVariables|GetSaveGame) MusicAudioVolumeDefault))
          (:then_2
            (Variables|/Game/MenuSystemPro/Blueprints/SaveGame/MenuSettingsSaveGameBP.MenuSettingsSaveGameBP_C|SetSFXAudioVolume (LocalVariables|GetSaveGame) SFXAudioVolumeDefault))
          (:then_3
            (Variables|/Game/MenuSystemPro/Blueprints/SaveGame/MenuSettingsSaveGameBP.MenuSettingsSaveGameBP_C|SetVoiceAudioVolume (LocalVariables|GetSaveGame) VoiceAudioVolumeDefault))
          (:then_4
            (Variables|/Game/MenuSystemPro/Blueprints/SaveGame/MenuSettingsSaveGameBP.MenuSettingsSaveGameBP_C|SetbAudioSettingsFirstRun (LocalVariables|GetSaveGame) false))
          (:then_5
            (CallFunction|SaveSettingstoSlot (LocalVariables|GetSaveGame) (LocalVariables|Get__WorldContext))))))
    (:then_2
      ;[1 1 1] Get Audio Settings from Settings Save Game
      (return (Variables|/Game/MenuSystemPro/Blueprints/SaveGame/MenuSettingsSaveGameBP.MenuSettingsSaveGameBP_C|GetMasterAudioVolume (LocalVariables|GetSaveGame)) (Variables|/Game/MenuSystemPro/Blueprints/SaveGame/MenuSettingsSaveGameBP.MenuSettingsSaveGameBP_C|GetMusicAudioVolume (LocalVariables|GetSaveGame)) (Variables|/Game/MenuSystemPro/Blueprints/SaveGame/MenuSettingsSaveGameBP.MenuSettingsSaveGameBP_C|GetSFXAudioVolume (LocalVariables|GetSaveGame)) (Variables|/Game/MenuSystemPro/Blueprints/SaveGame/MenuSettingsSaveGameBP.MenuSettingsSaveGameBP_C|GetVoiceAudioVolume (LocalVariables|GetSaveGame))))))

(fn SetSoundClassVolumeProperty
  (params (SoundClass :type Sound%20Class%20Object%20Reference) (VolumeValue :type Float%20%28single-precision%29))
  (Audio|SetSoundMixClassOverride (LocalVariables|Get__WorldContext) "/Game/MenuSystemPro/Sounds/MenuSoundMix.MenuSoundMix" SoundClass VolumeValue (.pitch (Variables|/Script/Engine.SoundClass|GetProperties SoundClass)) 0.1 true)
  (Audio|PushSoundMixModifier 0 "/Game/MenuSystemPro/Sounds/MenuSoundMix.MenuSoundMix"))

(fn GetGameSettings
  (params (DifficultyDefault :type Integer) (LanguageDefault :type Integer) (SubtitlesEnabledDefault :type Boolean))
  (Utilities|FlowControl|Sequence
    (:then_0
      ;[1 1 1] Get Menu Settings Save Game instance
      (LocalVariables|SetSaveGame (CallFunction|GetSettingsSaveGame (LocalVariables|Get__WorldContext))))
    (:then_1
      ;[1 1 1] First Run: Set Variables from Default Values
      (if (Variables|/Game/MenuSystemPro/Blueprints/SaveGame/MenuSettingsSaveGameBP.MenuSettingsSaveGameBP_C|GetbGameSettingsFirstRun (LocalVariables|GetSaveGame)) ; Is first run?
        (Utilities|FlowControl|Sequence
          (:then_0
            (Variables|/Game/MenuSystemPro/Blueprints/SaveGame/MenuSettingsSaveGameBP.MenuSettingsSaveGameBP_C|SetDifficulty (LocalVariables|GetSaveGame) DifficultyDefault))
          (:then_1
            (Variables|/Game/MenuSystemPro/Blueprints/SaveGame/MenuSettingsSaveGameBP.MenuSettingsSaveGameBP_C|SetLanguage (LocalVariables|GetSaveGame) LanguageDefault))
          (:then_2
            (Variables|/Game/MenuSystemPro/Blueprints/SaveGame/MenuSettingsSaveGameBP.MenuSettingsSaveGameBP_C|SetSubtitlesEnabled (LocalVariables|GetSaveGame) SubtitlesEnabledDefault))
          (:then_3
            (Variables|/Game/MenuSystemPro/Blueprints/SaveGame/MenuSettingsSaveGameBP.MenuSettingsSaveGameBP_C|SetbGameSettingsFirstRun (LocalVariables|GetSaveGame) false))
          (:then_4
            (CallFunction|SaveSettingstoSlot (LocalVariables|GetSaveGame) (LocalVariables|Get__WorldContext))))))
    (:then_2
      ;[1 1 1] Get Game Settings from Settings Save Game
      (return (Variables|/Game/MenuSystemPro/Blueprints/SaveGame/MenuSettingsSaveGameBP.MenuSettingsSaveGameBP_C|GetDifficulty (LocalVariables|GetSaveGame)) (Variables|/Game/MenuSystemPro/Blueprints/SaveGame/MenuSettingsSaveGameBP.MenuSettingsSaveGameBP_C|GetLanguage (LocalVariables|GetSaveGame)) (Variables|/Game/MenuSystemPro/Blueprints/SaveGame/MenuSettingsSaveGameBP.MenuSettingsSaveGameBP_C|GetSubtitlesEnabled (LocalVariables|GetSaveGame)) (CallFunction|GetLanguageCodeArray (LocalVariables|Get__WorldContext))))))

(fn SetGameSettings
  (params (Difficulty :type Integer) (Language :type Integer) (SubtitlesEnabled :type Boolean))
  (Utilities|FlowControl|Sequence
    (:then_0
      ;[1 1 1] Get Menu Settings Save Game instance
      (LocalVariables|SetSaveGame (CallFunction|GetSettingsSaveGame (LocalVariables|Get__WorldContext))))
    (:then_1
      ;[1 1 1] Set Variables
      (Utilities|FlowControl|Sequence
        (:then_0
          (Variables|/Game/MenuSystemPro/Blueprints/SaveGame/MenuSettingsSaveGameBP.MenuSettingsSaveGameBP_C|SetDifficulty (LocalVariables|GetSaveGame) Difficulty))
        (:then_1
          (Variables|/Game/MenuSystemPro/Blueprints/SaveGame/MenuSettingsSaveGameBP.MenuSettingsSaveGameBP_C|SetLanguage (LocalVariables|GetSaveGame) Language))
        (:then_2
          (Variables|/Game/MenuSystemPro/Blueprints/SaveGame/MenuSettingsSaveGameBP.MenuSettingsSaveGameBP_C|SetSubtitlesEnabled (LocalVariables|GetSaveGame) SubtitlesEnabled))))
    (:then_2
      ;[1 1 1] Save Settings to Save Game Slot
      (CallFunction|SaveSettingstoSlot (LocalVariables|GetSaveGame) (LocalVariables|Get__WorldContext)))))

(fn SetControlsSettings
  (params (InvertLookX :type Boolean) (InvertLookY :type Boolean) (CameraSpeedX :type Float%20%28single-precision%29) (CameraSpeedY :type Float%20%28single-precision%29) (Rumble :type Boolean))
  (Utilities|FlowControl|Sequence
    (:then_0
      ;[1 1 1] Get Menu Settings Save Game instance
      (LocalVariables|SetSaveGame (CallFunction|GetSettingsSaveGame (LocalVariables|Get__WorldContext))))
    (:then_1
      ;[1 1 1] Set Variables
      (Utilities|FlowControl|Sequence
        (:then_0
          (Variables|/Game/MenuSystemPro/Blueprints/SaveGame/MenuSettingsSaveGameBP.MenuSettingsSaveGameBP_C|SetInvertLookX (LocalVariables|GetSaveGame) InvertLookX))
        (:then_1
          (Variables|/Game/MenuSystemPro/Blueprints/SaveGame/MenuSettingsSaveGameBP.MenuSettingsSaveGameBP_C|SetInvertLookY (LocalVariables|GetSaveGame) InvertLookY))
        (:then_2
          (Variables|/Game/MenuSystemPro/Blueprints/SaveGame/MenuSettingsSaveGameBP.MenuSettingsSaveGameBP_C|SetCameraSpeedX (LocalVariables|GetSaveGame) CameraSpeedX))
        (:then_3
          (Variables|/Game/MenuSystemPro/Blueprints/SaveGame/MenuSettingsSaveGameBP.MenuSettingsSaveGameBP_C|SetCameraSpeedY (LocalVariables|GetSaveGame) CameraSpeedY))
        (:then_4
          (Variables|/Game/MenuSystemPro/Blueprints/SaveGame/MenuSettingsSaveGameBP.MenuSettingsSaveGameBP_C|SetRumble (LocalVariables|GetSaveGame) Rumble))))
    (:then_2
      ;[1 1 1] Save Settings to Save Game Slot
      (CallFunction|SaveSettingstoSlot (LocalVariables|GetSaveGame) (LocalVariables|Get__WorldContext)))))

(fn GetControlsSettings
  (params (InvertLookXDefault :type Boolean) (InvertLookYDefault :type Boolean) (CameraSpeedXDefault :type Float%20%28single-precision%29) (CameraSpeedYDefault :type Float%20%28single-precision%29) (RumbleDefault :type Boolean))
  (Utilities|FlowControl|Sequence
    (:then_0
      ;[1 1 1] Get Menu Settings Save Game instance
      (LocalVariables|SetSaveGame (CallFunction|GetSettingsSaveGame (LocalVariables|Get__WorldContext))))
    (:then_1
      ;[1 1 1] First Run: Set Variables from Default Values
      (if (Variables|/Game/MenuSystemPro/Blueprints/SaveGame/MenuSettingsSaveGameBP.MenuSettingsSaveGameBP_C|GetbControlsSettingsFirstRun (LocalVariables|GetSaveGame)) ; Is first run?
        (Utilities|FlowControl|Sequence
          (:then_0
            (Variables|/Game/MenuSystemPro/Blueprints/SaveGame/MenuSettingsSaveGameBP.MenuSettingsSaveGameBP_C|SetInvertLookX (LocalVariables|GetSaveGame) InvertLookXDefault))
          (:then_1
            (Variables|/Game/MenuSystemPro/Blueprints/SaveGame/MenuSettingsSaveGameBP.MenuSettingsSaveGameBP_C|SetInvertLookY (LocalVariables|GetSaveGame) InvertLookYDefault))
          (:then_2
            (Variables|/Game/MenuSystemPro/Blueprints/SaveGame/MenuSettingsSaveGameBP.MenuSettingsSaveGameBP_C|SetCameraSpeedX (LocalVariables|GetSaveGame) CameraSpeedXDefault))
          (:then_3
            (Variables|/Game/MenuSystemPro/Blueprints/SaveGame/MenuSettingsSaveGameBP.MenuSettingsSaveGameBP_C|SetCameraSpeedY (LocalVariables|GetSaveGame) CameraSpeedYDefault))
          (:then_4
            (Variables|/Game/MenuSystemPro/Blueprints/SaveGame/MenuSettingsSaveGameBP.MenuSettingsSaveGameBP_C|SetRumble (LocalVariables|GetSaveGame) RumbleDefault))
          (:then_5
            (Variables|/Game/MenuSystemPro/Blueprints/SaveGame/MenuSettingsSaveGameBP.MenuSettingsSaveGameBP_C|SetbControlsSettingsFirstRun (LocalVariables|GetSaveGame) false))
          (:then_6
            (CallFunction|SaveSettingstoSlot (LocalVariables|GetSaveGame) (LocalVariables|Get__WorldContext))))))
    (:then_2
      ;[1 1 1] Get Controls Settings from Settings Save Game
      (return (Variables|/Game/MenuSystemPro/Blueprints/SaveGame/MenuSettingsSaveGameBP.MenuSettingsSaveGameBP_C|GetInvertLookX (LocalVariables|GetSaveGame)) (Variables|/Game/MenuSystemPro/Blueprints/SaveGame/MenuSettingsSaveGameBP.MenuSettingsSaveGameBP_C|GetInvertLookY (LocalVariables|GetSaveGame)) (Variables|/Game/MenuSystemPro/Blueprints/SaveGame/MenuSettingsSaveGameBP.MenuSettingsSaveGameBP_C|GetCameraSpeedX (LocalVariables|GetSaveGame)) (Variables|/Game/MenuSystemPro/Blueprints/SaveGame/MenuSettingsSaveGameBP.MenuSettingsSaveGameBP_C|GetCameraSpeedY (LocalVariables|GetSaveGame)) (Variables|/Game/MenuSystemPro/Blueprints/SaveGame/MenuSettingsSaveGameBP.MenuSettingsSaveGameBP_C|GetRumble (LocalVariables|GetSaveGame))))))

(fn SetLanguageCodeArray
  (params (LanguageCodeArray :type Array%20of%20Strings))
  (bind _output_get (LocalVariables|SetSaveGame (CallFunction|GetSettingsSaveGame (LocalVariables|Get__WorldContext))))
  (Variables|/Game/MenuSystemPro/Blueprints/SaveGame/MenuSettingsSaveGameBP.MenuSettingsSaveGameBP_C|SetLanguageCodeArray _output_get LanguageCodeArray)
  (CallFunction|SaveSettingstoSlot _output_get (LocalVariables|Get__WorldContext)))

(fn GetLanguageCodeArray
  (return (Variables|/Game/MenuSystemPro/Blueprints/SaveGame/MenuSettingsSaveGameBP.MenuSettingsSaveGameBP_C|GetLanguageCodeArray (CallFunction|GetSettingsSaveGame (LocalVariables|Get__WorldContext)))))