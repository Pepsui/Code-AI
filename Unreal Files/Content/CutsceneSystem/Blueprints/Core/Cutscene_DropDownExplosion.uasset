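; A cutscene bomb actor that, after a delay, launches by projectile movement, signals its owner the scene is complete, and explodes on hit.
; The explosion can ragdoll nearby characters and make static mesh actors simulate physics, then fires particles and radial force at a preset strength.
; It optionally plays sound, applies radial damage and later destroys affected actors and itself.
; The construction script applies radius, size, speed, color, visibility and particle settings.
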(event Custom|ExplosionStart
  (params (WaitForExplode :type Float%20%28single-precision%29) (SimulatePhysicsForNearbyObjects :type Boolean) (SimulatePhysicsForNearbyCharacters :type Boolean) (DestroySimulatedActorsSec :type Float%20%28single-precision%29) (DamageToActors :type Boolean) (DamageValue :type Float%20%28single-precision%29) (Sound :type Sound%20Cue%20Object%20Reference) (CutsceneOwner :type Cutscene%20Tool%20Object%20Reference))
  ;[1 1 1] Activate Bomb and Complete Scene
  (Utilities|FlowControl|Delay WaitForExplode)
  (Components|Activation|Activate (Variables|Default|GetProjectileMovement) false)
  (Default|SceneComplete CutsceneOwner))

(event Custom|ExplosionCalculate
  (bind _radialforce (Variables|Default|GetRadialForce))
  ;[1 1 1] Play Sound On Location
  (Utilities|IsValid (stale Custom|ExplosionStart Sound)
    (:Is%20Valid
      (Audio|PlaySoundatLocation (stale Custom|ExplosionStart Sound) (Transformation|GetWorldLocation (Variables|Default|GetSphere)) "0, 0, 0" 1.0 1.0 0.0 0 0 0))
    (:Is%20Not%20Valid
      _))
  ;[1 1 1] Object Physics Explosion
  (if (stale Custom|ExplosionStart SimulatePhysicsForNearbyObjects)
    (bind _outactors (Collision|SphereOverlapActors (Transformation|GetWorldLocation (Variables|Default|GetAreaCalculate)) (Variables|Default|GetEffectedArea) (Utilities|Array|MakeArray "ObjectTypeQuery2") 0))
    (for _array_element _outactors
      (Utilities|Array|Add (Variables|Default|GetExplodedActors) _array_element)
      (bind _asstatic_mesh_actor (Utilities|Casting|CastToStaticMeshActor _array_element))
      (Physics|SetSimulatePhysics (Variables|/Script/Engine.StaticMeshActor|GetStaticMeshComponent _asstatic_mesh_actor) true)
      (Collision|SetCollisionProfileName (Variables|/Script/Engine.StaticMeshActor|GetStaticMeshComponent _asstatic_mesh_actor) "PhysicsActor" true :!class /Script/Engine.PrimitiveComponent)
      (Class|PrimitiveComponent|SetMassOverrideinKg (Variables|/Script/Engine.StaticMeshActor|GetStaticMeshComponent _asstatic_mesh_actor) "None" 1.0 true))
    ;[1 1 1] Character Physics Explosion
    (bind _outactors_2 (Collision|SphereOverlapActors (Transformation|GetWorldLocation (Variables|Default|GetAreaCalculate)) (Variables|Default|GetEffectedArea) (Utilities|Array|MakeArray "ObjectTypeQuery3") 0 :!label _label))
    (for _array_element_2 _outactors_2
      (Utilities|Array|Add (Variables|Default|GetExplodedActors) _array_element_2)
      (bind _ascharacter (Utilities|Casting|CastToCharacter _array_element_2))
      (Physics|SetSimulatePhysics (Variables|/Script/Engine.Character|GetMesh _ascharacter) true)
      (Collision|SetCollisionProfileName (Variables|/Script/Engine.Character|GetMesh _ascharacter) "Ragdoll" true :!class /Script/Engine.PrimitiveComponent)
      (Class|PrimitiveComponent|SetMassOverrideinKg (Variables|/Script/Engine.Character|GetMesh _ascharacter) "None" 1.0 true))
    ;[1 1 1] Explosion Strength
    (switch Utilities|FlowControl|Switch|SwitchonCutscene_ExplosionStrength (Variables|Default|GetExplosionStrength)
      (:NewEnumerator0
        (Variables|/Script/Engine.RadialForceComponent|SetForceStrength _radialforce 3e+03))
      (:NewEnumerator1
        (Variables|/Script/Engine.RadialForceComponent|SetForceStrength _radialforce 1e+05))
      (:NewEnumerator2
        (Variables|/Script/Engine.RadialForceComponent|SetForceStrength _radialforce 1e+06)))
    ;[1 1 1] Activate Particle Effect and Radial Force
    (Components|Activation|Activate (Variables|Default|GetParticleSystem) false)
    (Components|Activation|Activate (Variables|Default|GetRadialForce) false)
    (Utilities|FlowControl|Sequence
      (:then_0
        ;[1 1 1] Apply Damage
        (if (stale Custom|ExplosionStart DamageToActors)
          (Game|Damage|ApplyRadialDamage (stale Custom|ExplosionStart DamageValue) (Transformation|GetWorldLocation (Variables|Default|GetAreaCalculate)) (Variables|Default|GetEffectedArea) 0 0 0 0 false "ECC_Visibility")))
      (:then_1
        ;[1 1 1] Destroy Actors After Explosion
        (if (> (stale Custom|ExplosionStart DestroySimulatedActorsSec) 0.0)
          (Utilities|FlowControl|Delay (stale Custom|ExplosionStart DestroySimulatedActorsSec))
          (for _array_element_3 (Variables|Default|GetExplodedActors)
            (Utilities|IsValid _array_element_3
              (:Is%20Valid
                (Actor|DestroyActor _array_element_3))))
          (Actor|DestroyActor))))
    (elif (stale Custom|ExplosionStart SimulatePhysicsForNearbyCharacters)
      (goto _label))))

(event Collision|EventHit
  (params (MyComp :type Primitive%20Component%20Object%20Reference) (Other :type Actor%20Object%20Reference) (OtherComp :type Primitive%20Component%20Object%20Reference) (bSelfMoved :type Boolean) (HitLocation :type Vector :default "0, 0, 0") (HitNormal :type Vector :default "0, 0, 0") (NormalImpulse :type Vector :default "0, 0, 0") (Hit :type Hit%20Result%20Structure%20%28by%20ref%29))
  (bind _sphere (Variables|Default|GetSphere))
  ;[1 1 1] When Bomb hit something, Explosion Start
  (CallFunction|ExplosionCalculate)
  (Utilities|IsValid _sphere
    (:Is%20Valid
      (Rendering|SetVisibility _sphere false false))))

(fn ConstructionScript
  ;[1 1 1] EffectArea
  (bind _output_get (Variables|/Script/Engine.RadialForceComponent|SetRadius (Variables|Default|GetRadialForce) (Variables|Default|GetEffectedArea)))
  (Components|Sphere|SetSphereRadius (Variables|Default|GetAreaCalculate) _output_get true)
  ;[1 1 1] BombSize
  (Transformation|SetRelativeTransform (Variables|Default|GetSphere) (Math|Transform|MakeTransform "0, 0, 0" "0, 0, 0" (Math|Conversions|ToVector(Float) (* (Variables|Default|GetBombSize) 1.0))) false false)
  ;[1 1 1] BombSpeed
  (Variables|/Script/Engine.ProjectileMovementComponent|SetMaxSpeed (Variables|Default|GetProjectileMovement) (* (Variables|Default|GetBombSpeed) 1e+03))
  ;[1 1 1] BombColor
  (bind _returnvalue (Rendering|Material|CreateDynamicMaterialInstance (Variables|Default|GetSphere) 0 "/Game/CutsceneSystem/Assets/Materials/Cutscene_Purple.Cutscene_Purple" "" :!class /Script/Engine.PrimitiveComponent))
  (Rendering|Material|SetVectorParameterValue _returnvalue "Color" (Variables|Default|GetBombColor) :!class /Script/Engine.MaterialInstanceDynamic)
  ;[1 1 1] BombHiddenInGame
  (Development|SetHiddeninGame (Variables|Default|GetSphere) (Variables|Default|GetBombHiddenInGame) false)
  ;[1 1 1] BombParticleEffect
  (Effects|Components|ParticleSystem|SetTemplate (Variables|Default|GetBombParticle) (Variables|Default|GetUseParticleEffectCoverBomb)))