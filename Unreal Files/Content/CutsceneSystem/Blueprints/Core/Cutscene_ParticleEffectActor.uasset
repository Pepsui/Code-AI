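; A cutscene actor that plays a particle effect, with optional sound, as one step of a scene.
; StartParticleEffect sets the particle system template, waits the given delay, activates it, plays any valid sound at the Cylinder's location, then calls SceneComplete on the cutscene owner.
; The construction script scales the Cylinder component uniformly from ParticleEffectSize.
; The RemoveParticleEndOfTheScene input is not used in this graph.
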(event Custom|StartParticleEffect
  (params (ParticleEffect :type Particle%20System%20Object%20Reference) (Delay :type Float%20%28single-precision%29) (Remove%20Particle%20End%20of%20The%20Scene? :type Boolean) (Sound :type Sound%20Cue%20Object%20Reference) (CutsceneOwner :type Cutscene%20Tool%20Object%20Reference))
  ;[1 1 1] Set Template for Particle Effect
  (Effects|Components|ParticleSystem|SetTemplate (Variables|Default|GetParticleSystem) ParticleEffect)
  (Utilities|FlowControl|Delay Delay)
  ;[1 1 1] Activate It
  (Components|Activation|Activate (Variables|Default|GetParticleSystem) false)
  ;[1 1 1] If there is a sound play it
  (Utilities|IsValid Sound
    (:Is%20Valid
      (Audio|PlaySoundatLocation Sound (Transformation|GetWorldLocation (Variables|Default|GetCylinder)) "0, 0, 0" 1.0 1.0 0.0 0 0 0))
    (:Is%20Not%20Valid
      _))
  (Default|SceneComplete CutsceneOwner))

(fn ConstructionScript
  (Transformation|SetRelativeTransform (Variables|Default|GetCylinder) (Math|Transform|MakeTransform "0, 0, 0" "0, 0, 0" (Math|Conversions|ToVector(Float) (* (Variables|Default|GetParticleEffectSize) 1.0))) false false))