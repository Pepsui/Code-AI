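; Cutscene explosion actor that, after a delay, hides its sphere, completes the owner's scene and plays an optional sound.
; Sphere overlaps within EffectedArea turn static mesh actors into physics bodies and characters into ragdolls; enabling object physics always includes characters.
; That physics path then fires particles and a strength-tiered radial force, with optional radial damage and delayed destruction of overlapped actors and itself.
; The construction script syncs force and preview radii to EffectedArea.
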(event Custom|ExplosionStart
  (params (WaitForExplode :type Float%20%28single-precision%29) (SimulatePhysicsForNearbyObjects :type Boolean) (SimulatePhysicsForNearbyCharacters :type Boolean) (DestroySimulatedActorsSec :type Float%20%28single-precision%29) (DamageToActors :type Boolean) (DamageValue :type Float%20%28single-precision%29) (Sound :type Sound%20Cue%20Object%20Reference) (CutsceneOwner :type Cutscene%20Tool%20Object%20Reference))
  (bind _radialforce (Variables|Default|GetRadialForce))
  (Utilities|FlowControl|Delay WaitForExplode)
  ;[1 1 1] Move to Next Scene
  (Rendering|SetVisibility (Variables|Default|GetSphere) false false)
  (Default|SceneComplete CutsceneOwner)
  ;[1 1 1] Play Sound On Location
  (Utilities|IsValid Sound
    (:Is%20Valid
      (Audio|PlaySoundatLocation Sound (Transformation|GetWorldLocation (Variables|Default|GetSphere)) "0, 0, 0" 1.0 1.0 0.0 0 0 0))
    (:Is%20Not%20Valid
      _))
  ;[1 1 1] Object Physics Explosion
  (if SimulatePhysicsForNearbyObjects
    (bind _outactors (Collision|SphereOverlapActors (Transformation|GetWorldLocation (Variables|Default|GetAreaCalculate)) (Variables|Default|GetEffectedArea) (Utilities|Array|MakeArray "ObjectTypeQuery2") 0))
    (for _array_element _outactors
      (Utilities|Array|Add (Variables|Default|GetExplodedActors) _array_element)
      (bind _asstatic_mesh_actor (Utilities|Casting|CastToStaticMeshActor _array_element))
      (Physics|SetSimulatePhysics (Variables|/Script/Engine.StaticMeshActor|GetStaticMeshComponent _asstatic_mesh_actor) true)
      (Collision|SetCollisionProfileName (Variables|/Script/Engine.StaticMeshActor|GetStaticMeshComponent _asstatic_mesh_actor) "PhysicsActor" true :!class /Script/Engine.PrimitiveComponent)
      (Class|PrimitiveComponent|SetMassOverrideinKg (Variables|/Script/Engine.StaticMeshActor|GetStaticMeshComponent _asstatic_mesh_actor) "None" 1.0 true))
    ;[1 1 1] Character Physics Explosion
    (bind _outactors_2 (Collision|SphereOverlapActors (Transformation|GetWorldLocation (Variables|Default|GetAreaCalculate)) (Variables|Default|GetEffectedArea) (Utilities|Array|MakeArray "ObjectTypeQuery3") 0 :!label _label))
    (for _array_element_2 _outactors_2
      (Utilities|Array|Add (Variables|Default|GetExplodedActors) _array_element_2)
      (bind _ascharacter (Utilities|Casting|CastToCharacter _array_element_2))
      (Physics|SetSimulatePhysics (Variables|/Script/Engine.Character|GetMesh _ascharacter) true)
      (Collision|SetCollisionProfileName (Variables|/Script/Engine.Character|GetMesh _ascharacter) "Ragdoll" true :!class /Script/Engine.PrimitiveComponent)
      (Class|PrimitiveComponent|SetMassOverrideinKg (Variables|/Script/Engine.Character|GetMesh _ascharacter) "None" 1.0 true))
    ;[1 1 1] Explosion Strength
    (switch Utilities|FlowControl|Switch|SwitchonCutscene_ExplosionStrength (Variables|Default|GetExplosionStrength)
      (:NewEnumerator0
        (Variables|/Script/Engine.RadialForceComponent|SetForceStrength _radialforce 3e+03))
      (:NewEnumerator1
        (Variables|/Script/Engine.RadialForceComponent|SetForceStrength _radialforce 1e+05))
      (:NewEnumerator2
        (Variables|/Script/Engine.RadialForceComponent|SetForceStrength _radialforce 1e+06)))
    ;[1 1 1] Activate Particle System and Radial Force
    (Components|Activation|Activate (Variables|Default|GetParticleSystem) false)
    (Components|Activation|Activate (Variables|Default|GetRadialForce) false)
    (Utilities|FlowControl|Sequence
      (:then_0
        ;[1 1 1] Apply Damage
        (if DamageToActors
          (Game|Damage|ApplyRadialDamage DamageValue (Transformation|GetWorldLocation (Variables|Default|GetAreaCalculate)) (Variables|Default|GetEffectedArea) 0 0 0 0 false "ECC_Visibility")))
      (:then_1
        ;[1 1 1] Destroy Actors After Explosion
        (if (> DestroySimulatedActorsSec 0.0)
          (Utilities|FlowControl|Delay DestroySimulatedActorsSec)
          (for _array_element_3 (Variables|Default|GetExplodedActors)
            (Utilities|IsValid _array_element_3
              (:Is%20Valid
                (Actor|DestroyActor _array_element_3))))
          (Actor|DestroyActor))))
    (elif SimulatePhysicsForNearbyCharacters
      (goto _label))))

(fn ConstructionScript
  (bind _output_get (Variables|/Script/Engine.RadialForceComponent|SetRadius (Variables|Default|GetRadialForce) (Variables|Default|GetEffectedArea)))
  (Components|Sphere|SetSphereRadius (Variables|Default|GetAreaCalculate) _output_get true))