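; Cutscene rail camera that travels along its rail during a scene of the cutscene system.
; CameraStart stores the owning cutscene, then loops on a short Delay rather than Tick or a Timeline to advance CurrentPositionOnRail.
; Each step's size derives from SecondToComplete through a clamped range mapping, so it is not scaled by delta time.
; At the rail's end, it calls SceneComplete on the owner if the MoveToNextSceneOption setting matches.
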(event Custom|CameraStart
  (params (OwnerCutscene :type Cutscene%20Tool%20Object%20Reference) (CutsceneSettings :type Cutscene%20Settings%20Structure))
  (bind _secondtocomplete (Variables|CutsceneCameraSettings|GetSecondToComplete))
  (bind _returnvalue (Math|Conversions|ToFloat(Integer) _secondtocomplete))
  (Variables|Default|SetOwner%20Cutscene OwnerCutscene)
  (bind _output_get (Variables|Default|SetCurrentPositionOnRail (+ (Variables|Default|GetCurrentPositionOnRail) (/ (Math|Float|MapRangeClamped _returnvalue (Variables|Default|GetCurrentPositionOnRail) (* _secondtocomplete 6e+01) 0.0 1.0) _returnvalue)) :!label _label))
  (if (< _output_get 1.0)
    (Utilities|FlowControl|Delay 0.01)
    (goto _label)
    (elif (Utilities|Enum|Equal(Enum) (.MoveToNextSceneOption (Utilities|Struct|BreakCutscene_Settings CutsceneSettings)) "NewEnumerator4")
      (Default|SceneComplete (Variables|Default|GetOwner%20Cutscene)))))

(fn ConstructionScript)