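; Cutscene director actor that plays an ordered list of scenes, then restores the player and can chain another cutscene.
; Each scene triggers character actions with camera modes, explosions, particles, sounds or level sequences.
; Helper actors report back through an owner reference, and SceneComplete advances to the next scene.
; Player lockout, character hiding and HUD hiding are optional, and the construction script spawns attached helper actors for setup.
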(event Custom|PlayCutscene
  (bind _cutscenesetup (Variables|Cutscenes|GetCutsceneSetup))
  (Utilities|FlowControl|Delay 0.2)
  ;[1 1 1] Check Cutscene Status
  (Variables|CutsceneData|SetCutsceneStatus (Variables|CutsceneData|GetCutsceneStatus))
  ;[1 1 1] Scene Order (each scene +1)
  (bind _output_get (Variables|CutsceneSettings|SetCutscene%20Start%20Order (+ (Variables|CutsceneSettings|GetCutscene%20Start%20Order) 1)))
  ;[1 1 1] If Cutscene Order Bigger than Last index, Complete the Cutscene
  (if (> (Variables|CutsceneSettings|GetCutscene%20Start%20Order) (Utilities|Array|LastIndex _cutscenesetup))
    (CutsceneSettings|CutsceneCompleted)
    (else
      (CallFunction|StartCutsceneSettings)
      ;[1 1 1] If you have Custom Event Add here
      (Variables|CutsceneData|SetScene%20Settings (Utilities|Struct|BreakCutscene_MainData (Utilities|Array|Get(acopy) _cutscenesetup _output_get)))
      (CallFunction|CustomEvents (Utilities|Struct|BreakCutscene_Settings (Variables|CutsceneData|GetScene%20Settings)))
      ;[1 1 1] Debug Scene Name
      (Debug|DebugPrint "SceneName:" (.SceneName (Utilities|Struct|BreakCutscene_MainData (Utilities|Array|Get(acopy) _cutscenesetup _output_get))) "(R=0.000000,G=1.000000,B=0.142576,A=1.000000)")
      ;[1 1 1] If player select "Jump to Next Scene" This will be work
      (CutsceneSettings|JumptoNextScene (Utilities|Struct|BreakCutscene_Settings (Variables|CutsceneData|GetScene%20Settings)))
      ;[1 1 1] Check Main Selected Option
      (switch Utilities|FlowControl|Switch|SwitchonCutscene_Mode (.SelectSceneMode (Utilities|Struct|BreakCutscene_MainData (Utilities|Array|Get(acopy) _cutscenesetup _output_get)))
        (:NewEnumerator0
          (CallFunction|CharacterAnimationCamera (.CharacterSetup (Utilities|Struct|BreakCutscene_CharacterAnimation (.CharacterAnimationCamera (Utilities|Struct|BreakCutscene_MainData (Utilities|Array|Get(acopy) _cutscenesetup _output_get))))) (.CharacterActions (Utilities|Struct|BreakCutscene_CharacterAnimation (.CharacterAnimationCamera (Utilities|Struct|BreakCutscene_MainData (Utilities|Array|Get(acopy) _cutscenesetup _output_get))))) (.CameraSettings (Utilities|Struct|BreakCutscene_CharacterAnimation (.CharacterAnimationCamera (Utilities|Struct|BreakCutscene_MainData (Utilities|Array|Get(acopy) _cutscenesetup _output_get)))))))
        (:NewEnumerator1
          (CallFunction|ExplosionSystem (.Explosion (Utilities|Struct|BreakCutscene_MainData (Utilities|Array|Get(acopy) _cutscenesetup _output_get)))))
        (:NewEnumerator2
          (CallFunction|ParticleEffectSelection (.ParticleEffect (Utilities|Struct|BreakCutscene_MainData (Utilities|Array|Get(acopy) _cutscenesetup _output_get)))))
        (:NewEnumerator3
          (CallFunction|SoundEffectSystem (.SoundEffect (Utilities|Struct|BreakCutscene_MainData (Utilities|Array|Get(acopy) _cutscenesetup _output_get)))))
        (:NewEnumerator4
          (CallFunction|StartLevelSequence (.SceneSettings (Utilities|Struct|BreakCutscene_MainData (Utilities|Array|Get(acopy) _cutscenesetup _output_get)))))))))

(event EventBeginPlay
  (bind _cutscenesetup (Variables|Cutscenes|GetCutsceneSetup))
  ;[1 1 1] If "Play Immediately" Selected, Play it on Begin Play
  (if (Variables|Debug|GetPlayImmediately)
    (Utilities|FlowControl|Delay 0.2)
    ;[1 1 1] Check Cutscene Status
    (Variables|CutsceneData|SetCutsceneStatus (Variables|CutsceneData|GetCutsceneStatus))
    ;[1 1 1] Scene Order (each scene +1)
    (bind _output_get (Variables|CutsceneSettings|SetCutscene%20Start%20Order (+ (Variables|CutsceneSettings|GetCutscene%20Start%20Order) 1)))
    ;[1 1 1] If Cutscene Order Bigger than Last index, Complete the Cutscene
    (if (> (Variables|CutsceneSettings|GetCutscene%20Start%20Order) (Utilities|Array|LastIndex _cutscenesetup))
      (CutsceneSettings|CutsceneCompleted)
      (else
        (CallFunction|StartCutsceneSettings)
        ;[1 1 1] If you have Custom Event Add here
        (Variables|CutsceneData|SetScene%20Settings (Utilities|Struct|BreakCutscene_MainData (Utilities|Array|Get(acopy) _cutscenesetup _output_get)))
        (CallFunction|CustomEvents (Utilities|Struct|BreakCutscene_Settings (Variables|CutsceneData|GetScene%20Settings)))
        ;[1 1 1] Debug Scene Name
        (Debug|DebugPrint "SceneName:" (.SceneName (Utilities|Struct|BreakCutscene_MainData (Utilities|Array|Get(acopy) _cutscenesetup _output_get))) "(R=0.000000,G=1.000000,B=0.142576,A=1.000000)")
        ;[1 1 1] If player select "Jump to Next Scene" This will be work
        (CutsceneSettings|JumptoNextScene (Utilities|Struct|BreakCutscene_Settings (Variables|CutsceneData|GetScene%20Settings)))
        ;[1 1 1] Check Main Selected Option
        (switch Utilities|FlowControl|Switch|SwitchonCutscene_Mode (.SelectSceneMode (Utilities|Struct|BreakCutscene_MainData (Utilities|Array|Get(acopy) _cutscenesetup _output_get)))
          (:NewEnumerator0
            (CallFunction|CharacterAnimationCamera (.CharacterSetup (Utilities|Struct|BreakCutscene_CharacterAnimation (.CharacterAnimationCamera (Utilities|Struct|BreakCutscene_MainData (Utilities|Array|Get(acopy) _cutscenesetup _output_get))))) (.CharacterActions (Utilities|Struct|BreakCutscene_CharacterAnimation (.CharacterAnimationCamera (Utilities|Struct|BreakCutscene_MainData (Utilities|Array|Get(acopy) _cutscenesetup _output_get))))) (.CameraSettings (Utilities|Struct|BreakCutscene_CharacterAnimation (.CharacterAnimationCamera (Utilities|Struct|BreakCutscene_MainData (Utilities|Array|Get(acopy) _cutscenesetup _output_get)))))))
          (:NewEnumerator1
            (CallFunction|ExplosionSystem (.Explosion (Utilities|Struct|BreakCutscene_MainData (Utilities|Array|Get(acopy) _cutscenesetup _output_get)))))
          (:NewEnumerator2
            (CallFunction|ParticleEffectSelection (.ParticleEffect (Utilities|Struct|BreakCutscene_MainData (Utilities|Array|Get(acopy) _cutscenesetup _output_get)))))
          (:NewEnumerator3
            (CallFunction|SoundEffectSystem (.SoundEffect (Utilities|Struct|BreakCutscene_MainData (Utilities|Array|Get(acopy) _cutscenesetup _output_get)))))
          (:NewEnumerator4
            (CallFunction|StartLevelSequence (.SceneSettings (Utilities|Struct|BreakCutscene_MainData (Utilities|Array|Get(acopy) _cutscenesetup _output_get))))))))))

(event Custom|CharacterAnimationCamera
  (params (Cutscene_CharacterSetup :type Cutscene%20Character%20Setup%20Structure%20%28by%20ref%29) (Cutscene_CharacterActions :type Cutscene%20Character%20Actions%20Structure%20%28by%20ref%29) (Cutscene_CameraMain :type Cutscene%20Camera%20Main%20Structure%20%28by%20ref%29))
  (Variables|CutsceneData|SetCutscene%20Character%20Setup Cutscene_CharacterSetup)
  (Variables|CutsceneData|SetCutscene%20Character%20Actions Cutscene_CharacterActions)
  (Variables|CutsceneData|SetCutscene%20Camera%20Main Cutscene_CameraMain)
  (CallFunction|CharacterSetup Cutscene_CharacterSetup))

(event Custom|CameraSystemStart
  (bind _cutscene_camera_main (Variables|CutsceneData|GetCutscene%20Camera%20Main))
  (bind (_wanttochangecamera_ _cameramods _selectcustommovcamera __or_selectnormalcamera _transitionsec) (Utilities|Struct|BreakCutscene_CameraMain _cutscene_camera_main))
  ;[0.007688 0 1] Camera System Start
  (if _wanttochangecamera_
    (switch Utilities|FlowControl|Switch|SwitchonCutscene_CameraMods _cameramods
      (:NewEnumerator1
        (CameraMods|Standing __or_selectnormalcamera _transitionsec))
      (:NewEnumerator7
        (CameraMods|LocktoCharacter __or_selectnormalcamera __or_selectnormalcamera))
      (:NewEnumerator3
        (CameraMods|MovewithCharacter __or_selectnormalcamera _transitionsec __or_selectnormalcamera))
      (:NewEnumerator5
        (CameraMods|CustomCameraMovement _selectcustommovcamera _transitionsec _selectcustommovcamera))
      (:NewEnumerator6
        (CameraMods|UseLevelSequenceCamera)))))

(event Custom|CharacterSetup
  (params (Cutscene_CharacterSetup :type Cutscene%20Character%20Setup%20Structure%20%28by%20ref%29))
  (bind (__or_usecharactername _spawnteleportpoint) (Utilities|Struct|BreakCutscene_CharacterSetup Cutscene_CharacterSetup))
  (bind (_useplayercharacter _spawnteleportpoint_2) (Utilities|Struct|BreakCutscene_CharacterSetup Cutscene_CharacterSetup))
  (bind (__or_spawncharacter _spawnteleportpoint_3) (Utilities|Struct|BreakCutscene_CharacterSetup Cutscene_CharacterSetup))
  (bind _staticmesh (Variables|/Game/CutsceneSystem/Blueprints/Core/Cutscene_SpawnPoint.Cutscene_SpawnPoint_C|GetStaticMesh _spawnteleportpoint_3))
  (bind _staticmesh_2 (Variables|/Game/CutsceneSystem/Blueprints/Core/Cutscene_SpawnPoint.Cutscene_SpawnPoint_C|GetStaticMesh _spawnteleportpoint))
  (bind _staticmesh_3 (Variables|/Game/CutsceneSystem/Blueprints/Core/Cutscene_SpawnPoint.Cutscene_SpawnPoint_C|GetStaticMesh _spawnteleportpoint_2))
  ;[0.04025 0.5884 1] Use Player Character
  (if _useplayercharacter
    (bind _ascharacter (Utilities|Casting|CastToCharacter (Game|Player|GetPlayerPawn 0)))
    (bind _output_get (Variables|CutsceneSystemVars|SetSelectedCharacter _ascharacter))
    (bind _output_get_2 (Variables|CutsceneSystemVars|SetPlayerCharacter _output_get))
    (if (Utilities|IsValid _spawnteleportpoint_2)
      (Transformation|Teleport _output_get_2 (Transformation|GetWorldLocation _staticmesh_3) (Transformation|GetWorldRotation _staticmesh_3)))
    ;[1 0 0.007234] Start Character Actions
    (Default|CharacterActions (Actor|GetComponentbyClass (Variables|CutsceneSystemVars|GetSelectedCharacter) "/Game/CutsceneSystem/Blueprints/Cutscene_ActorComponent.Cutscene_ActorComponent_C") (Variables|CutsceneData|GetCutscene%20Character%20Actions) (Variables|CutsceneData|GetCutscene%20Character%20Setup) self (Variables|CutsceneData|GetScene%20Settings) :!label _label)
    (CallFunction|CameraSystemStart)
    (else
      ;[0.3381 0 1] Spawn AI Character
      (if (Utilities|IsValidClass __or_spawncharacter)
        (Utilities|IsValid _staticmesh
          (:Is%20Valid
            (bind _returnvalue (AI|SpawnAIFromClass __or_spawncharacter 0 (Transformation|GetWorldLocation _staticmesh) (Transformation|GetWorldRotation _staticmesh) false 0))
            (bind _ascharacter_2 (Utilities|Casting|CastToCharacter _returnvalue))
            (bind _output_get_3 (Variables|CutsceneSystemVars|SetSelectedCharacter _ascharacter_2))
            ;;[0 0 0] Debug Spawned Character Name
            (Debug|DebugPrint "SpawnedCharacter:" (Utilities|String|ToString(Name) (Variables|/Game/CutsceneSystem/Blueprints/Cutscene_ActorComponent.Cutscene_ActorComponent_C|GetCharacterName (Actor|GetComponentbyClass _output_get_3 "/Game/CutsceneSystem/Blueprints/Cutscene_ActorComponent.Cutscene_ActorComponent_C"))) "(R=0.703125,G=0.133152,B=0.379252,A=1.000000)")
            (goto _label))
          (:Is%20Not%20Valid
            (Debug|DebugPrint "Try to Spawn AI:" "But no Selected Spawn Point" "(R=0.166085,G=0.000000,B=0.276042,A=1.000000)")))
        (else
          ;[1 0.2852 0.508] Use Character Name to Select Actor
          (if (Utilities|Name|NotEqual(Name) __or_usecharactername "None")
            (bind _outactors (Actor|GetAllActorsOfClass "/Script/Engine.Character"))
            (bind _array_element (Utilities|Array|ForEachLoopwithBreak _outactors :!label _label_2)
              (:LoopBody
                (if (Utilities|Name|Equal(Name) (Variables|/Game/CutsceneSystem/Blueprints/Cutscene_ActorComponent.Cutscene_ActorComponent_C|GetCharacterName (Actor|GetComponentbyClass _array_element "/Game/CutsceneSystem/Blueprints/Cutscene_ActorComponent.Cutscene_ActorComponent_C")) __or_usecharactername)
                  (Utilities|FlowControl|Sequence
                    (:then_0
                      (goto _label_2 Break))
                    (:then_1
                      (bind _ascharacter_3 (Utilities|Casting|CastToCharacter (Components|GetOwner (Actor|GetComponentbyClass _array_element "/Game/CutsceneSystem/Blueprints/Cutscene_ActorComponent.Cutscene_ActorComponent_C"))))
                      (bind _output_get_4 (Variables|CutsceneSystemVars|SetSelectedCharacter _ascharacter_3))
                      (if (Utilities|IsValid _spawnteleportpoint)
                        (Transformation|Teleport _output_get_4 (Transformation|GetWorldLocation _staticmesh_2) (Transformation|GetWorldRotation _staticmesh_2))
                        (goto _label)
                        (else
                          (goto _label))))))))
            (else
              (CallFunction|CameraSystemStart))))))))

(event Custom|SceneComplete
  (bind _cutscene_character_setup (Variables|CutsceneData|GetCutscene%20Character%20Setup))
  (bind _selectedcharacter (Variables|CutsceneSystemVars|GetSelectedCharacter))
  (bind _teleportcharacterafterthisscene (Utilities|Struct|BreakCutscene_CharacterSetup _cutscene_character_setup))
  (bind _staticmesh (Variables|/Game/CutsceneSystem/Blueprints/Core/Cutscene_TargetPoint.Cutscene_TargetPoint_C|GetStaticMesh _teleportcharacterafterthisscene))
  ;[1 1 1] Wait Before Scene Finished
  (Utilities|FlowControl|Delay (.ExtraWaitbeforethenextsceneSec (Utilities|Struct|BreakCutscene_Settings (Variables|CutsceneData|GetScene%20Settings))))
  ;[1 1 1] Hide Dialogue Widget
  (bind _foundwidgets (Widget|GetAllWidgetsOfClass "/Game/CutsceneSystem/Blueprints/Widgets/Cutscene_Subtitle.Cutscene_Subtitle_C" true))
  (for _array_element _foundwidgets
    (Widget|SetVisibility (Variables|/Game/CutsceneSystem/Blueprints/Widgets/Cutscene_Subtitle.Cutscene_Subtitle_C|GetPanel _array_element) "Hidden"))
  ;[1 1 1] Remove Actor After Scene
  (if (Utilities|Struct|BreakCutscene_CharacterSetup (Variables|CutsceneData|GetCutscene%20Character%20Setup))
    (Utilities|IsValid _selectedcharacter
      (:Is%20Valid
        (Actor|DestroyActor _selectedcharacter))
      (:Is%20Not%20Valid
        _)))
  ;[1 1 1] Teleport Character Actor After Scene
  (Utilities|IsValid _teleportcharacterafterthisscene
    (:Is%20Valid
      (Utilities|IsValid _selectedcharacter
        (:Is%20Valid
          (Transformation|Teleport _selectedcharacter (Transformation|GetWorldLocation _staticmesh) (Transformation|GetWorldRotation _staticmesh)))
        (:Is%20Not%20Valid
          _)))
    (:Is%20Not%20Valid
      _))
  ;[1 1 1] Back to Player Camera End of the Scene (IF SELECTED)
  (if (Utilities|Struct|BreakCutscene_CameraMain (Variables|CutsceneData|GetCutscene%20Camera%20Main))
    (Game|Player|SetViewTargetwithBlend (Game|GetPlayerController 0) (Game|Player|GetPlayerPawn 0) 0.0 "VTBlend_Linear" 0.0 false))
  ;[1 1 1] Play Next Scene
  (CallFunction|PlayCutscene))

(event Custom|DialogueSkipButton
  (bind _cutscene_character_setup (Variables|CutsceneData|GetCutscene%20Character%20Setup))
  (bind _selectedcharacter (Variables|CutsceneSystemVars|GetSelectedCharacter))
  (bind _teleportcharacterafterthisscene (Utilities|Struct|BreakCutscene_CharacterSetup _cutscene_character_setup))
  (bind _staticmesh (Variables|/Game/CutsceneSystem/Blueprints/Core/Cutscene_TargetPoint.Cutscene_TargetPoint_C|GetStaticMesh _teleportcharacterafterthisscene))
  ;[1 1 1] Dialogue Skip Action
  (bind _foundwidgets (Widget|GetAllWidgetsOfClass "/Game/CutsceneSystem/Blueprints/Widgets/Cutscene_Subtitle.Cutscene_Subtitle_C" true))
  (for _array_element _foundwidgets
    (Widget|SetVisibility (Variables|/Game/CutsceneSystem/Blueprints/Widgets/Cutscene_Subtitle.Cutscene_Subtitle_C|GetPanel _array_element) "Hidden")
    ;[1 1 1] Remove Actor After Scene
    (if (Utilities|Struct|BreakCutscene_CharacterSetup (Variables|CutsceneData|GetCutscene%20Character%20Setup))
      (Utilities|IsValid _selectedcharacter
        (:Is%20Valid
          (Actor|DestroyActor _selectedcharacter))
        (:Is%20Not%20Valid
          _)))
    ;[1 1 1] Teleport Character Actor After Scene
    (Utilities|IsValid _teleportcharacterafterthisscene
      (:Is%20Valid
        (Utilities|IsValid _selectedcharacter
          (:Is%20Valid
            (Transformation|Teleport _selectedcharacter (Transformation|GetWorldLocation _staticmesh) (Transformation|GetWorldRotation _staticmesh)))
          (:Is%20Not%20Valid
            _)))
      (:Is%20Not%20Valid
        _))
    ;[1 1 1] Back to Player Camera End of the Scene (IF SELECTED)
    (if (Utilities|Struct|BreakCutscene_CameraMain (Variables|CutsceneData|GetCutscene%20Camera%20Main))
      (Game|Player|SetViewTargetwithBlend (Game|GetPlayerController 0) (Game|Player|GetPlayerPawn 0) 0.0 "VTBlend_Linear" 0.0 false))
    ;[1 1 1] Play Next Scene
    (CallFunction|PlayCutscene)))

(event Custom|ExplosionSystem
  (params (CutsceneExplosion :type Cutscene%20Explosion%20Main%20Structure))
  (bind (_explosiontype _selectstandingexplosion _selectdropdownexplosion _selectparticleeffect _waitforexplosionsec _simulatephysicsfornearbyobjects_ _simulatephysicsfornearbycharacters_ _destroysimulatedactorsaftersec _damagetoactors_ _damagevalue _playsoundonexplosion) (Utilities|Struct|BreakCutscene_ExplosionMain CutsceneExplosion))
  (switch Utilities|FlowControl|Switch|SwitchonCutscene_ExplosionType _explosiontype
    (:NewEnumerator1
      ;[1 1 1] Standing Bomb
      (bind _output_get (Variables|CutsceneExplosion|SetSelectedStandingExplosion _selectstandingexplosion))
      (Effects|Components|ParticleSystem|SetTemplate (Variables|/Game/CutsceneSystem/Blueprints/Core/Cutscene_StandingExplosion.Cutscene_StandingExplosion_C|GetParticleSystem _output_get) _selectparticleeffect)
      (Default|ExplosionStart _output_get _waitforexplosionsec _simulatephysicsfornearbyobjects_ _simulatephysicsfornearbycharacters_ _destroysimulatedactorsaftersec _damagetoactors_ _damagevalue _playsoundonexplosion self))
    (:NewEnumerator0
      ;[1 1 1] Drop Down Bomb
      (bind _output_get_2 (Variables|CutsceneExplosion|SetSelect%20Drop%20Down%20Explosion _selectdropdownexplosion))
      (Effects|Components|ParticleSystem|SetTemplate (Variables|/Game/CutsceneSystem/Blueprints/Core/Cutscene_DropDownExplosion.Cutscene_DropDownExplosion_C|GetParticleSystem _output_get_2) _selectparticleeffect)
      (Default|ExplosionStart _output_get_2 _waitforexplosionsec _simulatephysicsfornearbyobjects_ _simulatephysicsfornearbycharacters_ _destroysimulatedactorsaftersec _damagetoactors_ _damagevalue _playsoundonexplosion self))))

(event Custom|ParticleEffectSelection
  (params (ParticleEffect :type Cutscene%20Particle%20Effect%20Structure))
  (bind (_selectcutsceneparticleeffectactor _particleeffect _waitbeforeactivatesec _removeparticleeffectendofthecutscene_ _attachparticleeffecttoactor __or_attachparticleeffecttoanycharactername _socketnametoattach _addsoundtoparticleactor) (Utilities|Struct|BreakCutscene_ParticleEffect ParticleEffect))
  ;[1 1 1] If "Remove Particle effect end of the cutscene" selected, collect that actor
  (bind _output_get (Variables|CutsceneParticleEffect|SetCutscene%20ParticleActor _selectcutsceneparticleeffectactor))
  (if _removeparticleeffectendofthecutscene_
    (Utilities|Array|Add (Variables|CutsceneParticleEffect|GetAllCutsceneParticleActors) _output_get))
  (Utilities|FlowControl|Sequence
    (:then_0
      ;[1 1 1] AttachtoActor
      (Utilities|IsValid _attachparticleeffecttoactor
        (:Is%20Valid
          (Transformation|AttachActorToActor _output_get _attachparticleeffecttoactor _socketnametoattach "KeepRelative" "KeepRelative" "KeepRelative" true))
        (:Is%20Not%20Valid
          (if (Utilities|Name|NotEqual(Name) __or_attachparticleeffecttoanycharactername "None")
            (bind _outactors (Actor|GetAllActorsOfClass "/Script/Engine.Character"))
            (for _array_element _outactors
              (if (Utilities|Name|Equal(Name) __or_attachparticleeffecttoanycharactername (Variables|/Game/CutsceneSystem/Blueprints/Cutscene_ActorComponent.Cutscene_ActorComponent_C|GetCharacterName (Actor|GetComponentbyClass _array_element "/Game/CutsceneSystem/Blueprints/Cutscene_ActorComponent.Cutscene_ActorComponent_C")))
                (Transformation|AttachActorToActor _output_get _array_element _socketnametoattach "KeepRelative" "KeepRelative" "KeepRelative" true)))))))
    (:then_1
      ;[1 1 1] Start Particle Effect
      (Default|StartParticleEffect _output_get _particleeffect _waitbeforeactivatesec _removeparticleeffectendofthecutscene_ _addsoundtoparticleactor self))))

(event Custom|SoundEffectSystem
  (params (SoundEffect :type Cutscene%20Sound%20Effect%20Structure))
  (bind (_cutscenesoundactor _sound _waitbeforeplaysec _volume _destroyaftercutscene) (Utilities|Struct|BreakCutscene_SoundEffect SoundEffect))
  (bind _output_get (Variables|CutsceneSoundEffect|SetCutscene%20Sound%20Object _cutscenesoundactor))
  ;[1 1 1] If "Destroy After Cutscene" Selected Collect That Actor
  (if _destroyaftercutscene
    (Utilities|Array|Add (Variables|CutsceneSoundEffect|GetAllCutsceneSoundActors) _output_get))
  ;[1 1 1] Play Sound
  (Default|PlaySoundSystem _output_get _sound _waitbeforeplaysec _volume self))

(event Custom|StartCutsceneSettings
  (CallFunction|DisableMovement)
  (CallFunction|DisableInputEvent)
  (CallFunction|HideCharacters)
  (CallFunction|HideWidgets))

(event Custom|DisableMovement
  ;[1 1 1] Disable & Enable Movement
  (if (Variables|CutsceneSettings|GetDisable%20Player%20Movement)
    (bind _ascharacter (Utilities|Casting|CastToCharacter (Game|Player|GetPlayerPawn 0)))
    (Pawn|Components|CharacterMovement|DisableMovement (Variables|/Script/Engine.Character|GetCharacterMovement _ascharacter))))

(event Custom|EnableMovement
  ;[1 1 1] Disable & Enable Movement
  (if (Variables|CutsceneSettings|GetDisable%20Player%20Movement)
    (bind _ascharacter (Utilities|Casting|CastToCharacter (Game|Player|GetPlayerPawn 0)))
    (Pawn|Components|CharacterMovement|SetMovementMode (Variables|/Script/Engine.Character|GetCharacterMovement _ascharacter) "MOVE_Walking" 0)))

(event Custom|EndCutsceneSettings
  (CallFunction|EnableMovement)
  (CallFunction|EnableInputEvent)
  (CallFunction|ShowCharacters)
  (CallFunction|ShowWidgets))

(event Custom|DisableInputEvent
  ;[1 1 1] Disable & Enable Input
  (if (Variables|CutsceneSettings|GetDisablePlayerInput)
    (Default|DisableInputEvent (Actor|GetComponentbyClass (Game|GetPlayerController 0) "/Game/CutsceneSystem/Blueprints/Cutscene_PlayerControllerComponent.Cutscene_PlayerControllerComponent_C"))))

(event Custom|EnableInputEvent
  ;[1 1 1] Disable & Enable Input
  (if (Variables|CutsceneSettings|GetDisablePlayerInput)
    (Default|EnableInputEvent (Actor|GetComponentbyClass (Game|GetPlayerController 0) "/Game/CutsceneSystem/Blueprints/Cutscene_PlayerControllerComponent.Cutscene_PlayerControllerComponent_C"))))

(event Custom|HideCharacters
  ;[1 1 1] Hide & Show Characters
  (for _array_element (Variables|CutsceneSettings|GetHide%20Game%20Characters%20In%20Cutscene)
    (Rendering|SetActorHiddenInGame _array_element true)))

(event Custom|ShowCharacters
  ;[1 1 1] Hide & Show Characters
  (for _array_element (Variables|CutsceneSettings|GetHide%20Game%20Characters%20In%20Cutscene)
    (Rendering|SetActorHiddenInGame _array_element false)))

(event Custom|HideWidgets
  ;[1 1 1] Show & Hide Widgets / HUD
  (if (Variables|CutsceneSettings|GetHide%20Player%20HUD%20%28Experimental%29)
    (bind _foundwidgets (Widget|GetAllWidgetsOfClass "/Script/UMG.UserWidget" true))
    (for _array_element _foundwidgets
      (Utilities|Array|Add (Variables|CutsceneSettings|GetHiddenWidgets) _array_element)
      (Widget|SetVisibility _array_element "Hidden"))))

(event Custom|ShowWidgets
  ;[1 1 1] Show & Hide Widgets / HUD
  (if (Variables|CutsceneSettings|GetHide%20Player%20HUD%20%28Experimental%29)
    (for _array_element (Variables|CutsceneSettings|GetHiddenWidgets)
      (Widget|SetVisibility _array_element "Visible"))))

(event Custom|StartLevelSequence
  (params (SceneSettings :type Cutscene%20Settings%20Structure))
  (bind (_uselevelsequence _movetonextsceneoption _extrawaitbeforethenextscenesec) (Utilities|Struct|BreakCutscene_Settings SceneSettings))
  (bind (_uselevelsequence_2 _selectlevelsequence _startframe _endframe) (Utilities|Struct|BreakCutscene_LevelSequence _uselevelsequence))
  (bind _sequenceplayer (Variables|/Script/LevelSequence.LevelSequenceActor|GetSequencePlayer _selectlevelsequence))
  ;[1 1 1] If "Use Level Sequence" Selected, play the level sequence
  (Utilities|FlowControl|Delay _extrawaitbeforethenextscenesec)
  (Utilities|IsValid _selectlevelsequence
    (:Is%20Valid
      (Class|MovieSceneSequencePlayer|SetFrameRange _sequenceplayer _startframe (- _endframe _startframe) 0.0)
      (Sequencer|Player|Play _sequenceplayer :!class /Script/MovieScene.MovieSceneSequencePlayer)
      ;[1 1 1] Check If "Wait for Level Sequence Finish" Selected Wait for complete scene
      (if (Utilities|Enum|Equal(Enum) _movetonextsceneoption "NewEnumerator3")
        (if (Audio|Components|Audio|IsPlaying _sequenceplayer) :!label _label
          (Utilities|FlowControl|Delay 0.1)
          (goto _label)
          (else
            (CallFunction|SceneComplete)))))))

(fn ConstructionScript
  (Utilities|FlowControl|Sequence
    (:then_0
      (AddtoScene|AddSpawnPoint)
      (AddToScene|AddTargetPoint)
      (AddToScene|AddNormalCamera)
      (AddToScene|AddStandingExplosion)
      (AddToScene|AddDropDownExplosion)
      (AddToScene|AddCutsceneParticleActor)
      (AddToScene|AddCustomMovementCamera)
      (AddToScene|AddCutsceneSound))))

(fn AddSpawnPoint
  (bind _returnvalue (Game|SpawnActorfromClass "/Game/CutsceneSystem/Blueprints/Core/Cutscene_SpawnPoint.Cutscene_SpawnPoint_C" (Math|Transform|MakeTransform "0, 0,5.000000" "0, 0, 0" "1,1,1") "Undefined" 0 0))
  (Transformation|AttachActorToActor _returnvalue self "None" "KeepRelative" "KeepRelative" "KeepRelative" true))

(fn AddTargetPoint
  (bind _returnvalue (Game|SpawnActorfromClass "/Game/CutsceneSystem/Blueprints/Core/Cutscene_TargetPoint.Cutscene_TargetPoint_C" (Math|Transform|MakeTransform "0, 0,5.000000" "0, 0, 0" "1,1,1") "Undefined" 0 0))
  (Transformation|AttachActorToActor _returnvalue self "None" "KeepRelative" "KeepRelative" "KeepRelative" true))

(fn AddCustomMovementCamera
  (bind _returnvalue (Game|SpawnActorfromClass "/Game/CutsceneSystem/Blueprints/Camera/Cutscene_Camera.Cutscene_Camera_C" (Math|Transform|MakeTransform "0, 0,5.000000" "0, 0, 0" "1,1,1") "Undefined" 0 0))
  (Transformation|AttachActorToActor _returnvalue self "None" "KeepRelative" "KeepRelative" "KeepRelative" true))

(fn AddNormalCamera
  (bind _returnvalue (Game|SpawnActorfromClass "/Script/CinematicCamera.CineCameraActor" (Math|Transform|MakeTransform "0, 0,5.000000" "0, 0, 0" "1,1,1") "Undefined" 0 0))
  (Transformation|AttachActorToActor _returnvalue self "None" "KeepRelative" "KeepRelative" "KeepRelative" true))

(fn DebugPrint
  (params (Title: :type String) (DebugText :type String) (TextColor :type Linear%20Color%20Structure))
  (if (Variables|Debug|GetActivateDebug)
    (Development|PrintString (Utilities|String|Append Title: DebugText) true true TextColor 5.0)))

(fn JumptoNextScene
  (params (JumpToNext :type Cutscene_NextSceneOptions%20Enum :default "NewEnumerator0"))
  (if (Utilities|Enum|Equal(Enum) JumpToNext "NewEnumerator0")
    (CallFunction|SceneComplete)))

(fn CutsceneCompleted
  (bind _playcutsceneafterthis (Variables|CutsceneSettings|GetPlayCutsceneAfterThis))
  (Variables|CutsceneSystemVars|SetCutsceneCompleted? true)
  (Variables|CutsceneData|SetCutsceneStatus "NewEnumerator2")
  (Debug|DebugPrint "Cutscene Status:" "Completed!" "(R=1.000000,G=0.000000,B=0.078311,A=1.000000)")
  ;[1 1 1] Particles and Sounds Destroyed
  (for _array_element (Variables|CutsceneParticleEffect|GetAllCutsceneParticleActors)
    (Actor|DestroyActor _array_element))
  (for _array_element_2 (Variables|CutsceneSoundEffect|GetAllCutsceneSoundActors)
    (Actor|DestroyActor _array_element_2))
  ;[1 1 1] Camera back to Player
  (Game|Player|SetViewTargetwithBlend (Game|GetPlayerController 0) (Game|Player|GetPlayerPawn 0) 0.0 "VTBlend_Linear" 0.0 false)
  (CallFunction|EndCutsceneSettings)
  (Utilities|IsValid _playcutsceneafterthis
    (:Is%20Valid
      (CallFunction|PlayCutscene _playcutsceneafterthis))))

(fn Standing
  (params (NewViewTarget :type Actor%20Object%20Reference) (BlendTime :type Float%20%28single-precision%29))
  (Game|Player|SetViewTargetwithBlend (Game|GetPlayerController 0) NewViewTarget BlendTime "VTBlend_Linear" 0.0 false))

(fn LocktoCharacter
  (params (NewViewTarget :type Actor%20Object%20Reference) (self2 :type Cine%20Camera%20Actor%20Object%20Reference))
  (Game|Player|SetViewTargetwithBlend (Game|GetPlayerController 0) NewViewTarget 0.0 "VTBlend_Linear" 0.0 false)
  (Variables|/Script/CinematicCamera.CineCameraActor|SetLookatTrackingSettings self2 (Utilities|Struct|MakeCameraLookatTrackingSettings true false 0.0 (Utilities|ResolveSoftReference (Variables|CutsceneSystemVars|GetSelectedCharacter)) "0.000000,0.000000,0.000000" false)))

(fn MovewithCharacter
  (params (NewViewTarget :type Actor%20Object%20Reference) (BlendTime :type Float%20%28single-precision%29) (self2 :type Actor%20Object%20Reference))
  (Game|Player|SetViewTargetwithBlend (Game|GetPlayerController 0) NewViewTarget BlendTime "VTBlend_Linear" 0.0 false)
  (Transformation|AttachActorToActor self2 (Variables|CutsceneSystemVars|GetSelectedCharacter) "None" "KeepWorld" "KeepRelative" "KeepRelative" true))

(fn CustomCameraMovement
  (params (NewViewTarget :type Actor%20Object%20Reference) (BlendTime :type Float%20%28single-precision%29) (self2 :type Cutscene%20Camera%20Object%20Reference))
  (Game|Player|SetViewTargetwithBlend (Game|GetPlayerController 0) NewViewTarget BlendTime "VTBlend_Linear" 0.0 false)
  (Default|CameraStart self2 self (Variables|CutsceneData|GetScene%20Settings)))

(fn UseLevelSequenceCamera
  (bind _scene_settings (Variables|CutsceneData|GetScene%20Settings))
  (bind _uselevelsequence (Utilities|Struct|BreakCutscene_Settings _scene_settings))
  (bind (_uselevelsequence_2 _selectlevelsequence _startframe _endframe) (Utilities|Struct|BreakCutscene_LevelSequence _uselevelsequence))
  (bind _sequenceplayer (Variables|/Script/LevelSequence.LevelSequenceActor|GetSequencePlayer _selectlevelsequence))
  (if _uselevelsequence_2
    (Class|MovieSceneSequencePlayer|SetFrameRange _sequenceplayer _startframe (- _endframe _startframe) 0.0)
    (Sequencer|Player|Play _sequenceplayer :!class /Script/MovieScene.MovieSceneSequencePlayer)))

(fn AddStandingExplosion
  (bind _returnvalue (Game|SpawnActorfromClass "/Game/CutsceneSystem/Blueprints/Core/Cutscene_StandingExplosion.Cutscene_StandingExplosion_C" (Math|Transform|MakeTransform "0, 0,5.000000" "0, 0, 0" "1,1,1") "Undefined" 0 0))
  (Transformation|AttachActorToActor _returnvalue self "None" "KeepRelative" "KeepRelative" "KeepRelative" true))

(fn AddDropDownExplosion
  (bind _returnvalue (Game|SpawnActorfromClass "/Game/CutsceneSystem/Blueprints/Core/Cutscene_DropDownExplosion.Cutscene_DropDownExplosion_C" (Math|Transform|MakeTransform "0, 0,5.000000" "0, 0, 0" "1,1,1") "Undefined" 0 0))
  (Transformation|AttachActorToActor _returnvalue self "None" "KeepRelative" "KeepRelative" "KeepRelative" true))

(fn AddCutsceneParticleActor
  (bind _returnvalue (Game|SpawnActorfromClass "/Game/CutsceneSystem/Blueprints/Core/Cutscene_ParticleEffectActor.Cutscene_ParticleEffectActor_C" (Math|Transform|MakeTransform "0, 0,5.000000" "0, 0, 0" "1,1,1") "Undefined" 0 0))
  (Transformation|AttachActorToActor _returnvalue self "None" "KeepRelative" "KeepRelative" "KeepRelative" true))

(fn AddCutsceneSound
  (bind _returnvalue (Game|SpawnActorfromClass "/Game/CutsceneSystem/Blueprints/Core/Cutscene_SoundEffect.Cutscene_SoundEffect_C" (Math|Transform|MakeTransform "0, 0,5.000000" "0, 0, 0" "1,1,1") "Undefined" 0 0))
  (Transformation|AttachActorToActor _returnvalue self "None" "KeepRelative" "KeepRelative" "KeepRelative" true))

(fn CustomEvents
  (params (Event%20ID :type Integer))
  (switch int Event%20ID))

(fn AddCutsceneStarter
  (bind _returnvalue (Game|SpawnActorfromClass "/Game/CutsceneSystem/Blueprints/Core/Cutscene_Starter.Cutscene_Starter_C" (Math|Transform|MakeTransform "0, 0,5.000000" "0, 0, 0" "1,1,1") "Undefined" self 0))
  (Transformation|AttachActorToActor _returnvalue self "None" "KeepRelative" "KeepRelative" "KeepRelative" true))