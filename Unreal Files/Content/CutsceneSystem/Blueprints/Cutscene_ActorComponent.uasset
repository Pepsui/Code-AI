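; Character component that performs one character's part in a cutscene when the owning cutscene sends its actions and settings.
; It plays or loops action montages, sets movement speed or ragdolls, and moves through up to three targets via AI MoveTo, or SimpleMove with overlap polling for the player.
; It handles approach, facing and sound, overhead or subtitle dialogue, can signal scene completion, and removes or teleports the character after the cutscene.
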(event Custom|CharacterActions
  (params (Cutscene_CharacterActions :type Cutscene%20Character%20Actions%20Structure) (Cutscene_CharacterSetup :type Cutscene%20Character%20Setup%20Structure) (OwnerCutscene :type Cutscene%20Tool%20Object%20Reference) (SceneSettings :type Cutscene%20Settings%20Structure))
  (Utilities|FlowControl|Sequence
    (:then_0
      (bind _output_get (Variables|!DONOTTOUCH|SetCutscene%20Character%20Actions Cutscene_CharacterActions))
      (Variables|!DONOTTOUCH|SetCutscene%20Character%20Setup Cutscene_CharacterSetup)
      (Variables|!DONOTTOUCH|SetOwner%20Cutscene OwnerCutscene)
      (Variables|!DONOTTOUCH|SetScene%20Settings SceneSettings)
      (Utilities|FlowControl|Sequence
        (:then_0
          ;[0 1 0.7247] Setting Montage And Movement Speed
          (Variables|!DONOTTOUCH|SetCharacter%20Actions (.CharacterActions (Utilities|Struct|BreakCutscene_CharacterActions _output_get)))
          (Variables|!DONOTTOUCH|SetLoop%20Animation%20Until%20Cutscene%20End (.LoopAnimationUntilCutsceneEnd (Utilities|Struct|BreakCutscene_CharacterActions _output_get)))
          (Variables|!DONOTTOUCH|SetCustom%20Animations (.CustomAnimations (Utilities|Struct|BreakCutscene_CharacterActions _output_get)))
          (CallFunction|SetAnimPlayRate)
          (CallFunction|SelectMontage)
          (switch Utilities|FlowControl|Switch|SwitchonCutscene_CharacterActions (Variables|!DONOTTOUCH|GetCharacter%20Actions)
            (:NewEnumerator0
              ;;[0.06939 0 1 1 12] If There is a Valid Custom Animation Move Animation will be change
              (CallFunction|PlayMontage :!label _label))
            (:NewEnumerator1
              ;;[0.2506 1 0] Change Move Speeds
              (CharacterSpeed|SetSlowWalkSpeed)
              (CallFunction|PlayMontage))
            (:NewEnumerator2
              (CharacterSpeed|SetWalkSpeed)
              (CallFunction|PlayMontage))
            (:NewEnumerator3
              (CharacterSpeed|SetRunSpeed)
              (CallFunction|PlayMontage))
            (:NewEnumerator4
              (goto _label))
            (:NewEnumerator5
              (goto _label))
            (:NewEnumerator6
              (goto _label))
            (:NewEnumerator10
              (goto _label))
            (:NewEnumerator7
              (CharacterSpeed|SetCustomMoveAnimaSpeed)
              (goto _label))
            (:NewEnumerator13
              (goto _label))
            (:NewEnumerator15
              (CallFunction|SetCharacterRagdoll))))
        (:then_1
          ;[1 0.6525 0] Character Movement Orders
          (Utilities|IsValid (Utilities|Struct|BreakCutscene_MoveTargets (Utilities|Struct|BreakCutscene_CharacterActions (Variables|!DONOTTOUCH|GetCutscene%20Character%20Actions)))
            (:Is%20Valid
              (switch Utilities|FlowControl|Switch|SwitchonCutscene_CharacterActions (Variables|!DONOTTOUCH|GetCharacter%20Actions)
                (:NewEnumerator1
                  _)
                (:NewEnumerator2
                  _)
                (:NewEnumerator3
                  _)
                (:NewEnumerator7
                  _))
              (CallFunction|CharacterMovement))))
        (:then_2
          ;[1 0.225 0.6933] Talk To Target
          ;;[1 1 1] Who is the character talking to?
          (if (.CharacterHasDialogue? (Utilities|Struct|BreakCutscene_TalkOptions (Utilities|Struct|BreakCutscene_CharacterActions (Variables|!DONOTTOUCH|GetCutscene%20Character%20Actions))))
            (if (not (Utilities|Name|Equal(Name) (.CharacterNameToTurnMoveForTalk (Utilities|Struct|BreakCutscene_TalkTarget (.TurnMovetoTargetBeforeTalk (Utilities|Struct|BreakCutscene_TalkOptions (Utilities|Struct|BreakCutscene_CharacterActions (Variables|!DONOTTOUCH|GetCutscene%20Character%20Actions)))))) "None"))
              (bind _outactors (Actor|GetAllActorsOfClass "/Script/Engine.Character"))
              (for _array_element _outactors
                (if (Utilities|Name|Equal(Name) (.CharacterNameToTurnMoveForTalk (Utilities|Struct|BreakCutscene_TalkTarget (.TurnMovetoTargetBeforeTalk (Utilities|Struct|BreakCutscene_TalkOptions (Utilities|Struct|BreakCutscene_CharacterActions (Variables|!DONOTTOUCH|GetCutscene%20Character%20Actions)))))) (Variables|Cutscene_ActorComponent_C|GetCharacterName (Actor|GetComponentbyClass _array_element "Cutscene_ActorComponent_C")))
                  (Variables|!DONOTTOUCH|SetTalkToCharacter _array_element)
                  (CallFunction|CharacterMovetoTalkTarget)))
              (elif (.-OR-IsitPlayerCharacter?ToMoveorTurn (Utilities|Struct|BreakCutscene_TalkTarget (.TurnMovetoTargetBeforeTalk (Utilities|Struct|BreakCutscene_TalkOptions (Utilities|Struct|BreakCutscene_CharacterActions (Variables|!DONOTTOUCH|GetCutscene%20Character%20Actions))))))
                (bind _ascharacter (Utilities|Casting|CastToCharacter (Game|Player|GetPlayerPawn 0)))
                (Variables|!DONOTTOUCH|SetTalkToCharacter _ascharacter)
                (CallFunction|CharacterMovetoTalkTarget)
                (else
                  (CallFunction|StartDialogue))))))))
    (:then_1
      ;[1 1 1] Remove & Teleport Character After Cutscene
      (CallFunction|RemoveCharacterAfterCutscene))
    (:then_2
      (CallFunction|TeleportCharacterAfterCutscene))))

(event Custom|PlayMontage
  (bind _montage_to_play (Variables|!DONOTTOUCH|GetMontage%20to%20Play))
  ;[0.2883 0.212 1] PlayMontage
  (if (Variables|!DONOTTOUCH|GetLoop%20Animation%20Until%20Cutscene%20End)
    (Utilities|IsValid _montage_to_play
      (:Is%20Valid
        (Animation|Montage|PlayMontage (Variables|/Script/Engine.Character|GetMesh (Variables|!DONOTTOUCH|GetCharacter)) (Variables|!DONOTTOUCH|GetMontage%20to%20Play) (Variables|!DONOTTOUCH|GetAnimPlayRate) :!label _label
          (:OnBlendOut
            (if (not (Variables|!DONOTTOUCH|GetCutsceneCompleted))
              (Utilities|FlowControl|Delay 0.1)
              (goto _label)
              (else
                (Animation|StopAnimMontage (Variables|!DONOTTOUCH|GetCharacter) (Variables|!DONOTTOUCH|GetMontage%20to%20Play))))))))
    (else
      ;;[1 1 1] Non-Loop Montage
      (Utilities|IsValid _montage_to_play
        (:Is%20Valid
          (Animation|Montage|PlayMontage (Variables|/Script/Engine.Character|GetMesh (Variables|!DONOTTOUCH|GetCharacter)) (Variables|!DONOTTOUCH|GetMontage%20to%20Play)))))))

(event Custom|Character%20Move%20To%20Talk%20Target
  (bind _cutscene_character_actions (Variables|!DONOTTOUCH|GetCutscene%20Character%20Actions))
  (bind _talktocharacter (Variables|!DONOTTOUCH|GetTalkToCharacter))
  (bind _talktarget (Utilities|Struct|BreakCutscene_CharacterActions _cutscene_character_actions))
  (bind _returnvalue (Transformation|GetActorLocation _talktocharacter))
  (bind (_characterhasdialogue_ _turnmovetotargetbeforetalk) (Utilities|Struct|BreakCutscene_TalkOptions _talktarget))
  (bind (_characternametoturnmovefortalk __or_isitplayercharacter_tomoveorturn _charactershouldmovetotargetbeforetalk_ _minimumhowclose_cm _charactershouldturntotarget_ _targetshouldturntospeaker_) (Utilities|Struct|BreakCutscene_TalkTarget _turnmovetotargetbeforetalk))
  ;[1 0.225 0.6933] Talk To Target
  ;;[1 1 1] Character Move To Target Before Talk
  (if _charactershouldmovetotargetbeforetalk_
    (if (not (Utilities|Struct|BreakCutscene_CharacterSetup (Variables|!DONOTTOUCH|GetCutscene%20Character%20Setup)))
      (CallFunction|ChangeMovementSpeed)
      (AI|AIMoveTo (Variables|!DONOTTOUCH|GetCharacter) "0, 0, 0" (Variables|!DONOTTOUCH|GetTalkToCharacter) (+ _minimumhowclose_cm 5.0) false
        (:OnSuccess
          (CallFunction|CharacterTurntoTarget :!label _label)))
      (else
        ;;;[1 1 1] If Speaker is Player Character Using Different Move To
        (AI|Navigation|SimpleMovetoActor (Game|GetPlayerController 0) _talktocharacter)
        (bind _returnvalue_2 (Collision|SphereOverlapActors (Math|Vector|MakeVector (.x _returnvalue) (.y _returnvalue) (.z _returnvalue)) 1.5e+02 (Utilities|Array|MakeArray "ObjectTypeQuery3") (Utilities|GetClass (Variables|!DONOTTOUCH|GetCharacter)) :!label _label_2))
        (if _returnvalue_2
          (CallFunction|CharacterTurntoTarget)
          (else
            (Utilities|FlowControl|Delay 0.2)
            (goto _label_2)))))
    (else
      (goto _label))))

(event Custom|CharacterMovement
  (bind _cutscene_character_actions (Variables|!DONOTTOUCH|GetCutscene%20Character%20Actions))
  (bind _cutscene_character_actions_2 (Variables|!DONOTTOUCH|GetCutscene%20Character%20Actions))
  (bind _movetargets (Utilities|Struct|BreakCutscene_CharacterActions _cutscene_character_actions))
  (bind _movetargets_2 (Utilities|Struct|BreakCutscene_CharacterActions _cutscene_character_actions_2))
  (bind (_target1 _wait _target2 _wait2 _target3) (Utilities|Struct|BreakCutscene_MoveTargets _movetargets_2))
  (bind (_target1_2 _wait_2 _target2_2 _wait2_2 _target3_2) (Utilities|Struct|BreakCutscene_MoveTargets _movetargets))
  (bind _returnvalue (Transformation|GetActorLocation _target1))
  (bind _returnvalue_2 (Transformation|GetActorLocation _target1))
  (bind _returnvalue_3 (Transformation|GetActorLocation _target2))
  (bind _returnvalue_4 (Transformation|GetActorLocation _target3))
  (bind _returnvalue_5 (Transformation|GetActorLocation _target2))
  ;[1 0.3096 0] Move To Target
  (if (Utilities|Struct|BreakCutscene_CharacterSetup (Variables|!DONOTTOUCH|GetCutscene%20Character%20Setup))
    ;;[1 1 1] Player Character Moving
    ;;;[1 1 1] Move Target 1
    (AI|Navigation|SimpleMovetoActor (Game|GetPlayerController 0) _target1)
    (Utilities|IsValid _target2
      (:Is%20Valid
        ;;;[1 1 1] Wait
        (Utilities|FlowControl|Delay _wait)
        ;;;[1 1 1] Player reach to target?
        (bind _returnvalue_6 (Collision|SphereOverlapActors (Math|Vector|MakeVector (.x _returnvalue) (.y _returnvalue) (+ (.z _returnvalue) 65.0)) 1.2e+02 (Utilities|Array|MakeArray "ObjectTypeQuery3") (Utilities|GetClass (Variables|!DONOTTOUCH|GetCharacter)) :!label _label))
        ;;;[1 1 1] Move Target 2
        (if _returnvalue_6
          (AI|Navigation|SimpleMovetoActor (Game|GetPlayerController 0) _target2)
          (Utilities|IsValid _target3
            (:Is%20Valid
              ;;;[1 1 1] Wait
              (Utilities|FlowControl|Delay _wait2)
              ;;;[1 1 1] Player Reach to Target?
              (bind _returnvalue_7 (Collision|SphereOverlapActors (Math|Vector|MakeVector (.x _returnvalue_5) (.y _returnvalue_5) (+ (.z _returnvalue_5) 65.0)) 1.2e+02 (Utilities|Array|MakeArray "ObjectTypeQuery3") (Utilities|GetClass (Variables|!DONOTTOUCH|GetCharacter)) :!label _label_2))
              (if _returnvalue_7
                ;;;[1 1 1] Move to Target 3
                (AI|Navigation|SimpleMovetoActor (Game|GetPlayerController 0) _target3)
                ;;;[1 1 1] Player Reach to Target?
                (bind _returnvalue_8 (Collision|SphereOverlapActors (Math|Vector|MakeVector (.x _returnvalue_4) (.y _returnvalue_4) (+ (.z _returnvalue_4) 65.0)) 1.2e+02 (Utilities|Array|MakeArray "ObjectTypeQuery3") (Utilities|GetClass (Variables|!DONOTTOUCH|GetCharacter)) :!label _label_3))
                (if _returnvalue_8
                  ;;;[1 1 1] Complete the Scene
                  (SceneCompleteOptions|MovementSceneComplete)
                  (else
                    (Utilities|FlowControl|Delay 0.2)
                    (goto _label_3)))
                (else
                  (Utilities|FlowControl|Delay 0.2)
                  (goto _label_2))))
            (:Is%20Not%20Valid
              ;;;[1 1 1] Player Character if Reach The Target Complete the scene (IF SELECTED)?
              (bind _returnvalue_9 (Collision|SphereOverlapActors (Math|Vector|MakeVector (.x _returnvalue_3) (.y _returnvalue_3) (+ (.z _returnvalue_3) 65.0)) 1.2e+02 (Utilities|Array|MakeArray "ObjectTypeQuery3") (Utilities|GetClass (Variables|!DONOTTOUCH|GetCharacter)) :!label _label_4))
              (if _returnvalue_9
                (SceneCompleteOptions|MovementSceneComplete)
                (else
                  (Utilities|FlowControl|Delay 0.2)
                  (goto _label_4)))))
          (else
            (Utilities|FlowControl|Delay 0.2)
            (goto _label))))
      (:Is%20Not%20Valid
        (bind _returnvalue_10 (Collision|SphereOverlapActors (Math|Vector|MakeVector (.x _returnvalue_2) (.y _returnvalue_2) (+ (.z _returnvalue_2) 65.0)) 1.2e+02 (Utilities|Array|MakeArray "ObjectTypeQuery3") (Utilities|GetClass (Variables|!DONOTTOUCH|GetCharacter)) :!label _label_5))
        (if _returnvalue_10
          (SceneCompleteOptions|MovementSceneComplete)
          (else
            (Utilities|FlowControl|Delay 0.2)
            (goto _label_5)))))
    (else
      ;;[1 1 1] AI Character Moving
      ;;;[1 1 1] Target 1 & Wait
      (Utilities|IsValid _target1_2
        (:Is%20Valid
          (AI|AIMoveTo (Variables|!DONOTTOUCH|GetCharacter) "0, 0, 0" _target1_2 5.0 false
            (:OnSuccess
              (Utilities|FlowControl|Delay _wait_2)
              (Utilities|IsValid _target2_2
                (:Is%20Valid
                  ;;;[1 1 1] Target 2 & Wait
                  (AI|AIMoveTo (Variables|!DONOTTOUCH|GetCharacter) "0, 0, 0" _target2_2 5.0 false
                    (:OnSuccess
                      (Utilities|FlowControl|Delay _wait2_2)
                      (Utilities|IsValid _target3_2
                        (:Is%20Valid
                          ;;;[1 1 1] Target 3
                          (AI|AIMoveTo (Variables|!DONOTTOUCH|GetCharacter) "0, 0, 0" _target3_2 5.0 false
                            (:OnSuccess
                              _)
                            (:OnFail
                              _))
                          (CharacterSpeed|ResetWalkSpeed)
                          (Animation|StopAnimMontage (Variables|!DONOTTOUCH|GetCharacter) (Variables|!DONOTTOUCH|GetMontage%20to%20Play))
                          ;[1 1 1] Next Target Doesn't Valid, Complete the Scene
                          ;;[1 1 1] After Target 3 Complete the Scene
                          (SceneCompleteOptions|MovementSceneComplete))
                        (:Is%20Not%20Valid
                          (CharacterSpeed|ResetWalkSpeed)
                          (Animation|StopAnimMontage (Variables|!DONOTTOUCH|GetCharacter) (Variables|!DONOTTOUCH|GetMontage%20to%20Play))
                          (SceneCompleteOptions|MovementSceneComplete))))
                    (:OnFail
                      (CharacterSpeed|ResetWalkSpeed :!label _label_6)
                      (Animation|StopAnimMontage (Variables|!DONOTTOUCH|GetCharacter) (Variables|!DONOTTOUCH|GetMontage%20to%20Play))
                      (SceneCompleteOptions|MovementSceneComplete))))
                (:Is%20Not%20Valid
                  (goto _label_6))))
            (:OnFail
              (CharacterSpeed|ResetWalkSpeed :!label _label_7)
              (Animation|StopAnimMontage (Variables|!DONOTTOUCH|GetCharacter) (Variables|!DONOTTOUCH|GetMontage%20to%20Play)))))
        (:Is%20Not%20Valid
          (goto _label_7))))))

(event Custom|ChangeMovementSpeed
  ;[0 1 0.7247] Setting Montage And Movement Speed
  (switch Utilities|FlowControl|Switch|SwitchonCutscene_CharacterActions (Variables|!DONOTTOUCH|GetCharacter%20Actions)
    (:NewEnumerator0
      ;;[0.06939 0 1 1 12] If There is a Valid Custom Animation Move Animation will be change
      (CallFunction|PlayMontage :!label _label))
    (:NewEnumerator1
      ;;[0.2506 1 0] Change Move Speeds
      (CharacterSpeed|SetSlowWalkSpeed)
      (CallFunction|PlayMontage))
    (:NewEnumerator2
      (CharacterSpeed|SetWalkSpeed)
      (CallFunction|PlayMontage))
    (:NewEnumerator3
      (CharacterSpeed|SetRunSpeed)
      (CallFunction|PlayMontage))
    (:NewEnumerator4
      (goto _label))
    (:NewEnumerator5
      (goto _label))
    (:NewEnumerator6
      (goto _label))
    (:NewEnumerator10
      (goto _label))
    (:NewEnumerator7
      (CharacterSpeed|SetCustomMoveAnimaSpeed)
      (goto _label))
    (:NewEnumerator13
      (goto _label))
    (:NewEnumerator15
      (CallFunction|SetCharacterRagdoll))))

(event Custom|Character%20Turn%20To%20Target
  (bind _character (Variables|!DONOTTOUCH|GetCharacter))
  ;[1 0.225 0.6933] Talk To Target
  ;;[1 1 1] Character Turn To Target Before Talk
  (if (.CharacterShouldTurntoTarget? (Utilities|Struct|BreakCutscene_TalkTarget (.TurnMovetoTargetBeforeTalk (Utilities|Struct|BreakCutscene_TalkOptions (Utilities|Struct|BreakCutscene_CharacterActions (Variables|!DONOTTOUCH|GetCutscene%20Character%20Actions))))))
    (Transformation|SetActorRotation _character (Math|Rotator|FindLookatRotation (Transformation|GetActorLocation _character) (Transformation|GetActorLocation (Variables|!DONOTTOUCH|GetTalkToCharacter)))))
  (CallFunction|TargetTurntoSpeaker))

(event Custom|Target%20Turn%20to%20Speaker
  (bind _talktocharacter (Variables|!DONOTTOUCH|GetTalkToCharacter))
  ;[1 0.225 0.6933] Talk To Target
  ;;[1 1 1] Target Turn to Speaker
  (Utilities|FlowControl|Delay 0.2)
  (if (.TargetShouldTurntoSpeaker? (Utilities|Struct|BreakCutscene_TalkTarget (.TurnMovetoTargetBeforeTalk (Utilities|Struct|BreakCutscene_TalkOptions (Utilities|Struct|BreakCutscene_CharacterActions (Variables|!DONOTTOUCH|GetCutscene%20Character%20Actions))))))
    (Transformation|SetActorRotation _talktocharacter (Math|Rotator|FindLookatRotation (Transformation|GetActorLocation _talktocharacter) (Transformation|GetActorLocation (Variables|!DONOTTOUCH|GetCharacter)))))
  (CallFunction|StartDialogue))

(event Custom|StartDialogue
  (bind _character (Variables|!DONOTTOUCH|GetCharacter))
  (bind _character_2 (Variables|!DONOTTOUCH|GetCharacter))
  (bind _cutscene_character_actions (Variables|!DONOTTOUCH|GetCutscene%20Character%20Actions))
  (bind _character_3 (Variables|!DONOTTOUCH|GetCharacter))
  (bind _talktarget (Utilities|Struct|BreakCutscene_CharacterActions _cutscene_character_actions))
  (bind _dialogue (Utilities|Struct|BreakCutscene_TalkOptions _talktarget))
  (bind (_dialogue_2 _dialoguesound _dialoguetextoptions _shouldclickfornextscene _extrawaitfornextscenesec) (Utilities|Struct|BreakCutscene_CharacterDialogue _dialogue))
  ;[0.123 1 0] Dialogue System
  (switch Utilities|FlowControl|Switch|SwitchonCutscene_DialogueOptions _dialoguetextoptions
    (:NewEnumerator0
      ;;[1 1 1] Only Play Sound For Dialogue
      (Utilities|IsValid _dialoguesound
        (:Is%20Valid
          (Audio|SpawnSoundatLocation _dialoguesound (Transformation|GetActorLocation _character) (Transformation|GetActorRotation _character) 1.0 1.0 0.0 0 0)
          (Utilities|FlowControl|Delay (Variables|/Script/Engine.SoundBase|GetDuration _dialoguesound)))
        (:Is%20Not%20Valid
          _))
      (Utilities|FlowControl|Delay _extrawaitfornextscenesec)
      (SceneCompleteOptions|DialogueSceneComplete))
    (:NewEnumerator1
      ;;[1 1 1] Overhead Dialogue & Sound
      (bind _returnvalue (Game|SpawnActorfromClass "/Game/CutsceneSystem/Blueprints/Cutscene_OverHeadTextActor.Cutscene_OverHeadTextActor_C" (Transformation|GetWorldTransform (Variables|/Script/Engine.Character|GetCapsuleComponent _character_2)) "AlwaysSpawn" 0 0))
      (bind _output_get (Variables|!DONOTTOUCH|SetOverheadText _returnvalue))
      (Transformation|AttachActorToActor _returnvalue _character_2 "" "KeepWorld" "KeepWorld" "KeepWorld" false)
      (Transformation|SetActorRelativeLocation _output_get (Variables|OverheadSettings|GetOverheadTextPosition))
      (bind _ascutscene_overhead (Utilities|Casting|CastToCutscene_Overhead (UserInterface|GetWidget (Variables|/Game/CutsceneSystem/Blueprints/Cutscene_OverHeadTextActor.Cutscene_OverHeadTextActor_C|GetWidget _returnvalue))))
      (Rendering|Components|TextRender|SetText (Variables|/Game/CutsceneSystem/Blueprints/Widgets/Cutscene_OverHead.Cutscene_Overhead_C|GetDialogueText _ascutscene_overhead) _dialogue_2)
      (Class|WidgetComponent|SetDrawSize (Variables|/Game/CutsceneSystem/Blueprints/Cutscene_OverHeadTextActor.Cutscene_OverHeadTextActor_C|GetWidget _returnvalue) (Variables|OverheadSettings|GetOverheadDrawSize))
      (Utilities|IsValid _dialoguesound
        (:Is%20Valid
          (Audio|SpawnSoundatLocation _dialoguesound (Transformation|GetActorLocation _character_3) (Transformation|GetActorRotation _character_3) 1.0 1.0 0.0 0 0)
          (Utilities|FlowControl|Delay (Variables|/Script/Engine.SoundBase|GetDuration _dialoguesound)))
        (:Is%20Not%20Valid
          _))
      (Utilities|FlowControl|Delay _extrawaitfornextscenesec)
      (Actor|DestroyActor (Variables|!DONOTTOUCH|GetOverheadText))
      (SceneCompleteOptions|DialogueSceneComplete))
    (:NewEnumerator2
      ;;[1 1 1] Subtitle Dialogue & Sound (Inside Widget)
      (Utilities|FlowControl|Delay 0.1)
      (bind _foundwidgets (Widget|GetAllWidgetsOfClass "/Game/CutsceneSystem/Blueprints/Widgets/Cutscene_Subtitle.Cutscene_Subtitle_C" true))
      (Variables|/Game/CutsceneSystem/Blueprints/Widgets/Cutscene_Subtitle.Cutscene_Subtitle_C|SetFullText (Utilities|Array|Get(acopy) _foundwidgets) _dialogue_2)
      (Rendering|Components|TextRender|SetText (Variables|/Game/CutsceneSystem/Blueprints/Widgets/Cutscene_Subtitle.Cutscene_Subtitle_C|GetCharName (Utilities|Array|Get(acopy) _foundwidgets)) (Utilities|Text|ToText(Name) (Variables|Cutscene_ActorComponent_C|GetCharacterName (Actor|GetComponentbyClass (Variables|!DONOTTOUCH|GetCharacter) "Cutscene_ActorComponent_C"))))
      (Default|PlayDialogueText (Utilities|Array|Get(acopy) _foundwidgets) _shouldclickfornextscene (Variables|!DONOTTOUCH|GetOwner%20Cutscene) _dialoguesound (Variables|!DONOTTOUCH|GetCharacter) _extrawaitfornextscenesec))))

(event EventBeginPlay
  ;[1 1 1] Register Default Character Speed
  (bind _ascharacter (Utilities|Casting|CastToCharacter (Components|GetOwner)))
  (Variables|!DONOTTOUCH|SetCharacter _ascharacter)
  (Variables|!DONOTTOUCH|SetDefaultCharacterSpeed (Variables|/Script/Engine.CharacterMovementComponent|GetMaxWalkSpeed (Variables|/Script/Engine.Character|GetCharacterMovement (Variables|!DONOTTOUCH|GetCharacter)))))

(event Custom|TeleportCharacterAfterCutscene
  (bind _cutscene_character_setup (Variables|!DONOTTOUCH|GetCutscene%20Character%20Setup))
  (bind _teleportcharacteraftercutscene (Utilities|Struct|BreakCutscene_CharacterSetup _cutscene_character_setup))
  (bind _staticmesh (Variables|/Game/CutsceneSystem/Blueprints/Core/Cutscene_TargetPoint.Cutscene_TargetPoint_C|GetStaticMesh _teleportcharacteraftercutscene))
  ;[1 1 1] Teleport Character After Cutscene
  (Utilities|IsValid _teleportcharacteraftercutscene
    (:Is%20Valid
      (if (Utilities|Enum|Equal(Enum) (Variables|/Game/CutsceneSystem/Blueprints/CutsceneTool.CutsceneTool_C|GetCutsceneStatus (Variables|!DONOTTOUCH|GetOwner%20Cutscene)) "NewEnumerator2") :!label _label
        (Transformation|Teleport (Variables|!DONOTTOUCH|GetCharacter) (Transformation|GetWorldLocation _staticmesh) (Transformation|GetWorldRotation _staticmesh))
        (else
          (Utilities|FlowControl|Delay 0.2)
          (goto _label))))))

(event Custom|RemoveCharacterAfterCutscene
  ;[1 1 1] Remove Character After Cutscene
  (if (Utilities|Struct|BreakCutscene_CharacterSetup (Variables|!DONOTTOUCH|GetCutscene%20Character%20Setup))
    (if (Utilities|Enum|Equal(Enum) (Variables|/Game/CutsceneSystem/Blueprints/CutsceneTool.CutsceneTool_C|GetCutsceneStatus (Variables|!DONOTTOUCH|GetOwner%20Cutscene)) "NewEnumerator2") :!label _label
      (Actor|DestroyActor (Variables|!DONOTTOUCH|GetCharacter))
      (else
        (Utilities|FlowControl|Delay 0.2)
        (goto _label)))))

(fn SetSlowWalkSpeed
  (bind _custom_animations (Variables|!DONOTTOUCH|GetCustom%20Animations))
  (bind _character (Variables|!DONOTTOUCH|GetCharacter))
  (bind _custommovementspeed (Utilities|Struct|BreakCutscene_CharacterCustomAnimations _custom_animations))
  (bind _charactermovement (Variables|/Script/Engine.Character|GetCharacterMovement _character))
  (if (== _custommovementspeed 0.0)
    (Variables|/Script/Engine.CharacterMovementComponent|SetMaxWalkSpeed _charactermovement (Variables|MovementSpeedsForCutscene|GetSlow%20Walk%20Speed))
    (else
      (Variables|/Script/Engine.CharacterMovementComponent|SetMaxWalkSpeed _charactermovement _custommovementspeed))))

(fn SetWalkSpeed
  (bind _custom_animations (Variables|!DONOTTOUCH|GetCustom%20Animations))
  (bind _character (Variables|!DONOTTOUCH|GetCharacter))
  (bind _custommovementspeed (Utilities|Struct|BreakCutscene_CharacterCustomAnimations _custom_animations))
  (bind _charactermovement (Variables|/Script/Engine.Character|GetCharacterMovement _character))
  (if (== _custommovementspeed 0.0)
    (Variables|/Script/Engine.CharacterMovementComponent|SetMaxWalkSpeed _charactermovement (Variables|MovementSpeedsforCutscene|GetWalk%20Speed))
    (else
      (Variables|/Script/Engine.CharacterMovementComponent|SetMaxWalkSpeed _charactermovement _custommovementspeed))))

(fn SetRunSpeed
  (bind _custom_animations (Variables|!DONOTTOUCH|GetCustom%20Animations))
  (bind _character (Variables|!DONOTTOUCH|GetCharacter))
  (bind _custommovementspeed (Utilities|Struct|BreakCutscene_CharacterCustomAnimations _custom_animations))
  (bind _charactermovement (Variables|/Script/Engine.Character|GetCharacterMovement _character))
  (if (== _custommovementspeed 0.0)
    (Variables|/Script/Engine.CharacterMovementComponent|SetMaxWalkSpeed _charactermovement (Variables|MovementSpeedsforCutscene|GetRun%20Speed))
    (else
      (Variables|/Script/Engine.CharacterMovementComponent|SetMaxWalkSpeed _charactermovement _custommovementspeed))))

(fn SetAnimPlayRate
  (bind _custom_animations (Variables|!DONOTTOUCH|GetCustom%20Animations))
  (bind _customanimationplayrate (Utilities|Struct|BreakCutscene_CharacterCustomAnimations _custom_animations))
  (if (== _customanimationplayrate 0.0)
    (Variables|!DONOTTOUCH|SetAnimPlayRate 1.0)
    (else
      (Variables|!DONOTTOUCH|SetAnimPlayRate _customanimationplayrate))))

(fn SelectMontage
  (switch Utilities|FlowControl|Switch|SwitchonCutscene_CharacterActions (Variables|!DONOTTOUCH|GetCharacter%20Actions)
    (:NewEnumerator0
      (CallFunction|CustomMontageValid? (Variables|Animations|GetWaitAnimation)))
    (:NewEnumerator4
      (CallFunction|CustomMontageValid? (Variables|Animations|GetAttackAnimation)))
    (:NewEnumerator5
      (CallFunction|CustomMontageValid? (Variables|Animations|GetTalkAnimation)))
    (:NewEnumerator6
      (CallFunction|CustomMontageValid? (Variables|Animations|GetSitAnimation)))
    (:NewEnumerator10
      (CallFunction|CustomMontageValid? (Variables|Animations|GetTalk-SittingAnimation)))
    (:NewEnumerator7
      (CallFunction|CustomMontageValid? (Variables|Animations|GetCustomAnimation)))
    (:NewEnumerator13
      (CallFunction|CustomMontageValid? (Variables|Animations|GetDieAnimation)))))

(fn SetCustomMoveAnimaSpeed
  (bind _custom_animations (Variables|!DONOTTOUCH|GetCustom%20Animations))
  (bind _character (Variables|!DONOTTOUCH|GetCharacter))
  (bind _custommovementspeed (Utilities|Struct|BreakCutscene_CharacterCustomAnimations _custom_animations))
  (bind _charactermovement (Variables|/Script/Engine.Character|GetCharacterMovement _character))
  (if (== _custommovementspeed 0.0)
    (Variables|/Script/Engine.CharacterMovementComponent|SetMaxWalkSpeed _charactermovement (Variables|MovementSpeedsforCutscene|GetRun%20Speed))
    (else
      (Variables|/Script/Engine.CharacterMovementComponent|SetMaxWalkSpeed _charactermovement _custommovementspeed))))

(fn CustomMontageValid?
  (params (Montage%20to%20Play :type Anim%20Montage%20Object%20Reference))
  (bind _custom_animations (Variables|!DONOTTOUCH|GetCustom%20Animations))
  (bind _customanimation (Utilities|Struct|BreakCutscene_CharacterCustomAnimations _custom_animations))
  (if (Utilities|IsValid _customanimation)
    (Variables|!DONOTTOUCH|SetMontage%20to%20Play _customanimation)
    (else
      (Utilities|IsValid Montage%20to%20Play
        (:Is%20Valid
          (Variables|!DONOTTOUCH|SetMontage%20to%20Play Montage%20to%20Play))))))

(fn ResetWalkSpeed
  (Variables|/Script/Engine.CharacterMovementComponent|SetMaxWalkSpeed (Variables|/Script/Engine.Character|GetCharacterMovement (Variables|!DONOTTOUCH|GetCharacter)) (Variables|!DONOTTOUCH|GetDefaultCharacterSpeed)))

(fn MovementSceneComplete
  (if (Utilities|Enum|Equal(Enum) (Utilities|Struct|BreakCutscene_Settings (Variables|!DONOTTOUCH|GetScene%20Settings)) "NewEnumerator1")
    (Default|SceneComplete (Variables|!DONOTTOUCH|GetOwner%20Cutscene))))

(fn DialogueSceneComplete
  (if (Utilities|Enum|Equal(Enum) (Utilities|Struct|BreakCutscene_Settings (Variables|!DONOTTOUCH|GetScene%20Settings)) "NewEnumerator2")
    (Default|SceneComplete (Variables|!DONOTTOUCH|GetOwner%20Cutscene))))

(fn SetCharacterRagdoll
  (bind _character (Variables|!DONOTTOUCH|GetCharacter))
  (bind _mesh (Variables|/Script/Engine.Character|GetMesh _character))
  (Collision|SetCollisionProfileName _mesh "Ragdoll" true :!class /Script/Engine.PrimitiveComponent)
  (Physics|SetSimulatePhysics _mesh true)
  (Pawn|Components|CharacterMovement|DisableMovement (Variables|/Script/Engine.Character|GetCharacterMovement _character)))