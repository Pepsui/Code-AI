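; BP_CS1 is a cutscene that defines three autoplay camera steps through the cutscene system's command helpers.
; On BeginPlay it stores the player character, then builds each step from commands and fills the Steps array.
; The view blends to a scene camera, switches to Actor2 alongside a forward-move command, then eases back to the player.
; The last two steps display the continue widget.
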(event EventBeginPlay
  ;[1 0.5883 0] If you want to use the player that spawns in, remember to set it in blueprint instead of in editor.
  (Variables|Default|SetActor (Game|GetPlayerCharacter 0))
  (Utilities|FlowControl|Sequence
    (:then_0
      ;[1 1 1] Step 1
      (bind _returnvalue (CallFunction|CmdSwitchCamera (Variables|Default|GetCamera) 1.5 "VTBlend_Linear" 1.0))
      (bind _returnvalue_2 (CallFunction|AddStep (Utilities|Array|MakeArray _returnvalue) true false)))
    (:then_1
      ;[1 1 1] Step 2
      (CallFunction|CmdMoveActorForward (Variables|Default|GetActor2) 0.0 25.0)
      (bind _returnvalue_3 (CallFunction|CmdSwitchCamera (Variables|Default|GetActor2) 0.0 "VTBlend_Linear" 0.0))
      (bind _returnvalue_4 (CallFunction|AddStep (Utilities|Array|MakeArray 0 _returnvalue_3) true true)))
    (:then_2
      ;[1 1 1] Step 3
      (bind _returnvalue_5 (CallFunction|CmdSwitchCamera (Game|GetPlayerCharacter 0) 2.0 "VTBlend_EaseInOut" 1.0))
      (bind _returnvalue_6 (CallFunction|AddStep (Utilities|Array|MakeArray _returnvalue_5) true true)))
    (:then_3
      (Variables|Default|SetSteps (Utilities|Array|MakeArray _returnvalue_2 _returnvalue_4 _returnvalue_6)))))

(fn ConstructionScript
  (|CallParentFunction))