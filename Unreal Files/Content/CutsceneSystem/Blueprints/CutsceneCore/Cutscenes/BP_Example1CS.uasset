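; Example cutscene for the cutscene system: a black-screen story intro, a fade into a scene camera, dialogue from "Donny", then a blend back to the player.
; On BeginPlay, a Sequence builds each step from fade, wait, text, say and camera-switch commands via AddStep, flagged to autoplay or show a continue widget.
; The last pin gathers the steps in order into the Steps array.
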(event EventBeginPlay
  ;[1 1 1] Helps to organise the steps, but feel free to experiment with your own organisation method.
  (Utilities|FlowControl|Sequence
    (:then_0
      ;[0.5972 1 0.1779] Step 1 - Makes Camera Black
      (bind _returnvalue (CallFunction|CmdFadeCamera :To%20Alpha 1.0 :Duration 0.01 :Hold%20when%20Finished true))
      (bind _returnvalue_2 (CallFunction|CmdWait 2.0))
      ;;[1 1 1] This is where you build a step
      (bind _returnvalue_3 (CallFunction|AddStep (Utilities|Array|MakeArray _returnvalue _returnvalue_2) true false)))
    (:then_1
      ;[0.5985 1 0.177] Step 2 - Once Upon a time...
      (bind _returnvalue_4 (CallFunction|CmdStoryText "Once upon a time..."))
      (bind _returnvalue_5 (CallFunction|AddStep (Utilities|Array|MakeArray _returnvalue_4) false true)))
    (:then_2
      ;[0.5985 1 0.177] Step 3 - A young man sought out to make a cutscene system.
      (bind _returnvalue_6 (CallFunction|CmdStoryText "A young man sought out to make his own cutscene system..."))
      (bind _returnvalue_7 (CallFunction|AddStep (Utilities|Array|MakeArray _returnvalue_6) false true)))
    (:then_3
      ;[0.5985 1 0.177] Step 4 - here we go...
      (bind _returnvalue_8 (CallFunction|CmdStoryText "Enough of that. Let's fade in shall we?"))
      (bind _returnvalue_9 (CallFunction|AddStep (Utilities|Array|MakeArray _returnvalue_8) false true)))
    (:then_4
      ;[0.5985 1 0.177] Step 5 - Switch To Camera in Scene
      (bind _returnvalue_10 (CallFunction|CmdSwitchCamera (Variables|Default|GetNew%20View%20Target) 0.0 "VTBlend_Linear" 0.0))
      (bind _returnvalue_11 (CallFunction|CmdWait 0.5))
      ;;[1 1 1] This Step will Auto play into the next one without needing input from the player
      (bind _returnvalue_12 (CallFunction|AddStep (Utilities|Array|MakeArray _returnvalue_10 _returnvalue_11) true false)))
    (:then_5
      ;[0.5972 1 0.1779] Step 6 - Fade Camera into Scene
      (bind _returnvalue_13 (CallFunction|CmdFadeCamera :From%20Alpha 1.0 :Duration 2.0 :Hold%20when%20Finished true))
      (bind _returnvalue_14 (CallFunction|CmdWait 3.0))
      (bind _returnvalue_15 (CallFunction|AddStep (Utilities|Array|MakeArray _returnvalue_13 _returnvalue_14) true false)))
    (:then_6
      ;[0.5972 1 0.1779] Step 7 - Greetings
      (bind _returnvalue_16 (CallFunction|CmdSay "Donny" "Hello there!" "(X=0.000000,Y=-200.000000)"))
      (bind _returnvalue_17 (CallFunction|AddStep (Utilities|Array|MakeArray _returnvalue_16) false true)))
    (:then_7
      ;[0.5972 1 0.1779] Step 8 - Thank you
      (bind _returnvalue_18 (CallFunction|CmdSay "Donny" "Thank you for purchasing my cutscene system. I hope you enjoy it and have fun expanding on it!" "(X=0.000000,Y=-200.000000)"))
      (bind _returnvalue_19 (CallFunction|AddStep (Utilities|Array|MakeArray _returnvalue_18) false true)))
    (:then_8
      ;[0.5972 1 0.1779] Step 9 - Swtich To Player Camera and Clean up for Gameplay
      (bind _returnvalue_20 (CallFunction|CmdSwitchCamera (Game|GetPlayerCharacter 0) 2.0 "VTBlend_Linear" 0.5))
      (bind _returnvalue_21 (CallFunction|AddStep (Utilities|Array|MakeArray _returnvalue_20) true false)))
    (:then_9
      ;[0.5985 1 0.177] This is where we combine all of the steps! Make sure to do it in the right order!
      (Variables|Default|SetSteps (Utilities|Array|MakeArray _returnvalue_3 _returnvalue_5 _returnvalue_7 _returnvalue_9 _returnvalue_12 _returnvalue_15 _returnvalue_17 _returnvalue_19 _returnvalue_21)))))

(fn ConstructionScript
  (|CallParentFunction))