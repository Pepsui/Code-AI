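; Master cutscene actor that plays scripted sequences of steps, then returns the player character to gameplay and optionally destroys itself, its commands and trigger.
; Helper functions spawn command actors (dialogue, camera, actor movement, waits and more) and group them into step actors.
; PlayStep executes a step's commands together and polls their completion on a looping timer.
; Finished steps either autoplay or wait for ContinueCutscene, optionally showing a continue prompt.
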(event Custom|PlayStep
  (if (>= (Variables|Hidden|GetCurrentStepIndex) (Utilities|Array|Length (Variables|Hidden|GetSteps)))
    ;[1 1 1] Returns to gameplay
    (bind _asmain_character_bp (Utilities|Casting|CastToMainCharacterBP (Game|GetPlayerCharacter 0)))
    (Variables|/Game/ThirdPersonBP/Blueprints/MainCharacterBP.MainCharacterBP_C|SetEPlayerState _asmain_character_bp "NewEnumerator0")
    (Variables|/Game/ThirdPersonBP/Blueprints/MainCharacterBP.MainCharacterBP_C|SetCurrentCutscene _asmain_character_bp 0)
    ;[1 1 1] Resets the cutscene index
    (Variables|Hidden|SetCurrentStepIndex 0)
    ;[1 1 1] This removes the cutscene and all assocuated actors. Use this if the cutscene only plays once.
    (if (Variables|Setup|GetDestroyOnCompletion?)
      (|DestroyCutsceneAndCommands))
    (else
      ;[1 1 1] Loops through Command Actions in current Step, executes each one and initiates the CheckStepComplete Timer
      (for _array_element (Variables|/Game/CutsceneSystem/Blueprints/CutsceneCore/BP_Step.BP_Step_C|GetCommands (Utilities|Array|Get(acopy) (Variables|Hidden|GetSteps) (Variables|Hidden|GetCurrentStepIndex)))
        (Default|Execute _array_element (Game|GetPlayerController 0)))
      (bind _returnvalue (Utilities|Time|SetTimerbyEvent (delegate Custom|CheckIfStepcomplete) 0.1 true)))))

(event Custom|CheckIfStepcomplete
  ;[1 1 1] Adds all the Command Actions into an integer
  (Variables|Hidden|SetnumOfCommands (Utilities|Array|Length (Variables|/Game/CutsceneSystem/Blueprints/CutsceneCore/BP_Step.BP_Step_C|GetCommands (Utilities|Array|Get(acopy) (Variables|Hidden|GetSteps) (Variables|Hidden|GetCurrentStepIndex)))))
  (for _array_element (Variables|/Game/CutsceneSystem/Blueprints/CutsceneCore/BP_Step.BP_Step_C|GetCommands (Utilities|Array|Get(acopy) (Variables|Hidden|GetSteps) (Variables|Hidden|GetCurrentStepIndex)))
    ;[1 1 1] Checks if the Command Action has been completed and counts down Number of commands Int
    (if (Variables|/Game/CutsceneSystem/Blueprints/CutsceneCore/BP_MasterCommandCmd.BP_MasterCommandCmd_C|GetCommandComplete? _array_element)
      (Variables|Hidden|SetnumOfCommands (- (Variables|Hidden|GetnumOfCommands) 1))))
  ;[1 1 1] If all commands have finished, stop timer
  (if (<= (Variables|Hidden|GetnumOfCommands) 0)
    (CallFunction|Stoptimer)
    (if (Variables|/Game/CutsceneSystem/Blueprints/CutsceneCore/BP_Step.BP_Step_C|Getautoplay? (Utilities|Array|Get(acopy) (Variables|Hidden|GetSteps) (Variables|Hidden|GetCurrentStepIndex)))
      ;[1 1 1] Add to Current Step index and play next step
      (Variables|Hidden|SetCurrentStepIndex (+ (Variables|Hidden|GetCurrentStepIndex) 1))
      (CallFunction|PlayStep)
      (else
        ;[1 1 1] Wait for player input "Press E"
        (bind _asmain_character_bp (Utilities|Casting|CastToMainCharacterBP (Game|GetPlayerCharacter 0)))
        (Variables|/Game/ThirdPersonBP/Blueprints/MainCharacterBP.MainCharacterBP_C|SetCanContinueCutscene? _asmain_character_bp true)
        (if (Variables|/Game/CutsceneSystem/Blueprints/CutsceneCore/BP_Step.BP_Step_C|GetdisplayContinueWidget? (Utilities|Array|Get(acopy) (Variables|Hidden|GetSteps) (Variables|Hidden|GetCurrentStepIndex)))
          (bind _returnvalue (UserInterface|CreateWidget "/Game/CutsceneSystem/UI/WB_Continue.WB_Continue_C"))
          (UserInterface|Viewport|AddtoViewport _returnvalue 0))))))

(event Custom|Stoptimer
  ;[1 1 1] Stop Timer
  (Utilities|Time|ClearandInvalidateTimerbyHandle (stale Custom|PlayStep _returnvalue)))

(event EventContinueCutscene
  ;[1 1 1] Player Inputs to Continue the cutscene
  (bind _asmain_character_bp (Utilities|Casting|CastToMainCharacterBP (Game|GetPlayerCharacter 0)))
  (Variables|/Game/ThirdPersonBP/Blueprints/MainCharacterBP.MainCharacterBP_C|SetCanContinueCutscene? _asmain_character_bp false)
  (Viewport|RemoveAllWidgets)
  ;[1 1 1] Add to Current Step index and play next step
  (Variables|Hidden|SetCurrentStepIndex (+ (Variables|Hidden|GetCurrentStepIndex) 1))
  (CallFunction|PlayStep))

(fn ConstructionScript
  (Rendering|Components|TextRender|SetText (Variables|Default|GetTextRender) (Variables|Setup|GetCutscene%20Name)))

(fn CmdSay
  (params (Name :type Text) (Dialogue :type Text) (Offset :type Vector%202D%20Structure))
  (bind _returnvalue (Game|SpawnActorfromClass "/Game/CutsceneSystem/Blueprints/CutsceneCore/Commands/BP_SayCmd.BP_SayCmd_C" (Math|Transform|MakeTransform "0, 0, 0" "0, 0, 0" "1,1,1") "Undefined" 0 Name Dialogue Offset 0))
  (return _returnvalue))

(fn CmdStoryText
  (params (Dialogue :type Text))
  (bind _returnvalue (Game|SpawnActorfromClass "/Game/CutsceneSystem/Blueprints/CutsceneCore/Commands/BP_StoryTextBoxCmd.BP_StoryTextBoxCmd_C" (Math|Transform|MakeTransform "0, 0, 0" "0, 0, 0" "1,1,1") "Undefined" 0 Dialogue 0))
  (return _returnvalue))

(fn CmdFadeCamera
  (params (From%20Alpha :type Float%20%28single-precision%29) (To%20Alpha :type Float%20%28single-precision%29) (Duration :type Float%20%28single-precision%29) (Color :type Linear%20Color%20Structure) (Should%20Fade%20Audio :type Boolean) (Hold%20when%20Finished :type Boolean))
  (bind _returnvalue (Game|SpawnActorfromClass "/Game/CutsceneSystem/Blueprints/CutsceneCore/Commands/BP_FadeCameraCmd.BP_FadeCameraCmd_C" (Math|Transform|MakeTransform "0, 0, 0" "0, 0, 0" "1,1,1") "Undefined" 0 From%20Alpha To%20Alpha Duration Color Should%20Fade%20Audio Hold%20when%20Finished 0))
  (return _returnvalue))

(fn CmdMoveActor
  (params (Actor :type Actor%20Object%20Reference) (TargetLoc :type Vector) (TimeTakenInSeconds :type Float%20%28single-precision%29))
  (bind _returnvalue (Game|SpawnActorfromClass "/Game/CutsceneSystem/Blueprints/CutsceneCore/Commands/BP_MoveActorCmd.BP_MoveActorCmd_C" (Math|Transform|MakeTransform "0, 0, 0" "0, 0, 0" "1,1,1") "Undefined" 0 Actor TargetLoc TimeTakenInSeconds 0))
  (return _returnvalue))

(fn CmdSpawnActor
  (params (ClassToSpawn :type Actor%20Class%20Reference) (Spawn%20Transform :type Transform))
  (bind _returnvalue (Game|SpawnActorfromClass "/Game/CutsceneSystem/Blueprints/CutsceneCore/Commands/BP_SpawnActorCmd.BP_SpawnActorCmd_C" (Math|Transform|MakeTransform "0, 0, 0" "0, 0, 0" "1,1,1") "Undefined" 0 ClassToSpawn Spawn%20Transform 0))
  (return _returnvalue))

(fn CmdSwitchCamera
  (params (New%20View%20Target :type Actor%20Object%20Reference) (Blend%20Time :type Float%20%28single-precision%29) (Blend%20Func :type EViewTargetBlendFunction%20Enum :default "VTBlend_Linear") (Blend%20Exp :type Float%20%28single-precision%29))
  (bind _returnvalue (Game|SpawnActorfromClass "/Game/CutsceneSystem/Blueprints/CutsceneCore/Commands/BP_SwitchCameraCmd.BP_SwitchCameraCmd_C" (Math|Transform|MakeTransform "0, 0, 0" "0, 0, 0" "1,1,1") "Undefined" 0 New%20View%20Target Blend%20Time Blend%20Func Blend%20Exp 0))
  (return _returnvalue))

(fn CmdTurntoFaceActor
  (params (Actor :type Actor%20Object%20Reference) (targetActor :type Actor%20Object%20Reference) (TimeTakenInSeconds :type Float%20%28single-precision%29))
  (bind _returnvalue (Game|SpawnActorfromClass "/Game/CutsceneSystem/Blueprints/CutsceneCore/Commands/BP_TurnToFaceActorCmd.BP_TurnToFaceActorCmd_C" (Math|Transform|MakeTransform "0, 0, 0" "0, 0, 0" "1,1,1") "Undefined" 0 Actor targetActor TimeTakenInSeconds 0))
  (return _returnvalue))

(fn CmdTurntoRotation
  (params (Actor :type Actor%20Object%20Reference) (TimeTakenInSeconds :type Float%20%28single-precision%29) (TargetRot :type Rotator))
  (bind _returnvalue (Game|SpawnActorfromClass "/Game/CutsceneSystem/Blueprints/CutsceneCore/Commands/BP_TurnToRotCmd.BP_TurnToRotCmd_C" (Math|Transform|MakeTransform "0, 0, 0" "0, 0, 0" "1,1,1") "Undefined" 0 Actor TimeTakenInSeconds TargetRot 0))
  (return _returnvalue))

(fn CmdWait
  (params (Duration :type Float%20%28single-precision%29))
  (bind _returnvalue (Game|SpawnActorfromClass "/Game/CutsceneSystem/Blueprints/CutsceneCore/Commands/BP_WaitCmd.BP_WaitCmd_C" (Math|Transform|MakeTransform "0, 0, 0" "0, 0, 0" "1,1,1") "Undefined" 0 Duration 0))
  (return _returnvalue))

(fn AddStep
  (params (Commands :type Array%20of%20BP%20Master%20Command%20Cmd%20Object%20References) (autoplay? :type Boolean) (displayContinueWidget? :type Boolean))
  (bind _returnvalue (Game|SpawnActorfromClass "/Game/CutsceneSystem/Blueprints/CutsceneCore/BP_Step.BP_Step_C" (Math|Transform|MakeTransform "0, 0, 0" "0, 0, 0" "1,1,1") "Undefined" 0 Commands autoplay? displayContinueWidget? 0))
  (return _returnvalue))

(fn CmdMoveActorForward
  (params (Actor :type Actor%20Object%20Reference) (Time%20Taken%20in%20Seconds :type Float%20%28single-precision%29) (UnitsToMove :type Float%20%28single-precision%29))
  (bind _returnvalue (Game|SpawnActorfromClass "/Game/CutsceneSystem/Blueprints/CutsceneCore/Commands/BP_MoveActorForwardCmd.BP_MoveActorForwardCmd_C" (Math|Transform|MakeTransform "0, 0, 0" "0, 0, 0" "1,1,1") "Undefined" 0 Actor Time%20Taken%20in%20Seconds UnitsToMove 0))
  (return _returnvalue))

(fn CmdDestroyActor
  (params (ActorToDestroy :type Actor%20Object%20Reference))
  (bind _returnvalue (Game|SpawnActorfromClass "/Game/CutsceneSystem/Blueprints/CutsceneCore/Commands/BP_DestroyActorCmd.BP_DestroyActorCmd_C" (Math|Transform|MakeTransform "0, 0, 0" "0, 0, 0" "1,1,1") "Undefined" 0 ActorToDestroy 0))
  (return _returnvalue))

(fn CmdClassicTextBox
  (params (Line1 :type Text) (Line2 :type Text) (Line3 :type Text) (TypeWriterDelay :type Float%20%28single-precision%29))
  (bind _returnvalue (Game|SpawnActorfromClass "/Game/CutsceneSystem/Blueprints/CutsceneCore/Commands/BP_ClassicTextBoxCmd.BP_ClassicTextBoxCmd_C" (Math|Transform|MakeTransform "0, 0, 0" "0, 0, 0" "1,1,1") "Undefined" 0 Line1 Line2 Line3 TypeWriterDelay 0.4 0))
  (return _returnvalue))