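; Cutscene command that smoothly moves an actor from its current location to a target location over a set time.
; On Execute it records the start location and scales a timeline's play rate by the inverse of the duration.
; Each timeline update lerps the actor's position with sweep enabled, and the command flags itself complete when the timeline finishes.
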(event EventExecute
  (params (PlayerController :type Player%20Controller%20Object%20Reference))
  (|CallParentFunction PlayerController)
  (Variables|Default|SetStartLoc (Transformation|GetActorLocation (Variables|Default|GetActor)))
  (Components|Timeline|SetPlayRate (Variables|Default|GetMoveTimeline) (/ 1.0 (Variables|Default|GetTimeTakenInSeconds)))
  (bind _alpha (Timeline|MoveTimeline PlayFromStart)
    (:Update
      (Transformation|SetActorLocation (Variables|Default|GetActor) (Math|Vector|Lerp(Vector) (Variables|Default|GetStartLoc) (Variables|Default|GetTargetLoc) _alpha) true false))
    (:Finished
      (Variables|Default|SetCommandComplete? true))))

(fn ConstructionScript
  (|CallParentFunction))