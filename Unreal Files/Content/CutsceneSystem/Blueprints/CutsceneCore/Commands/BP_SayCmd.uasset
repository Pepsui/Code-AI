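; BP_SayCmd is a cutscene command that shows a line of dialogue with a speaker name on screen.
; On Execute it calls the parent, creates a WB_Say widget, fills in the Name and Dialogue text, shifts it by Offset and adds it to the viewport.
; It sets CommandComplete after a brief fixed delay, without waiting for input or removing the widget itself.
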(event EventExecute
  (params (PlayerController :type Player%20Controller%20Object%20Reference))
  (|CallParentFunction PlayerController)
  (bind _returnvalue (UserInterface|CreateWidget "/Game/CutsceneSystem/UI/WB_Say.WB_Say_C"))
  (Rendering|Components|TextRender|SetText (Variables|/Game/CutsceneSystem/UI/WB_Say.WB_Say_C|GetText_Name _returnvalue) (Variables|Default|GetName))
  (Rendering|Components|TextRender|SetText (Variables|/Game/CutsceneSystem/UI/WB_Say.WB_Say_C|GetText_Dialogue _returnvalue) (Variables|Default|GetDialogue))
  (Class|Widget|SetRenderTranslation _returnvalue (Variables|Default|GetOffset))
  (UserInterface|Viewport|AddtoViewport _returnvalue 0)
  (Utilities|FlowControl|Delay 0.2)
  (Variables|Default|SetCommandComplete? true))

(fn ConstructionScript
  (|CallParentFunction))