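; BP_TurnToRotCmd is a cutscene command that smoothly turns an actor to a target yaw over a set number of seconds.
; On Execute it scales a timeline's play rate by the duration, then lerps from the starting rotation along the shortest path each update.
; Only yaw changes; pitch and roll keep their starting values.
; It marks the command complete when the timeline finishes.
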(event EventExecute
  (params (PlayerController :type Player%20Controller%20Object%20Reference))
  (|CallParentFunction PlayerController)
  (Components|Timeline|SetPlayRate (Variables|Default|GetTurnTimeline) (/ 1.0 (Variables|Default|GetTimeTakenInSeconds)))
  (Variables|Default|SetStartRot (Transformation|GetActorRotation (Variables|Default|GetActor)))
  (bind _alpha (Timeline|TurnTimeline PlayFromStart)
    (:Update
      (Transformation|SetActorRotation (Variables|Default|GetActor) (Math|Rotator|Lerp(Rotator) (Variables|Default|GetStartRot) (Math|Rotator|MakeRotator (.Roll (Math|Rotator|BreakRotator (Variables|Default|GetStartRot))) (.Pitch (Math|Rotator|BreakRotator (Variables|Default|GetStartRot))) (.Yaw (Math|Rotator|BreakRotator (Variables|Default|GetTargetRot)))) _alpha true)))
    (:Finished
      (Variables|Default|SetCommandComplete? true))))

(fn ConstructionScript
  (|CallParentFunction))