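; Cutscene command that switches the camera by blending the player's view to a configured target actor.
; On Execute it runs the parent logic, then calls SetViewTargetWithBlend on player controller 0 with the configured blend time, function and exponent.
; It ignores the passed-in controller, waits for the blend time with a Delay, then sets CommandComplete to true.
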(event EventExecute
  (params (PlayerController :type Player%20Controller%20Object%20Reference))
  (|CallParentFunction PlayerController)
  (Game|Player|SetViewTargetwithBlend (Game|GetPlayerController 0) (Variables|Default|GetNew%20View%20Target) (Variables|Default|GetBlend%20Time) (Variables|Default|GetBlend%20Func) (Variables|Default|GetBlend%20Exp) false)
  (Utilities|FlowControl|Delay (Variables|Default|GetBlend%20Time))
  (Variables|Default|SetCommandComplete? true))

(fn ConstructionScript
  (|CallParentFunction))