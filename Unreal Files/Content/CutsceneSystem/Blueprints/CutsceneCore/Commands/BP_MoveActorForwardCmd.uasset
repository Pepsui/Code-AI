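; Cutscene command that slides a target actor forward along its facing direction by a set distance over a set duration.
; On Execute it captures start and end locations, then scales a timeline's play rate by the inverse of the duration.
; Each update lerps the actor with a swept move, so blocking collision can stop it short.
; The command flags itself complete when the timeline finishes.
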(event EventExecute
  (params (PlayerController :type Player%20Controller%20Object%20Reference))
  (bind _actor (Variables|Default|GetActor))
  (bind _returnvalue (Transformation|GetActorLocation _actor))
  (|CallParentFunction PlayerController)
  (Variables|Default|SetStartLoc _returnvalue)
  (Variables|Default|SetTargetLoc (+ _returnvalue (* (Transformation|GetActorForwardVector _actor) (Variables|Default|GetUnitsToMove))))
  (Components|Timeline|SetPlayRate (Variables|Default|GetMoveTimeline) (/ 1.0 (Variables|Default|GetTime%20Taken%20in%20Seconds)))
  (bind _alpha (Timeline|MoveTimeline PlayFromStart)
    (:Update
      (Transformation|SetActorLocation (Variables|Default|GetActor) (Math|Vector|Lerp(Vector) (Variables|Default|GetStartLoc) (Variables|Default|GetTargetLoc) _alpha) true false))
    (:Finished
      (Variables|Default|SetCommandComplete? true))))

(fn ConstructionScript
  (|CallParentFunction))