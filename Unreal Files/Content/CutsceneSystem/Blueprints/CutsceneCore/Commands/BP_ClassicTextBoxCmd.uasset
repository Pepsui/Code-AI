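; Cutscene command that shows a classic three-line text box with a typewriter effect.
; Execute adds a WB_ClassicTextBox widget to the viewport and gathers the three lines for display.
; TypeWriter re-calls itself after delays, appending one character using the displayed text length as cursor, and pausing between lines.
; It flags CommandComplete after the third line; SkipTypewriter halts the loop without filling remaining text here.
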(event Custom|TypeWriter
  (bind _widget (Variables|Default|GetWidget))
  (Variables|Default|Setcurrentstringtodisplay (Utilities|String|ToString(Text) (Utilities|Array|Get(acopy) (Variables|Default|GetDialogueArray) (Variables|Default|Getindex))))
  (Variables|Default|SetcharsInLine (Utilities|String|Len (Utilities|String|ToString(Text) (Utilities|Array|Get(acopy) (Variables|Default|GetDialogueArray) (Variables|Default|Getindex)))))
  (Rendering|Components|TextRender|SetText (Utilities|Array|Get(acopy) (Utilities|Array|MakeArray (Variables|/Game/CutsceneSystem/UI/WB_ClassicTextBox.WB_ClassicTextBox_C|GetText_Line1 _widget) (Variables|/Game/CutsceneSystem/UI/WB_ClassicTextBox.WB_ClassicTextBox_C|GetText_Line2 _widget) (Variables|/Game/CutsceneSystem/UI/WB_ClassicTextBox.WB_ClassicTextBox_C|GetText_Line3 _widget)) (Variables|Default|Getindex)) (Utilities|Text|ToText(String) (Utilities|String|Append (Utilities|String|ToString(Text) (Class|TextBlock|GetText (Utilities|Array|Get(acopy) (Utilities|Array|MakeArray (Variables|/Game/CutsceneSystem/UI/WB_ClassicTextBox.WB_ClassicTextBox_C|GetText_Line1 _widget) (Variables|/Game/CutsceneSystem/UI/WB_ClassicTextBox.WB_ClassicTextBox_C|GetText_Line2 _widget) (Variables|/Game/CutsceneSystem/UI/WB_ClassicTextBox.WB_ClassicTextBox_C|GetText_Line3 _widget)) (Variables|Default|Getindex)))) (Utilities|String|GetSubstring (Variables|Default|Getcurrentstringtodisplay) (Utilities|String|Len (Utilities|String|ToString(Text) (Class|TextBlock|GetText (Utilities|Array|Get(acopy) (Utilities|Array|MakeArray (Variables|/Game/CutsceneSystem/UI/WB_ClassicTextBox.WB_ClassicTextBox_C|GetText_Line1 _widget) (Variables|/Game/CutsceneSystem/UI/WB_ClassicTextBox.WB_ClassicTextBox_C|GetText_Line2 _widget) (Variables|/Game/CutsceneSystem/UI/WB_ClassicTextBox.WB_ClassicTextBox_C|GetText_Line3 _widget)) (Variables|Default|Getindex)))))))))
  (if (not (Variables|Default|GetSkipTypewriter))
    (if (>= (Utilities|String|Len (Utilities|String|ToString(Text) (Class|TextBlock|GetText (Utilities|Array|Get(acopy) (Utilities|Array|MakeArray (Variables|/Game/CutsceneSystem/UI/WB_ClassicTextBox.WB_ClassicTextBox_C|GetText_Line1 _widget) (Variables|/Game/CutsceneSystem/UI/WB_ClassicTextBox.WB_ClassicTextBox_C|GetText_Line2 _widget) (Variables|/Game/CutsceneSystem/UI/WB_ClassicTextBox.WB_ClassicTextBox_C|GetText_Line3 _widget)) (Variables|Default|Getindex))))) (Variables|Default|GetcharsInLine))
      (bind _output_get (Variables|Default|Setindex (+ (Variables|Default|Getindex) 1)))
      (if (>= _output_get 3)
        (Variables|Default|Setindex 0)
        (Variables|Default|SetCommandComplete? true)
        (else
          (Utilities|FlowControl|Delay (Variables|Default|GetDelayBetweenLines))
          (CallFunction|TypeWriter)))
      (else
        (Utilities|FlowControl|Delay (Variables|Default|GetTypeWriterDelay))
        (CallFunction|TypeWriter)))))

(event EventExecute
  (params (PlayerController :type Player%20Controller%20Object%20Reference))
  (|CallParentFunction 0)
  (bind _returnvalue (UserInterface|CreateWidget "/Game/CutsceneSystem/UI/WB_ClassicTextBox.WB_ClassicTextBox_C"))
  (bind _output_get (Variables|Default|SetWidget _returnvalue))
  (UserInterface|Viewport|AddtoViewport _output_get 0)
  (Variables|Default|SetDialogueArray (Utilities|Array|MakeArray (Variables|Default|GetLine1) (Variables|Default|GetLine2) (Variables|Default|GetLine3)))
  (CallFunction|TypeWriter))

(fn ConstructionScript
  (|CallParentFunction))