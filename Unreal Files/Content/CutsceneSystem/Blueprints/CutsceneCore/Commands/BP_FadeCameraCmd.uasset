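; BP_FadeCameraCmd is a cutscene system command that fades the player camera.
; On Execute it calls the parent, then starts a camera fade on player 0's camera manager using its alpha, duration, color, audio-fade and hold settings.
; It waits for the fade duration with a Delay, then sets CommandComplete to mark the command finished.
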(event EventExecute
  (params (PlayerController :type Player%20Controller%20Object%20Reference))
  (|CallParentFunction PlayerController)
  (CameraFades|StartCameraFade (Game|GetPlayerCameraManager 0) (Variables|Default|GetFrom%20Alpha) (Variables|Default|GetTo%20Alpha) (Variables|Default|GetDuration) (Variables|Default|GetColor) (Variables|Default|GetShould%20Fade%20Audio) (Variables|Default|GetHold%20when%20Finished))
  (Utilities|FlowControl|Delay (Variables|Default|GetDuration))
  (Variables|Default|SetCommandComplete? true))

(fn ConstructionScript
  (|CallParentFunction))