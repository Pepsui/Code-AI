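; Player controller component for the cutscene system that owns the dialogue subtitle widget and provides input toggling.
; Shortly after BeginPlay, Setup creates the Cutscene_Subtitle widget, stores it as DialogueSubtitle and adds it to the viewport.
; DisableInputEvent and EnableInputEvent cast the owner to PlayerController and switch input on that controller itself, passing player controller 0.
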(event Custom|DisableInputEvent
  ;[1 1 1] Disable & Enable Input for Player Character
  (bind _asplayer_controller (Utilities|Casting|CastToPlayerController (Components|GetOwner)))
  (Input|DisableInput _asplayer_controller (Game|GetPlayerController 0)))

(event Custom|EnableInputEvent
  ;[1 1 1] Disable & Enable Input for Player Character
  (bind _asplayer_controller (Utilities|Casting|CastToPlayerController (Components|GetOwner)))
  (Input|EnableInput _asplayer_controller (Game|GetPlayerController 0)))

(event EventBeginPlay
  (Utilities|FlowControl|Delay 0.2)
  ;[1 1 1] Create Subtitle Widget & Hide it
  (CallFunction|Setup))

(fn Setup
  (bind _returnvalue (UserInterface|CreateWidget "/Game/CutsceneSystem/Blueprints/Widgets/Cutscene_Subtitle.Cutscene_Subtitle_C"))
  (bind _output_get (Variables|!DONOTTOUCH|SetDialogueSubtitle _returnvalue))
  (UserInterface|Viewport|AddtoViewport _output_get 0))