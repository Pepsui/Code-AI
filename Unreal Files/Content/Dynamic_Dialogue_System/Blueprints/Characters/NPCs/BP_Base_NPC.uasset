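; Base NPC character for the Dynamic Dialogue System, demonstrating how an actor engages the player in dialogue.
; The interact area registers it with BP_Player_Character, Interaction requests dialogue through AC_Dialogue_Component, and leaving mid-dialogue disengages it.
; Activate and deactivate events maintain the IsInDialogue gate, and another event plays montages.
; Sample dialogue-fired function and condition-check events report back to the player's dialogue component, the check always returning false.
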(event OnComponentBeginOverlap(Interact_Area)
  (params (OverlappedComponent :type Primitive%20Component%20Object%20Reference) (OtherActor :type Actor%20Object%20Reference) (OtherComp :type Primitive%20Component%20Object%20Reference) (OtherBodyIndex :type Integer) (bFromSweep :type Boolean) (SweepResult :type Hit%20Result%20Structure%20%28by%20ref%29))
  ;[1 0 0] Demonstration: Interaction
  ;
  ; You may have your own interaction system, and thats GREAT!
  ; This section is only for demonstration purposes and the only code actually required in your NPCs is what is below.
  ; to get an NPC, sign, or trigger to engage the player in dialogue only requires that the actor implement the "BPI_Dialogue" interface,
  ; the Actor needs to implement the "AC_Dialogue_Component",
  ; And the actor needs to use the "Request Dialogue" function, and thats it! You are DONE!
  (bind _asbp_player_character (Utilities|Casting|CastToBP_Player_Character OtherActor))
  (Class|BPIInteract|RegisterInteractable(Message) _asbp_player_character self))

(event OnComponentEndOverlap(Interact_Area)
  (params (OverlappedComponent :type Primitive%20Component%20Object%20Reference) (OtherActor :type Actor%20Object%20Reference) (OtherComp :type Primitive%20Component%20Object%20Reference) (OtherBodyIndex :type Integer))
  ;[1 0 0] Demonstration: Interaction
  ;
  ; You may have your own interaction system, and thats GREAT!
  ; This section is only for demonstration purposes and the only code actually required in your NPCs is what is below.
  ; to get an NPC, sign, or trigger to engage the player in dialogue only requires that the actor implement the "BPI_Dialogue" interface,
  ; the Actor needs to implement the "AC_Dialogue_Component",
  ; And the actor needs to use the "Request Dialogue" function, and thats it! You are DONE!
  (bind _asbp_player_character (Utilities|Casting|CastToBP_Player_Character OtherActor))
  (Class|BPIInteract|UnregisterInteractable(Message) _asbp_player_character)
  (if (Variables|Default|GetIs_In_Dialogue?)
    ;;[1 1 1] This section is only for demonstration purposes, and none of this code is required to funtion. Howeve you should read it to find out how to implement certain functionality.
    ;;;[1 1 1] This is how you can disengage dialogue with the player under certain circumstances. For this demonstration, we dont want the player character engaging an NPC in dialogue while far away, but if you wanted a tutorial message, you do not need to fire this.
    (Default|DisengageDialogue (Variables|/Game/Dynamic_Dialogue_System/Blueprints/Components/AC_Dialogue_Component.AC_Dialogue_Component_C|GetPC_Dialogue_Component (Variables|Default|GetAC_Dialogue_Component)))))

(event Custom|Test_Condition_Check
  ;[1 0 0] Demonstration: Interaction
  ;
  ; You may have your own interaction system, and thats GREAT!
  ; This section is only for demonstration purposes and the only code actually required in your NPCs is what is below.
  ; to get an NPC, sign, or trigger to engage the player in dialogue only requires that the actor implement the "BPI_Dialogue" interface,
  ; the Actor needs to implement the "AC_Dialogue_Component",
  ; And the actor needs to use the "Request Dialogue" function, and thats it! You are DONE!
  ;;[1 1 1] This section is only for demonstration purposes, and none of this code is required to funtion. Howeve you should read it to find out how to implement certain functionality.
  ;;;[1 1 1] This dialogue supports condition checks, and may not be necessary in all games. however, if it is necessary in YOUR game, you can resolve condition checks in theis manner. The condition must always return a Boolean value in order to function. For example, if you want to make sure the player has enough money, you could cast to that player and ask the result. Then you can translate that result into a "Coins > Required?" statement and return the Boolean value.
  (Class|BPIDialogue|ConfirmDialogueConditionCheck(Message) (Variables|/Game/Dynamic_Dialogue_System/Blueprints/Components/AC_Dialogue_Component.AC_Dialogue_Component_C|GetPC_Dialogue_Component (Variables|Default|GetAC_Dialogue_Component)) false))

(event Custom|Test_Function
  ;[1 0 0] Demonstration: Interaction
  ;
  ; You may have your own interaction system, and thats GREAT!
  ; This section is only for demonstration purposes and the only code actually required in your NPCs is what is below.
  ; to get an NPC, sign, or trigger to engage the player in dialogue only requires that the actor implement the "BPI_Dialogue" interface,
  ; the Actor needs to implement the "AC_Dialogue_Component",
  ; And the actor needs to use the "Request Dialogue" function, and thats it! You are DONE!
  ;;[1 1 1] This section is only for demonstration purposes, and none of this code is required to funtion. Howeve you should read it to find out how to implement certain functionality.
  ;;;[1 1 1] This Dialogue system supports firing events to the NPCs blueprint by its function name. You may not need this functionality, but if you want to implement it, you just need to create a function, and when you want to return the function as complete, end it with the "Fired_Event_Complete" message targetting the "AC_Dialogue_Component"s "PC_Dialogue_Component" component.
  ;;;
  ;;; You may be wondering how to implement this functionality into the Player Character, However this is a One Way system for a reason. Filling your Character Blueprint with Tons of function calls will be very disorderly, and have you searching for bugs very quickly. So for neatness sake, all of your functions must be located in the NPC or dialogue participant. If you want a function to fire in the player, tie it to the NPC or Dialogue Participant for easy testing.
  (Character|Jump)
  (Utilities|FlowControl|Delay 5.0)
  (Class|BPIDialogue|FiredEventComplete(Message) (Variables|/Game/Dynamic_Dialogue_System/Blueprints/Components/AC_Dialogue_Component.AC_Dialogue_Component_C|GetPC_Dialogue_Component (Variables|Default|GetAC_Dialogue_Component))))

(event EventInteraction
  (params (Instigator :type Actor%20Object%20Reference))
  ;[1 0 0] Demonstration: Interaction
  ;
  ; You may have your own interaction system, and thats GREAT!
  ; This section is only for demonstration purposes and the only code actually required in your NPCs is what is below.
  ; to get an NPC, sign, or trigger to engage the player in dialogue only requires that the actor implement the "BPI_Dialogue" interface,
  ; the Actor needs to implement the "AC_Dialogue_Component",
  ; And the actor needs to use the "Request Dialogue" function, and thats it! You are DONE!
  (if (not (Variables|Default|GetIs_In_Dialogue?))
    (Variables|Default|SetIs_In_Dialogue? true)
    ;[1 1 1] This is the only function you need to fire to engage the player in dialogue.
    ; Just plug in the execute pin, Plug in a pin that references the Player Character,
    ; and set your own "AC_Dialogue_Component" to the target and you are DONE!
    (Default|RequestDialogue (Variables|Default|GetAC_Dialogue_Component) Instigator)))

(event EventActivateDialogue
  ;[1 0 0] Demonstration: Interaction
  ;
  ; You may have your own interaction system, and thats GREAT!
  ; This section is only for demonstration purposes and the only code actually required in your NPCs is what is below.
  ; to get an NPC, sign, or trigger to engage the player in dialogue only requires that the actor implement the "BPI_Dialogue" interface,
  ; the Actor needs to implement the "AC_Dialogue_Component",
  ; And the actor needs to use the "Request Dialogue" function, and thats it! You are DONE!
  ;;[1 1 1] This section is only for demonstration purposes, and none of this code is required to funtion. Howeve you should read it to find out how to implement certain functionality.
  ;;;[1 1 1] Sometimes, it may not matter if the NPC is in Dialogue or not. But, most times it does. These 2 events are the logic gates that control what the NPC does when Dialogue begins, or ends.
  (Variables|Default|SetIs_In_Dialogue? true))

(event EventDeactivateDialogue
  ;[1 0 0] Demonstration: Interaction
  ;
  ; You may have your own interaction system, and thats GREAT!
  ; This section is only for demonstration purposes and the only code actually required in your NPCs is what is below.
  ; to get an NPC, sign, or trigger to engage the player in dialogue only requires that the actor implement the "BPI_Dialogue" interface,
  ; the Actor needs to implement the "AC_Dialogue_Component",
  ; And the actor needs to use the "Request Dialogue" function, and thats it! You are DONE!
  ;;[1 1 1] This section is only for demonstration purposes, and none of this code is required to funtion. Howeve you should read it to find out how to implement certain functionality.
  ;;;[1 1 1] Sometimes, it may not matter if the NPC is in Dialogue or not. But, most times it does. These 2 events are the logic gates that control what the NPC does when Dialogue begins, or ends.
  (Variables|Default|SetIs_In_Dialogue? false))

(event EventSkeletalMeshPlayAnimation
  (params (Montage_To_Play :type Anim%20Montage%20Object%20Reference))
  ;[1 0 0] Demonstration: Interaction
  ;
  ; You may have your own interaction system, and thats GREAT!
  ; This section is only for demonstration purposes and the only code actually required in your NPCs is what is below.
  ; to get an NPC, sign, or trigger to engage the player in dialogue only requires that the actor implement the "BPI_Dialogue" interface,
  ; the Actor needs to implement the "AC_Dialogue_Component",
  ; And the actor needs to use the "Request Dialogue" function, and thats it! You are DONE!
  ;;[1 1 1] This section is only for demonstration purposes, and none of this code is required to funtion. Howeve you should read it to find out how to implement certain functionality.
  ;;;[1 1 1] You may not want the dialogue system controlling animation, however if you do, this is how you implement playing montages from the "AC_Dialogue_Component"
  (Animation|PlayAnimMontage Montage_To_Play 1.0 "None"))

(fn ConstructionScript)