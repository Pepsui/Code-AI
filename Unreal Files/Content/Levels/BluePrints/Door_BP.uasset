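; Sliding door Blueprint that moves its Pivot component along the relative Y axis to open and close.
; BeginPlay reverses a separate timeline from its end to drive the Pivot's starting motion.
; An Open/Close event alternates the DoorMovement timeline forward and backward through a FlipFlop.
; Component A's overlap events also play that timeline forward when a Robot enters and reverse it when one leaves.
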(event OnComponentBeginOverlap(a)
  (params (OverlappedComponent :type Primitive%20Component%20Object%20Reference) (OtherActor :type Actor%20Object%20Reference) (OtherComp :type Primitive%20Component%20Object%20Reference) (OtherBodyIndex :type Integer) (bFromSweep :type Boolean) (SweepResult :type Hit%20Result%20Structure%20%28by%20ref%29))
  (Utilities|Casting|CastToRobot OtherActor)
  (bind _newtrack_0 (Timeline|Door%20Movement PlayFromStart)
    (:Update
      (Transformation|SetRelativeLocation (Variables|Default|GetPivot) (Math|Vector|MakeVector 0.0 _newtrack_0 0.0) false false))))

(event OnComponentEndOverlap(a)
  (params (OverlappedComponent :type Primitive%20Component%20Object%20Reference) (OtherActor :type Actor%20Object%20Reference) (OtherComp :type Primitive%20Component%20Object%20Reference) (OtherBodyIndex :type Integer))
  (Utilities|Casting|CastToRobot OtherActor)
  (bind _newtrack_0 (Timeline|Door%20Movement ReverseFromEnd)
    (:Update
      (Transformation|SetRelativeLocation (Variables|Default|GetPivot) (Math|Vector|MakeVector 0.0 _newtrack_0 0.0) false false))))

(event Custom|Open/Close
  (Class|PrimitiveComponent|BoxOverlapComponent :self (Variables|Default|Geta))
  (Utilities|FlowControl|FlipFlop
    (:A
      (bind _newtrack_0 (Timeline|Door%20Movement PlayFromStart)
        (:Update
          (Transformation|SetRelativeLocation (Variables|Default|GetPivot) (Math|Vector|MakeVector 0.0 _newtrack_0 0.0) false false))))
    (:B
      (Timeline|Door%20Movement ReverseFromEnd))))

(event EventBeginPlay
  (bind _newtrack_0 (Timeline|Timeline_0 ReverseFromEnd)
    (:Update
      (Transformation|SetRelativeLocation (Variables|Default|GetPivot) (Math|Vector|MakeVector 0.0 _newtrack_0 0.0) false false))))

(fn ConstructionScript)