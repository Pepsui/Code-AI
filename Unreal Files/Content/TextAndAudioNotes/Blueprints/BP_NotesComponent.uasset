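; Actor component that lets the player pick up text and audio notes and review them in a journal.
; A camera line trace tracks the note in view; reading it opens a text widget, or plays 2D audio with its own widget.
; Picked-up notes store their Settings in the journal list, then the level actor is destroyed.
; It also manages journal display, closing active notes and switching between game and UI input.
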(event Custom|E_StopActiveAudioNote
  ;[1 0.2172 0] Stop audio note
  (Utilities|FlowControl|Sequence
    (:then_0
      (Utilities|IsValid (Variables|State|GetActiveAudioNoteWidget)
        (:Is%20Valid
          (Widget|RemovefromParent (Variables|State|GetActiveAudioNoteWidget)))
        (:Is%20Not%20Valid
          _))
      (Variables|State|SetActiveAudioNoteWidget 0))
    (:then_1
      (Utilities|IsValid (Variables|State|GetActiveAudio)
        (:Is%20Valid
          (Components|Activation|SetActive (Variables|State|GetActiveAudio) false false))
        (:Is%20Not%20Valid
          _))
      (Variables|State|SetActiveAudio 0))))

(event Custom|E_ToggleJournal
  (params (Show :type Boolean))
  ;[0.02812 0.7171 1] Show / close journal
  (if Show
    (bind _returnvalue (UserInterface|CreateWidget "/Game/TextAndAudioNotes/Blueprints/Widgets/BP_W_Journal.BP_W_Journal_C" 0 (Variables|Journal|GetJournalEntries) self))
    (bind _output_get (Variables|Journal|SetJournalWidget _returnvalue))
    (UserInterface|Viewport|AddtoViewport _output_get (Variables|ZOrderSettings|GetJournalZOrder))
    (CallFunction|EStopActiveAudioNote)
    (CallFunction|ECloseActiveNote)
    (CallFunction|EToggleUIMode true)
    (else
      (bind _journalwidget (Variables|Journal|GetJournalWidget)
        (:then
          (Widget|RemovefromParent _journalwidget)
          (Variables|Journal|SetJournalWidget 0)
          (CallFunction|EToggleUIMode false)
          (CallFunction|EStopActiveAudioNote)
          (CallFunction|ECloseActiveNote))
        (:else)))))

(event Custom|E_ReadOrPlayNote
  (bind _noteyouarelookingat (Variables|State|GetNoteYouAreLookingAt))
  (bind _settings (Variables|/Game/TextAndAudioNotes/Blueprints/BP_TextNote.BP_TextNote_C|GetSettings _noteyouarelookingat))
  (bind (_isaudio _title _text _audio) (Utilities|Struct|BreakS_NoteSettings _settings))
  ;[0.1994 0.1886 1] 1. Read text note or play audio note
  ; 2. Add note to journal
  ; 3. Destroy note actor on level
  (Utilities|IsValid _noteyouarelookingat
    (:Is%20Valid
      (if _isaudio
        ;;[1 1 1] If you are listening audio note and picking up another audio note
        ;; - stop current audio note
        ;; - start playing picked up audio note
        (CallFunction|EStopActiveAudioNote)
        ;;[1 1 1] Play audio note and add it to journal
        (Utilities|FlowControl|Sequence
          (:then_0
            (bind _returnvalue (UserInterface|CreateWidget "/Game/TextAndAudioNotes/Blueprints/Widgets/BP_W_AudioNote.BP_W_AudioNote_C" 0 (Variables|/Game/TextAndAudioNotes/Blueprints/BP_TextNote.BP_TextNote_C|GetSettings (Variables|State|GetNoteYouAreLookingAt))))
            (bind _output_get (Variables|State|SetActiveAudioNoteWidget _returnvalue))
            (UserInterface|Viewport|AddtoViewport _output_get (Variables|ZOrderSettings|GetAudioNoteZOrder)))
          (:then_1
            (bind _returnvalue_2 (Audio|SpawnSound2D _audio 1.0 1.0 0.0 0))
            (Variables|State|SetActiveAudio _returnvalue_2))
          (:then_2
            (Utilities|FlowControl|Delay (Variables|/Script/Engine.SoundBase|GetDuration _audio)))
          (:then_3
            (CallFunction|EAddNotetoJournal)))
        (else
          ;;[1 1 1] Show text note and add it to journal
          (bind _returnvalue_3 (UserInterface|CreateWidget "/Game/TextAndAudioNotes/Blueprints/Widgets/BP_W_TextNote.BP_W_TextNote_C" 0 (Variables|/Game/TextAndAudioNotes/Blueprints/BP_TextNote.BP_TextNote_C|GetSettings (Variables|State|GetNoteYouAreLookingAt)) self))
          (bind _output_get_2 (Variables|State|SetActiveTextNoteWidget _returnvalue_3))
          (UserInterface|Viewport|AddtoViewport _output_get_2 (Variables|ZOrderSettings|GetTextNoteZOrder))
          (CallFunction|EAddNotetoJournal)
          (CallFunction|EToggleUIMode true))))))

(event Custom|E_AddNoteToJournal
  (bind _noteyouarelookingat (Variables|State|GetNoteYouAreLookingAt))
  ;[0.02812 0.7171 1] Add note to journal
  (Utilities|IsValid _noteyouarelookingat
    (:Is%20Valid
      (Utilities|Array|Add (Variables|Journal|GetJournalEntries) (Variables|/Game/TextAndAudioNotes/Blueprints/BP_TextNote.BP_TextNote_C|GetSettings _noteyouarelookingat))
      (Actor|DestroyActor (Variables|State|GetNoteYouAreLookingAt)))))

(event Custom|E_CloseActiveNote
  ;[1 0.2172 0] Close active note - try to close text widget, if there is one, else try to close audio witget
  (Utilities|IsValid (Variables|State|GetActiveTextNoteWidget)
    (:Is%20Valid
      (Widget|RemovefromParent (Variables|State|GetActiveTextNoteWidget))
      (Variables|State|SetActiveTextNoteWidget 0)
      (Utilities|IsValid (Variables|Journal|GetJournalWidget)
        (:Is%20Not%20Valid
          (CallFunction|EToggleUIMode false))))
    (:Is%20Not%20Valid
      (Utilities|IsValid (Variables|State|GetActiveAudioNoteWidget)
        (:Is%20Valid
          (Widget|RemovefromParent (Variables|State|GetActiveAudioNoteWidget))
          (Variables|State|SetActiveAudioNoteWidget 0))
        (:Is%20Not%20Valid
          _))
      (Utilities|IsValid (Variables|State|GetActiveAudio)
        (:Is%20Valid
          (Components|Activation|SetActive (Variables|State|GetActiveAudio) false false)
          (Variables|State|SetActiveAudio 0))))))

(event Custom|E_NoteTrace
  (params (PlayerCamera :type Scene%20Component%20Object%20Reference))
  (bind _returnvalue (Transformation|GetWorldLocation PlayerCamera))
  ;[0 1 0.531] Search tray
  (bind (_outhit _returnvalue_2) (Collision|LineTraceByChannel _returnvalue (+ _returnvalue (* (Math|Vector|GetForwardVector PlayerCamera) (Variables|Settings|GetTraceLenght))) "TraceTypeQuery1" false 0 "None"))
  (if _returnvalue_2
    (bind _asbp_text_note (Utilities|Casting|CastToBP_TextNote (.HitActor (Collision|BreakHitResult _outhit)))
      (:then
        (Utilities|IsValid (Variables|State|GetNoteYouAreLookingAt)
          (:Is%20Not%20Valid
            (Variables|State|SetNoteYouAreLookingAt _asbp_text_note))))
      (:CastFailed
        (Utilities|IsValid (Variables|State|GetNoteYouAreLookingAt)
          (:Is%20Valid
            (Variables|State|SetNoteYouAreLookingAt 0)))))
    (else
      (Utilities|IsValid (Variables|State|GetNoteYouAreLookingAt)
        (:Is%20Valid
          (Variables|State|SetNoteYouAreLookingAt 0))))))

(event Custom|E_ToggleUIMode
  (params (IsReadingNotes :type Boolean))
  (bind _returnvalue (Game|GetPlayerController 0))
  (bind _returnvalue_2 (Game|GetPlayerController 0))
  ;[0.4905 1 0] Switch between game and ui input modes
  (if IsReadingNotes
    (Variables|/Script/Engine.PlayerController|SetbShowMouseCursor _returnvalue_2 true)
    (Input|SetInputModeGameandUI _returnvalue_2 (Variables|Journal|GetJournalWidget) "DoNotLock" true)
    (else
      (Variables|/Script/Engine.PlayerController|SetbShowMouseCursor _returnvalue false)
      (Input|SetInputModeGameOnly _returnvalue))))

(event Custom|E_ShowTextNote
  (params (Settings :type S%20Note%20Settings%20Structure))
  ;[0.02812 0.7171 1] Show text note - function for journal entries
  (Utilities|FlowControl|Sequence
    (:then_0
      (Utilities|IsValid (Variables|State|GetActiveTextNoteWidget)
        (:Is%20Valid
          (Widget|RemovefromParent (Variables|State|GetActiveTextNoteWidget)))
        (:Is%20Not%20Valid
          _))
      (Variables|State|SetActiveTextNoteWidget 0))
    (:then_1
      (bind _returnvalue (UserInterface|CreateWidget "/Game/TextAndAudioNotes/Blueprints/Widgets/BP_W_TextNote.BP_W_TextNote_C" 0 Settings self))
      (bind _output_get (Variables|State|SetActiveTextNoteWidget _returnvalue))
      (UserInterface|Viewport|AddtoViewport _output_get (Variables|ZOrderSettings|GetTextNoteZOrder))
      (CallFunction|EToggleUIMode true))))