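; FlashlightBP is a flashlight pickup that the player collects with the Interact/Hide input.
; Overlapping its mesh as MainCharacterBP enables input and opens a gate; leaving disables input and closes it.
; The press adds the item to the character's inventory widget, then passes the gate to set HasFlashlight, play a sound and destroy the actor.
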(event OnComponentBeginOverlap(FlashlightSM)
  (params (OverlappedComponent :type Primitive%20Component%20Object%20Reference) (OtherActor :type Actor%20Object%20Reference) (OtherComp :type Primitive%20Component%20Object%20Reference) (OtherBodyIndex :type Integer) (bFromSweep :type Boolean) (SweepResult :type Hit%20Result%20Structure%20%28by%20ref%29))
  (bind _asmain_character_bp (Utilities|Casting|CastToMainCharacterBP OtherActor))
  (Input|EnableInput (Game|GetPlayerController 0))
  (Utilities|FlowControl|Gate true) ; enters at Open
)

(event OnComponentEndOverlap(FlashlightSM)
  (params (OverlappedComponent :type Primitive%20Component%20Object%20Reference) (OtherActor :type Actor%20Object%20Reference) (OtherComp :type Primitive%20Component%20Object%20Reference) (OtherBodyIndex :type Integer))
  (Utilities|Casting|CastToMainCharacterBP OtherActor)
  (Input|DisableInput (Game|GetPlayerController 0))
  (Utilities|FlowControl|Gate true) ; enters at Close
)

(event Input|ActionEvents|InputActionInteract/Hide
  (params (Key :type Key%20Structure :default "None"))
  (:Pressed
    (bind _asmain_character_bp (Utilities|Casting|CastToMainCharacterBP (Game|GetPlayerCharacter 0)))
    (Default|AddtoInventory (Variables|/Game/ThirdPersonBP/Blueprints/MainCharacterBP.MainCharacterBP_C|GetInventoryWG _asmain_character_bp) (Variables|Default|GetItemInfoStruct))
    (Utilities|FlowControl|Gate true
      (:Exit
        (Variables|/Game/ThirdPersonBP/Blueprints/MainCharacterBP.MainCharacterBP_C|SetHasFlashlight? (stale OnComponentBeginOverlap(FlashlightSM) _asmain_character_bp) true)
        (Audio|PlaySoundatLocation "/Game/MenuSystemPro/Sounds/sfx/sfx_ui_03.sfx_ui_03" (Transformation|GetActorLocation) "0, 0, 0" 1.0 1.0 0.0 0 0 0)
        (Actor|DestroyActor)))))

(fn ConstructionScript)